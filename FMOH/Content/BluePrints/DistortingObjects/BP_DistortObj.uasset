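; BP_DistortObj is an object whose static mesh distorts according to the player character's movement along world X.
; BeginPlay caches the mesh's original scale, and Tick checks the sign of that velocity.
; Negative X restarts the Distort timeline, which cumulatively stretches Y scale from its current value.
; Positive X restarts a second timeline, which lerps the current scale back toward the original.
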(event EventTick
  (params (DeltaSeconds :type Float%20%28single-precision%29))
  (bind _returnvalue (Game|GetPlayerCharacter 0))
  (bind _staticmesh (Variables|Default|GetStaticMesh))
  (bind _staticmesh_2 (Variables|Default|GetStaticMesh))
  (bind _returnvalue_2 (Transformation|GetVelocity _returnvalue))
  (bind _returnvalue_3 (Transformation|GetWorldScale _staticmesh))
  (if (< (.x _returnvalue_2) 0.0)
    (bind _newtrack_0 (Timeline|Distort PlayFromStart)
      (:Update
        (Transformation|SetWorldScale3D _staticmesh (Math|Vector|Lerp(Vector) _returnvalue_3 (+ _returnvalue_3 "0.000000,0.300000,0.000000") _newtrack_0))))
    (elif (> (.x _returnvalue_2) 0.0)
      (bind _newtrack_0_2 (Timeline|Timeline PlayFromStart)
        (:Update
          (Transformation|SetWorldScale3D _staticmesh_2 (Math|Vector|Lerp(Vector) (Transformation|GetWorldScale _staticmesh_2) (Variables|Default|GetOriginal%20Scale) _newtrack_0_2)))))))

(event EventBeginPlay
  (Variables|Default|SetOriginal%20Scale (Transformation|GetWorldScale (Variables|Default|GetStaticMesh))))

(fn ConstructionScript)