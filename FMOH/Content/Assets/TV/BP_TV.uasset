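; BP_TV is a television actor that can be switched on and off and flipped between two video channels.
; OnActivation alternates opening or closing the media player and toggles "Video Visibility" on a dynamic M_TV material, with a short delay before showing.
; SwitchChannel swaps between two MPL_TV_Vids playlist entries.
; Work-in-progress resume seeks to LastKnownTime on media open, though that time is read after open or close calls.
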(event Custom|Event%20Switch%20Channel
  (bind _tv_media_player (Variables|Default|GetTV%20Media%20Player))
  (bind _returnvalue (Class|MediaPlayer|GetTime _tv_media_player))
  ;[0.5181 0 1] Switching channels
  (if (not (Variables|Default|GetbIsIndex1%20Open))
    (Class|MediaPlayer|OpenPlaylistIndex _tv_media_player "/Game/Assets/TV/MPL_TV_Vids.MPL_TV_Vids" 1)
    (Variables|Default|SetbIsIndex1%20Open true)
    (Variables|Default|SetLast%20Known%20Time _returnvalue)
    (else
      (Class|MediaPlayer|OpenPlaylistIndex _tv_media_player "/Game/Assets/TV/MPL_TV_Vids.MPL_TV_Vids")
      (Variables|Default|SetbIsIndex1%20Open false)
      (Variables|Default|SetLast%20Known%20Time _returnvalue)))
  (Media|MediaPlayer|BindEventtoOnMediaOpened (Variables|Default|GetTV%20Media%20Player) (delegate Custom|Event%20On%20Media%20Opened)))

(event Custom|Event%20On%20Media%20Opened
  (params (OpenedUrl :type String))
  ;[0.521 0 1] Resuming video (WIP)
  (Media|MediaPlayer|Seek (Variables|Default|GetTV%20Media%20Player) (Variables|Default|GetLast%20Known%20Time)))

(event EventBeginPlay
  ;[0.521 0 1] Resuming video (WIP)
  (|CallParentFunction)
  (Media|MediaPlayer|BindEventtoOnMediaOpened (Variables|Default|GetTV%20Media%20Player) (delegate Custom|Event%20On%20Media%20Opened)))

(event Collision|EventActorBeginOverlap
  (params (OtherActor :type Actor%20Object%20Reference))
  (|CallParentFunction OtherActor) ; This node is disabled and will not be called.\nDrag off pins to build functionality.
)

(event EventTick
  (params (DeltaSeconds :type Float%20%28single-precision%29))
  (|CallParentFunction DeltaSeconds) ; This node is disabled and will not be called.\nDrag off pins to build functionality.
)

(event EventOnActivation
  (params (PlayerRef :type BP%20Third%20Person%20Character%20Object%20Reference))
  (bind _tv_visibility (Variables|Default|GetTV%20Visibility))
  (bind _tv_media_player (Variables|Default|GetTV%20Media%20Player))
  ;[0.5181 0 1] Turning power on/off
  (Utilities|FlowControl|FlipFlop
    (:A
      (if (Variables|Default|GetbIsIndex1%20Open)
        (Class|MediaPlayer|OpenPlaylistIndex _tv_media_player "/Game/Assets/TV/MPL_TV_Vids.MPL_TV_Vids" 1)
        (Variables|Default|SetbIsIndex1%20Open true)
        (else
          (Class|MediaPlayer|OpenPlaylistIndex _tv_media_player "/Game/Assets/TV/MPL_TV_Vids.MPL_TV_Vids")
          (Variables|Default|SetbIsIndex1%20Open false)))
      (Utilities|FlowControl|Delay 0.275)
      (Rendering|Material|SetScalarParameterValue _tv_visibility "Video Visibility" 1.0 :!class /Script/Engine.MaterialInstanceDynamic))
    (:B
      (Media|MediaPlayer|Close _tv_media_player :!class /Script/MediaAssets.MediaPlayer)
      (Variables|Default|SetLast%20Known%20Time (Class|MediaPlayer|GetTime _tv_media_player))
      (Rendering|Material|SetScalarParameterValue _tv_visibility "Video Visibility" 0.0 :!class /Script/Engine.MaterialInstanceDynamic))))

(fn ConstructionScript
  (|CallParentFunction)
  (bind _returnvalue (Rendering|Material|CreateDynamicMaterialInstance (Variables|Default|GetPlane) 0 "/Game/Assets/TV/M_TV.M_TV" "None" :!class /Script/Engine.PrimitiveComponent))
  (Variables|Default|SetTV%20Visibility _returnvalue))