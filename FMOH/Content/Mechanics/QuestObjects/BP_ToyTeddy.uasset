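; BP_ToyTeddy is a toy teddy quest item, a child Blueprint that builds on its parent's quest object behavior.
; On BeginPlay it applies a material to the first slot of the QuestItemMesh after running the parent setup.
; On interaction it runs the parent's OnInteract logic, then plays a 2D pickup sound.
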(event EventBeginPlay
  (|CallParentFunction)
  (Rendering|Material|SetMaterial (Variables|Default|GetQuestItemMesh) 0 (Variables|Default|GetMaterial)))

(event Collision|EventActorBeginOverlap
  (params (OtherActor :type Actor%20Object%20Reference))
  (|CallParentFunction OtherActor) ; This node is disabled and will not be called.\nDrag off pins to build functionality.
)

(event EventTick
  (params (DeltaSeconds :type Float%20%28single-precision%29))
  (|CallParentFunction DeltaSeconds) ; This node is disabled and will not be called.\nDrag off pins to build functionality.
)

(event EventOnInteract
  (params (PlayerRef :type BP%20Third%20Person%20Character%20Object%20Reference))
  (|CallParentFunction PlayerRef)
  (Audio|PlaySound2D "/Game/SoundSystem/Sounds/SFX/Actions/MS_PickUp.MS_PickUp" 1.0 1.0 0.0 0 0))

(fn ConstructionScript
  (|CallParentFunction))