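; Breakable glass quest object that shatters on interaction and reports the break to fracture listeners.
; OnInteract crumbles its Geometry Collection, plays a breaking sound, and adds a push along the player's forward vector plus a radial impulse to scatter the pieces.
; It then flags itself broken and passes the transform saved at BeginPlay to the BP_FractureListener actors found in the level.
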(event EventBeginPlay
  (Variables|Default|SetStartLocation (Transformation|GetActorTransform)))

(event Collision|EventActorBeginOverlap
  (params (OtherActor :type Actor%20Object%20Reference)))

(event EventTick
  (params (DeltaSeconds :type Float%20%28single-precision%29)))

(event EventOnInteract
  (params (PlayerRef :type BP%20Third%20Person%20Character%20Object%20Reference))
  (bind _geometrycollectioncomponent (Variables|Default|GetGeometryCollectionComponent))
  (bind _returnvalue (Transformation|GetWorldLocation _geometrycollectioncomponent))
  (Class|GeometryCollectionComponent|CrumbleCluster _geometrycollectioncomponent)
  (Development|PrintString "Velocity applied")
  (Audio|SpawnSoundatLocation "/Game/SoundSystem/Sounds/SFX/Actions/glass-breaking_Cue.glass-breaking_Cue" _returnvalue "0, 0, 0" 1.0 1.0 0.0 0 0)
  (Physics|AddImpulse _geometrycollectioncomponent (* (Transformation|GetActorForwardVector (Game|GetPlayerCharacter 0)) 1e+02) "None" false)
  (Physics|AddRadialImpulse _geometrycollectioncomponent _returnvalue 9e+01 6e+01 "RIF_Constant" false)
  (Variables|Default|SetbIsBroken true)
  (bind _outactors (Actor|GetAllActorsOfClass "/Game/Mechanics/ActivatableObject/BP_FractureListener.BP_FractureListener_C"))
  (Default|EventObjectBroken _outactors (Variables|Default|GetStartLocation)))

(fn ConstructionScript)