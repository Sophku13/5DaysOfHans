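; Base quest-object portal door that walks the player into position and swings open when interacted with while openable.
; Interaction fires activation, sound and camera shake, then a timeline lerps player location and view toward a scene point, with play rate set by distance.
; It then plays an entering montage and spawned camera animation before a delayed timeline rotates the Anchor.
; Reset closes and locks an opened door and unhides it.
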(event Custom|MoveDoor
  (bind _newtrack_0 (Timeline|Timeline PlayFromStart)
    (:Update
      (Transformation|SetRelativeRotation (Variables|Default|GetAnchor) (Math|Rotator|MakeRotator 0.0 0.0 (* _newtrack_0 90)) false false))
    (:Finished
      (Variables|Default|SetbIsDoorOpen true))))

(event Collision|EventActorBeginOverlap
  (params (OtherActor :type Actor%20Object%20Reference))
  (|CallParentFunction OtherActor) ; This node is disabled and will not be called.\nDrag off pins to build functionality.
)

(event EventOnInteract
  (params (PlayerRef :type BP%20Third%20Person%20Character%20Object%20Reference))
  (bind _returnvalue (Game|GetPlayerController 0))
  (bind _returnvalue_2 (Game|GetPlayerCharacter 0))
  (bind _scene (Variables|Default|GetScene))
  (bind _returnvalue_3 (Transformation|GetWorldLocation _scene))
  (bind _returnvalue_4 (Transformation|GetActorTransform _returnvalue_2))
  (if (Variables|Default|GetbCanBeOpened)
    (Variables|Default|SetPlayer%20Ref PlayerRef)
    (CallFunction|OnActivation PlayerRef)
    (Audio|PlaySoundatLocation 0 "0, 0, 0" "0, 0, 0" 1.0 1.0 0.0 0 0 0 0)
    ;[1 1 1] Change the speed of the timline depeding o how far the player is from the door
    (if (< (Transformation|GetDistanceTo (Variables|Default|GetPlayer%20Ref)) 1e+02)
      (Variables|Default|SetDynamicPlaeyrate 1.0)
      (elif (> (Transformation|GetDistanceTo (Variables|Default|GetPlayer%20Ref)) 2.5e+02)
        (Variables|Default|SetDynamicPlaeyrate 0.3)
        (else
          (Variables|Default|SetDynamicPlaeyrate 0.5))))
    ;[1 1 1] Move character to the door
    (Game|Feedback|ClientStartCameraShake _returnvalue "/Game/Mechanics/CameraBPs/BP_Walk.BP_Walk_C" 1.0 "CameraLocal" "0, 0, 0")
    (Components|Timeline|SetPlayRate (Variables|Default|GetMoveCHaracter) (Variables|Default|GetDynamicPlaeyrate))
    (bind (_direction _newtrack_0 _newtrack_1) (Timeline|Timeline_0 PlayFromStart)
      (:Update
        (Pawn|SetControlRotation _returnvalue (Math|Rotator|Lerp(Rotator) (Pawn|GetControlRotation _returnvalue :!class /Script/Engine.Controller) (* (Transformation|GetWorldRotation _scene) -1.0) _newtrack_1 true))
        (Transformation|SetActorLocation (Variables|Default|GetPlayer%20Ref) (Math|Vector|MakeVector (.x (Math|Vector|Lerp(Vector) (Transformation|GetActorLocation (Game|GetPlayerCharacter 0)) (Math|Vector|MakeVector (.x _returnvalue_3) (+ (.y _returnvalue_3) -6e+01) (.z (Transformation|GetActorLocation (Game|GetPlayerCharacter 0)))) _newtrack_0)) (.y (Math|Vector|Lerp(Vector) (Transformation|GetActorLocation (Game|GetPlayerCharacter 0)) (Math|Vector|MakeVector (.x _returnvalue_3) (+ (.y _returnvalue_3) -6e+01) (.z (Transformation|GetActorLocation (Game|GetPlayerCharacter 0)))) _newtrack_0)) (.z (Math|Vector|Lerp(Vector) (Transformation|GetActorLocation (Game|GetPlayerCharacter 0)) (Math|Vector|MakeVector (.x _returnvalue_3) (+ (.y _returnvalue_3) -6e+01) (.z (Transformation|GetActorLocation (Game|GetPlayerCharacter 0)))) _newtrack_0))) false false))
      (:Finished
        ;[0.9492 1 0.8181] animation code (4 arya)
        (Animation|Montage|PlayMontage (Variables|/Script/Engine.Character|GetMesh (Variables|Default|GetPlayer%20Ref)) "/Game/Characters/Mannequins/Animations/Arys_folder/other_animations/AM_door_entering_movement.AM_door_entering_movement"
          (:then
            (bind _returnvalue_5 (Game|SpawnActorfromClass "/Game/Characters/Mannequins/Animations/Arys_folder/other_animations/BP_door_entering_camera_animation.BP_door_entering_camera_animation_C" (Math|Transform|MakeTransform (.location _returnvalue_4) (.rotation _returnvalue_4) "1.000000,1.000000,1.000000") "Undefined" "MultiplyWithRoot" 0 0))
            (Default|PlayDoorAnimation _returnvalue_5)
            (Utilities|FlowControl|Delay 1.14) ; chng
            (bind _newtrack_0_2 (Timeline|Timeline PlayFromStart)
              (:Update
                (Transformation|SetRelativeRotation (Variables|Default|GetAnchor) (Math|Rotator|MakeRotator 0.0 0.0 (* _newtrack_0_2 90)) false false))
              (:Finished
                (Variables|Default|SetbIsDoorOpen true)))))))))

(event EventOnActivation
  (params (PlayerRef :type BP%20Third%20Person%20Character%20Object%20Reference))
  (|CallParentFunction PlayerRef))

(event EventOnReset
  (if (Variables|Default|GetbIsDoorOpen)
    (|CallParentFunction)
    (Transformation|SetRelativeRotation (Variables|Default|GetAnchor) (Math|Rotator|MakeRotator 0.0 0.0 0.0) false false)
    (Variables|Default|SetbCanBeOpened false)
    (Rendering|SetActorHiddenInGame false)))

(event EventSaveforReset
  (|CallParentFunction))

(fn ConstructionScript
  (|CallParentFunction))

(fn CreateListOfComponents
  (return 0))