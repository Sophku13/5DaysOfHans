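; BP_Prolog_Radio is a prologue radio quest object with an alarm, a clock display and four switchable channels.
; AlarmOff triggers OnActivation to set IsActivated, while Tick adds one minute to the clock every frame and refreshes its text.
; SwitchChannel cycles the channels, and OnOff uses a FlipFlop that re-announces the current channel when turned on.
; All sound playback is stubbed with PrintString, and the ChannelMap lookups are unused.
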(event Custom|AlarmOff
  (Development|PrintString "Stop Alarmsound")
  (CallFunction|OnActivation))

(event Custom|OnOff
  (Utilities|FlowControl|FlipFlop
    (:A
      (Development|PrintString "Radio On")
      (switch int (Variables|Default|GetcurrentChannel)
        (:1
          (Development|PrintString "Playing Channel 1"))
        (:2
          (Development|PrintString "Playing Channel 2"))
        (:3
          (Development|PrintString "Playing Channel 3"))
        (:4
          (Development|PrintString "Playing Channel 4"))))
    (:B
      (Development|PrintString "Radio Off"))))

(event Custom|Switch%20Channel
  (if (== (Variables|Default|GetcurrentChannel) 4)
    (Variables|Default|SetcurrentChannel 1)
    (else
      (Math|Integer|IncrementInt (Variables|Default|GetcurrentChannel)
        (:%20%20
          _))))
  (switch int (Variables|Default|GetcurrentChannel)
    (:1
      (Development|PrintString "Playing Channel 1"))
    (:2
      (Development|PrintString "Playing Channel 2"))
    (:3
      (Development|PrintString "Playing Channel 3"))
    (:4
      (Development|PrintString "Playing Channel 4"))))

(event Collision|EventActorBeginOverlap
  (params (OtherActor :type Actor%20Object%20Reference))
  (|CallParentFunction OtherActor) ; This node is disabled and will not be called.\nDrag off pins to build functionality.
)

(event EventTick
  (params (DeltaSeconds :type Float%20%28single-precision%29))
  (bind _output_get (Variables|Default|SetTime (Utilities|Struct|MakeTimecode (.hours (Variables|Default|GetTime)) (+ (.minutes (Variables|Default|GetTime)) 1) 0 0 false)))
  (Variables|/Script/Text3D.Text3DComponent|SetText (Variables|Default|GetTimeText) (Utilities|Text|ToText(String) (Utilities|String|Append (Utilities|String|ToString(Integer) (.hours _output_get)) ":" (Utilities|String|ToString(Integer) (.minutes _output_get))))))

(event EventOnActivation
  (params (PlayerRef :type BP%20Third%20Person%20Character%20Object%20Reference))
  (Variables|Default|SetbIsActivated true))

(event EventBeginPlay
  (Development|PrintString "Playing Alarmsound"))

(fn ConstructionScript
  (|CallParentFunction))