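; Quest key pickup for Room 1 that unlocks progress on a referenced door and triggers narrated story beats about Hans.
; Interacting flags the key as picked on the door, sets the door's tags, hides the key and spawns a BP_InterMono voice line with subtitle.
; A separate overlap box plays another monologue once by disabling its own collision.
; Reset clears the picked flag, re-shows the key and re-arms the box, leaving door tags unchanged.
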(event OnComponentBeginOverlap(FirstCommentBox)
  (params (OverlappedComponent :type Primitive%20Component%20Object%20Reference) (OtherActor :type Actor%20Object%20Reference) (OtherComp :type Primitive%20Component%20Object%20Reference) (OtherBodyIndex :type Integer) (bFromSweep :type Boolean) (SweepResult :type Hit%20Result%20Structure%20%28by%20ref%29))
  ;[0 0.02136 1] Sound!
  (bind _returnvalue (Game|SpawnActorfromClass "/Game/SoundSystem/Sounds/BP_InterMono.BP_InterMono_C" (Transformation|GetActorTransform (Game|GetPlayerCharacter 0)) "Undefined" "MultiplyWithRoot" 0 "/Game/SoundSystem/Sounds/VoiceRecordings/Narrator/HansThoughtCouldLeave_4.HansThoughtCouldLeave_4" 1.0 "Hans thought that since no one would notice he could leave the apartment to play outside. Or should he stay at home?" 8.0 true 0))
  (Default|CheckValues _returnvalue)
  (Collision|SetCollisionEnabled (Variables|Default|GetFirstCommentBox) "NoCollision"))

(event EventBeginPlay
  (|CallParentFunction) ; This node is disabled and will not be called.\nDrag off pins to build functionality.
)

(event Collision|EventActorBeginOverlap
  (params (OtherActor :type Actor%20Object%20Reference))
  (|CallParentFunction OtherActor) ; This node is disabled and will not be called.\nDrag off pins to build functionality.
)

(event EventTick
  (params (DeltaSeconds :type Float%20%28single-precision%29))
  (|CallParentFunction DeltaSeconds) ; This node is disabled and will not be called.\nDrag off pins to build functionality.
)

(event EventOnInteract
  (params (PlayerRef :type BP%20Third%20Person%20Character%20Object%20Reference))
  (bind _doorref (Variables|Default|GetDoorRef))
  (Variables|/Game/Mechanics/QuestObjects/BP_Quest_Door_Room1_1.BP_Quest_Door_Room1_1_C|SetbKeyIsPicked _doorref true)
  (Variables|/Script/Engine.Actor|SetTags _doorref (Variables|Default|GetTag))
  (bind _returnvalue (Game|SpawnActorfromClass "/Game/SoundSystem/Sounds/BP_InterMono.BP_InterMono_C" (Transformation|GetActorTransform (Game|GetPlayerCharacter 0)) "Undefined" "MultiplyWithRoot" 0 "/Game/SoundSystem/Sounds/VoiceRecordings/Narrator/HansFindsKey_1.HansFindsKey_1" 1.0 "As the key slipped in his hands Hans thought about his Father. He never let him outside alone." 8.0 true 0))
  (Default|CheckValues _returnvalue)
  (Development|SetHiddeninGame (Variables|Default|GetKey) true false))

(event EventOnReset
  (Variables|/Game/Mechanics/QuestObjects/BP_Quest_Door_Room1_1.BP_Quest_Door_Room1_1_C|SetbKeyIsPicked (Variables|Default|GetDoorRef) false)
  (Collision|SetCollisionEnabled (Variables|Default|GetFirstCommentBox) "QueryOnly")
  (Development|SetHiddeninGame (Variables|Default|GetKey) false false))

(fn ConstructionScript
  (|CallParentFunction))