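; BP_QuestButtonPrototype_Listener is a quest button variant that only activates while none of the buttons it listens to is completed.
; On activation it checks IsQuestCompleted on each entry in ButtonsListeningTo and clears IsRelevant if any is true.
; The parent activation logic runs only while IsRelevant remains true, and this Blueprint never sets that flag back.
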(event EventBeginPlay
  (|CallParentFunction) ; This node is disabled and will not be called.\nDrag off pins to build functionality.
)

(event Collision|EventActorBeginOverlap
  (params (OtherActor :type Actor%20Object%20Reference))
  (|CallParentFunction OtherActor) ; This node is disabled and will not be called.\nDrag off pins to build functionality.
)

(event EventTick
  (params (DeltaSeconds :type Float%20%28single-precision%29))
  (|CallParentFunction DeltaSeconds) ; This node is disabled and will not be called.\nDrag off pins to build functionality.
)

(event EventOnActivation
  (params (PlayerRef :type BP%20Third%20Person%20Character%20Object%20Reference))
  ;[0.1647 1 0.702] Is only relevant and will activate, when none of the Buttons this one is listening to are already completed.
  (for _array_element (Variables|Default|GetButtonsListeningTo)
    (if (Variables|/Game/Mechanics/BaseBlueprints/BP_BaseQuestItem.BP_BaseQuestItem_C|GetbIsQuestCompleted _array_element)
      (Variables|Default|SetbIsRelevant false)))
  (if (Variables|Default|GetbIsRelevant)
    (|CallParentFunction PlayerRef)))

(fn ConstructionScript
  (|CallParentFunction))