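; BP_CorridorTrigger is a quest object that, when a player or other object overlaps its trigger box, activates and prepares the next room.
; OnActivation runs the parent logic, copies the activated state into the quest-completed flag, then async loads the next room reference.
; When loading completes, the current room spawns a room switcher for that room; an invalid reference prints a debug error.
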(event OnComponentBeginOverlap(TriggerBox)
  (params (OverlappedComponent :type Primitive%20Component%20Object%20Reference) (OtherActor :type Actor%20Object%20Reference) (OtherComp :type Primitive%20Component%20Object%20Reference) (OtherBodyIndex :type Integer) (bFromSweep :type Boolean) (SweepResult :type Hit%20Result%20Structure%20%28by%20ref%29))
  (CallFunction|OnActivation))

(event EventOnActivation
  (params (PlayerRef :type BP%20Third%20Person%20Character%20Object%20Reference))
  (|CallParentFunction 0)
  (Variables|Default|SetbIsQuestCompleted (Variables|Default|GetbIsActivated))
  (bind __nextroomref (Variables|Default|Get_NextRoomRef)
    (:then
      (Utilities|AsyncLoadAsset __nextroomref
        (:Completed
          (Default|SpawnRoomSwitcher (Variables|Default|Get_currentRoomRef) __nextroomref))))
    (:else
      (Development|PrintString "ButtonNextRoomRef NOT WORKING!"))))

(fn ConstructionScript
  (|CallParentFunction))