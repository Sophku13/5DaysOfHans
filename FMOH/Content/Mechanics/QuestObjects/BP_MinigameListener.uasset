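; BP_MinigameListener is a quest object that turns a decision into a transition to the next room.
; ActivateChoice looks up the soft room reference for the decision number in NextRoomsRefs, then calls OnActivation.
; OnActivation runs the parent logic, copies IsActivated to IsQuestCompleted, async loads the chosen room and has the current room spawn a room switcher to it.
; An invalid reference only prints a debug message.
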(event Custom|ActivateChoice
  (params (DecisionNumber :type Integer%20%28by%20ref%29) (PlayerRef :type BP%20Third%20Person%20Character%20Object%20Reference))
  (Variables|Default|Set_NextRoomRef (.Value (Utilities|Map|Find (Variables|Default|GetNextRoomsRefs) DecisionNumber)))
  (CallFunction|OnActivation PlayerRef))

(event EventBeginPlay
  (|CallParentFunction) ; This node is disabled and will not be called.\nDrag off pins to build functionality.
)

(event Collision|EventActorBeginOverlap
  (params (OtherActor :type Actor%20Object%20Reference))
  (|CallParentFunction OtherActor) ; This node is disabled and will not be called.\nDrag off pins to build functionality.
)

(event EventTick
  (params (DeltaSeconds :type Float%20%28single-precision%29))
  (|CallParentFunction DeltaSeconds) ; This node is disabled and will not be called.\nDrag off pins to build functionality.
)

(event EventOnActivation
  (params (PlayerRef :type BP%20Third%20Person%20Character%20Object%20Reference))
  (|CallParentFunction 0)
  (Variables|Default|SetbIsQuestCompleted (Variables|Default|GetbIsActivated))
  (bind __nextroomref (Variables|Default|Get_NextRoomRef)
    (:then
      (Utilities|AsyncLoadAsset __nextroomref
        (:Completed
          (Default|SpawnRoomSwitcher (Variables|Default|Get_currentRoomRef) __nextroomref))))
    (:else
      (Development|PrintString "ButtonNextRoomRef NOT WORKING!"))))

(fn ConstructionScript
  (|CallParentFunction))