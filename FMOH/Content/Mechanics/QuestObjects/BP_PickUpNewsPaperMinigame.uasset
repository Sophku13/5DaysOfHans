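; Interactable quest pickup for a newspaper that launches the newspaper minigame when the player interacts with it.
; After the parent interaction, it snaps to the player's item actor, then waits briefly before disabling character input.
; It then shows the minigame widget with UI-only input and a visible mouse cursor, and hides the crosshair.
; The graph contains no logic to restore input or the crosshair afterward.
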(event EventOnInteract
  (params (PlayerRef :type BP%20Third%20Person%20Character%20Object%20Reference))
  (bind _returnvalue (Game|GetPlayerController 0))
  (|CallParentFunction PlayerRef)
  (Transformation|AttachComponentToComponent self (Variables|/Game/ThirdPerson/Blueprints/BP_ThirdPersonCharacter.BP_ThirdPersonCharacter_C|GetItemActor PlayerRef) "None" "SnapToTarget" "SnapToTarget" "SnapToTarget" true)
  (Utilities|FlowControl|Delay 0.2)
  (Input|DisableInput (Game|GetPlayerCharacter 0) (Game|GetPlayerController 0))
  (bind _returnvalue_2 (UserInterface|CreateWidget "/Game/UI/UIMinigames/WBP_NewsPaperMinigame.WBP_NewsPaperMinigame_C"))
  (UserInterface|Viewport|AddtoViewport _returnvalue_2 0)
  (Input|SetInputModeUIOnly _returnvalue 0 "DoNotLock" false)
  (Variables|/Script/Engine.PlayerController|SetbShowMouseCursor _returnvalue true)
  (Widget|SetVisibility (Variables|/Game/ThirdPerson/Blueprints/BP_ThirdPersonCharacter.BP_ThirdPersonCharacter_C|GetCrosshair%20REF PlayerRef) "Hidden"))

(fn ConstructionScript
  (|CallParentFunction))