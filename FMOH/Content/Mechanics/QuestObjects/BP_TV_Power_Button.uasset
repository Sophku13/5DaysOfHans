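; BP_TV_Power_Button is an interactable power button for a TV quest object.
; On interact it calls OnActivation on the referenced TV Blueprint, passing the player reference.
; It then nudges its Sphere component along world X, waits a second on a Delay, and moves it back to fake a button press.
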(event EventBeginPlay
  (|CallParentFunction) ; This node is disabled and will not be called.\nDrag off pins to build functionality.
)

(event Collision|EventActorBeginOverlap
  (params (OtherActor :type Actor%20Object%20Reference)))

(event EventTick
  (params (DeltaSeconds :type Float%20%28single-precision%29)))

(event EventOnInteract
  (params (PlayerRef :type BP%20Third%20Person%20Character%20Object%20Reference))
  (bind _sphere (Variables|Default|GetSphere))
  (bind _sphere_2 (Variables|Default|GetSphere))
  (Default|OnActivation (Variables|Default|GetTV%20BP) PlayerRef)
  (Transformation|SetWorldLocation _sphere_2 (+ (Transformation|GetWorldLocation _sphere_2) "1.500000,0.000000,0.000000") false false)
  (Utilities|FlowControl|Delay 1.0)
  (Transformation|SetWorldLocation _sphere (+ (Transformation|GetWorldLocation _sphere) "-1.500000,0.000000,0.000000") false false))

(fn ConstructionScript
  (|CallParentFunction))