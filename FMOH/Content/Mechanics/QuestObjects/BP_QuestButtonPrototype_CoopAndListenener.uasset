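; A quest button prototype that combines cooperation with other buttons and listening to "main" buttons.
; On activation it clears its relevance if any listened-to button is completed, then checks whether every cooperating button is completed.
; If all are completed and it is still relevant, it runs the parent activation.
; If any cooperator is unfinished, it only flags its own quest as completed, skipping the parent logic.
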(event EventBeginPlay
  (|CallParentFunction) ; This node is disabled and will not be called.\nDrag off pins to build functionality.
)

(event Collision|EventActorBeginOverlap
  (params (OtherActor :type Actor%20Object%20Reference))
  (|CallParentFunction OtherActor) ; This node is disabled and will not be called.\nDrag off pins to build functionality.
)

(event EventTick
  (params (DeltaSeconds :type Float%20%28single-precision%29))
  (|CallParentFunction DeltaSeconds) ; This node is disabled and will not be called.\nDrag off pins to build functionality.
)

(event EventOnActivation
  (params (PlayerRef :type BP%20Third%20Person%20Character%20Object%20Reference))
  ;[0.1647 1 0.702] Will only be fully completed if all other cooperating buttons are also completed and none of the main buttons are activated
  (for _array_element (Variables|Default|GetButtonsListeningTo)
    (if (Variables|/Game/Mechanics/BaseBlueprints/BP_BaseQuestItem.BP_BaseQuestItem_C|GetbIsQuestCompleted _array_element)
      (Variables|Default|SetbIsRelevant false)))
  (for (_array_element_2 _array_index) (Variables|Default|GetCooperatingButtonsList)
    (if (== _array_index 0)
      (Variables|Default|SetbAllConnectedItemsCompleted (Variables|/Game/Mechanics/BaseBlueprints/BP_BaseQuestItem.BP_BaseQuestItem_C|GetbIsQuestCompleted _array_element_2))
      (elif (not (and (Variables|/Game/Mechanics/BaseBlueprints/BP_BaseQuestItem.BP_BaseQuestItem_C|GetbIsQuestCompleted _array_element_2) (Variables|Default|GetbAllConnectedItemsCompleted)))
        (Variables|Default|SetbAllConnectedItemsCompleted false))))
  (if (Variables|Default|GetbAllConnectedItemsCompleted)
    (if (Variables|Default|GetbIsRelevant)
      (|CallParentFunction PlayerRef))
    (else
      (Variables|Default|SetbIsQuestCompleted true))))

(fn ConstructionScript
  (|CallParentFunction))