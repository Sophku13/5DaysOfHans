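; Base quest door that, when activated, asynchronously loads the next room and has the current room spawn a room switcher for it.
; Interacting activates it and triggers a linked second door.
; Once completed, holding the drag input while a camera trace hits a quest door rotates the hinge by player turn rate, using open/close angle limits.
; Reset closes the linked door and restores this one, but destroys completed death doors.
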(event Input|EnhancedActionEvents|EnhancedInputActionIA_DragObjects
  (params (ActionValue :type Boolean) (ElapsedSeconds :type Float%20%28double-precision%29) (TriggeredSeconds :type Float%20%28double-precision%29) (InputAction :type Input%20Action%20Object%20Reference :default "/Game/Character/Input/Actions/IA_DragObjects.IA_DragObjects"))
  ;[1 1 1] Comment
  ;;[1 1 1] Comment
  (:Started
    (Variables|Default|SetbIsHoldingLMB true)
    (bind _asbp_third_person_character (Utilities|Casting|CastToBP_ThirdPersonCharacter (Game|GetPlayerCharacter 0)))
    (bind (_outhit _returnvalue) (Collision|LineTraceForObjects (Transformation|GetWorldLocation (Variables|/Game/ThirdPerson/Blueprints/BP_ThirdPersonCharacter.BP_ThirdPersonCharacter_C|GetFollowCamera _asbp_third_person_character)) (+ (Transformation|GetWorldLocation (Variables|/Game/ThirdPerson/Blueprints/BP_ThirdPersonCharacter.BP_ThirdPersonCharacter_C|GetFollowCamera _asbp_third_person_character)) (* (Math|Vector|GetForwardVector (Variables|/Game/ThirdPerson/Blueprints/BP_ThirdPersonCharacter.BP_ThirdPersonCharacter_C|GetFollowCamera _asbp_third_person_character)) 5e+02)) (Utilities|Array|MakeArray "ObjectTypeQuery1") false 0 "None" false))
    (if _returnvalue
      (Utilities|Casting|CastToBP_Quest_Door_Base (.HitActor (Collision|BreakHitResult _outhit)))
      (Variables|Default|SetbLookingAtDoor true)
      (else
        (Variables|Default|SetbLookingAtDoor false))))
  (:Canceled
    (Variables|Default|SetbIsHoldingLMB false :!label _label))
  (:Completed
    (goto _label)))

(event EventBeginPlay
  ;[1 1 1] Comment
  (|CallParentFunction)
  (Input|EnableInput (Game|GetPlayerController 0)))

(event Collision|EventActorBeginOverlap
  (params (OtherActor :type Actor%20Object%20Reference))
  (|CallParentFunction OtherActor) ; This node is disabled and will not be called.\nDrag off pins to build functionality.
)

(event EventOnInteract
  (params (PlayerRef :type BP%20Third%20Person%20Character%20Object%20Reference))
  (CallFunction|OnActivation)
  (Default|OnInteract (Variables|Default|GetSecondDoorRef)))

(event EventOnActivation
  (params (PlayerRef :type BP%20Third%20Person%20Character%20Object%20Reference))
  (|CallParentFunction 0)
  (Variables|Default|SetbIsQuestCompleted (Variables|Default|GetbIsActivated))
  (bind __nextroomref (Variables|Default|Get_NextRoomRef)
    (:then
      (Utilities|AsyncLoadAsset __nextroomref
        (:Completed
          (Default|SpawnRoomSwitcher (Variables|Default|Get_currentRoomRef) __nextroomref))))
    (:else
      (Development|PrintString "DoorNextRoomRef NOT WORKING!"))))

(event EventOnReset
  (bind _seconddoorref (Variables|Default|GetSecondDoorRef))
  (if (not (and (Variables|Default|GetbIsQuestCompleted) (Variables|Default|GetbIsDeathDoor)))
    (|CallParentFunction)
    (if (Variables|/Game/Mechanics/InteractableObjects/BP_DoorUsable.BP_DoorUsable_C|GetbIsDoorOpen _seconddoorref)
      (Default|OnInteract _seconddoorref)
      (Rendering|SetActorHiddenInGame self false)
      (Collision|SetCollisionEnabled (Variables|Default|GetDoor) "QueryAndPhysics")
      (Transformation|SetRelativeRotation (Variables|Default|GetAnchor) (Math|Rotator|MakeRotator 0.0 0.0 0.0) false false))
    (else
      (Actor|DestroyActor))))

(event EventSaveforReset
  (|CallParentFunction))

(event EventTick
  (params (DeltaSeconds :type Float%20%28single-precision%29))
  (bind _anchor (Variables|Default|GetAnchor))
  (bind _openangle (Variables|Default|GetOpenAngle))
  (bind _returnvalue (Transformation|GetWorldRotation _anchor))
  ;[1 1 1] Comment
  ;;[1 1 1] Comment
  (if (Variables|Default|GetbIsQuestCompleted)
    (if (Variables|Default|GetbIsHoldingLMB)
      (if (Variables|Default|GetbLookingAtDoor)
        (if (not (== (.yaw _returnvalue) (Math|Float|ClampAngle (.yaw _returnvalue) (Variables|Default|GetCloseAngle) (Variables|Default|GetOpenAngle))))
          (Transformation|AddLocalRotation _anchor (Math|Rotator|MakeRotator 0.0 0.0 (* (Variables|/Game/ThirdPerson/Blueprints/BP_ThirdPersonCharacter.BP_ThirdPersonCharacter_C|GetTurnRate (stale Input|EnhancedActionEvents|EnhancedInputActionIA_DragObjects _asbp_third_person_character)) (Variables|Default|GetSensitivity))) false false)
          (elif (>= (.yaw _returnvalue) _openangle)
            (Transformation|SetRelativeRotation _anchor (Math|Rotator|MakeRotator 0.0 0.0 (- _openangle 1.0)) false false)
            (else
              (Transformation|SetRelativeRotation _anchor (Math|Rotator|MakeRotator 0.0 0.0 (+ (Variables|Default|GetCloseAngle) 1.0)) false false))))))))

(fn ConstructionScript
  (|CallParentFunction))

(fn CreateListOfComponents
  (return 0))