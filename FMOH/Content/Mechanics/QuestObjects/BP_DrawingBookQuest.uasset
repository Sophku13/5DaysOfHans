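; BP_DrawingBookQuest is an interactable quest object for a drawing book, locked according to the state of the red toy boat.
; Tick sets the lock every frame while the boat is picked up or its quest is completed.
; Interacting while unlocked runs the parent interaction and activation, which copies the activated state into quest completion.
; Disconnected leftover logic would async-load the next room and spawn a room switcher.
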(event EventBeginPlay
  (|CallParentFunction) ; This node is disabled and will not be called.\nDrag off pins to build functionality.
)

(event Collision|EventActorBeginOverlap
  (params (OtherActor :type Actor%20Object%20Reference))
  (|CallParentFunction OtherActor) ; This node is disabled and will not be called.\nDrag off pins to build functionality.
)

(event EventTick
  (params (DeltaSeconds :type Float%20%28single-precision%29))
  (bind _toyboatred (Variables|Default|GetToyBoatRed))
  (|CallParentFunction DeltaSeconds)
  (if (or (Variables|/Game/Mechanics/BaseBlueprints/BP_BaseQuestItem.BP_BaseQuestItem_C|GetbIsQuestCompleted _toyboatred) (Variables|/Game/Mechanics/QuestObjects/BP_BaseQuestPickUpItem.BP_BaseQuestPickUpItem_C|GetbIsPickedUp _toyboatred))
    (Variables|Default|SetbIsLocked true)
    (else
      (Variables|Default|SetbIsLocked false))))

(event EventOnActivation
  (params (PlayerRef :type BP%20Third%20Person%20Character%20Object%20Reference))
  (|CallParentFunction 0)
  (Variables|Default|SetbIsQuestCompleted (Variables|Default|GetbIsActivated)))

(event EventOnInteract
  (params (PlayerRef :type BP%20Third%20Person%20Character%20Object%20Reference))
  (if (not (Variables|Default|GetbIsLocked))
    (|CallParentFunction PlayerRef)
    (CallFunction|OnActivation PlayerRef)))

(event EventOnReset
  (|CallParentFunction))

(event EventSaveforReset
  (|CallParentFunction))

(fn ConstructionScript
  (|CallParentFunction))