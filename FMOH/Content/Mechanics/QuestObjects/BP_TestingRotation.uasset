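; BP_TestingRotation is a test quest object for inspecting an item and spinning it by mouse drag.
; OnInteract snaps it to the player's InspectableItem, shows the cursor, and locks movement and camera.
; ScrollComponent click, release and cursor-exit events toggle dragging.
; DragKnife builds yaw velocity from axis input and RotateKnife applies it with damping, but Tick is empty and their calls are disconnected, so rotation never runs.
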(event OnClicked(ScrollComponent)
  (params (TouchedComponent :type Primitive%20Component%20Object%20Reference) (ButtonPressed :type Key%20Structure :default "None"))
  (bind _output_get (Variables|Default|SetIsDragging true))
  (Development|PrintString (Utilities|String|ToString(Boolean) _output_get)))

(event OnReleased(ScrollComponent)
  (params (TouchedComponent :type Primitive%20Component%20Object%20Reference) (ButtonReleased :type Key%20Structure :default "None"))
  (Variables|Default|SetIsDragging false))

(event OnEndCursorOver(ScrollComponent)
  (params (TouchedComponent :type Primitive%20Component%20Object%20Reference))
  (Variables|Default|SetIsDragging false))

(event Custom|RotateKnife
  (params (Delta%20Seconds :type Float%20%28double-precision%29))
  (Class|Actor|AddActorWorldRotation (Math|Rotator|MakeRotator 0.0 0.0 (* Delta%20Seconds (Variables|Default|GetRotateVelocity))))
  (if (or (< (Variables|Default|GetRotateVelocity) 1.0) (> (Variables|Default|GetRotateVelocity) -1.0))
    (Variables|Default|SetRotateVelocity (* (Variables|Default|GetRotateVelocity) 0.95))
    (Variables|Default|SetdragSumX (* (Variables|Default|GetdragSumX) 0.95))))

(event Custom|DragKnife
  (params (DeltaSeconds :type Float%20%28double-precision%29))
  (if (Variables|Default|GetIsDragging)
    (bind _output_get (Variables|Default|SetdragSumX (- (Variables|Default|GetdragSumX) (Class|Actor|GetInputAxisKeyValue))))
    (Variables|Default|SetRotateVelocity (+ (Variables|Default|GetRotateVelocity) (* (* _output_get DeltaSeconds) 3e+01)))
    (else
      (Variables|Default|SetdragSumX 0.0))))

(event EventTick
  (params (DeltaSeconds :type Float%20%28single-precision%29)))

(event EventOnInteract
  (params (PlayerRef :type BP%20Third%20Person%20Character%20Object%20Reference))
  (Transformation|AttachComponentToComponent (Variables|/Game/ThirdPerson/Blueprints/BP_ThirdPersonCharacter.BP_ThirdPersonCharacter_C|GetinspectableItem PlayerRef) "None" "SnapToTarget" "SnapToTarget" "SnapToTarget" true)
  (Utilities|FlowControl|Delay 0.1)
  (Variables|/Script/Engine.PlayerController|SetbShowMouseCursor (Game|GetPlayerController 0) true)
  (Variables|/Game/ThirdPerson/Blueprints/BP_ThirdPersonCharacter.BP_ThirdPersonCharacter_C|SetIsMovementLocked PlayerRef true)
  (Variables|/Game/ThirdPerson/Blueprints/BP_ThirdPersonCharacter.BP_ThirdPersonCharacter_C|SetbIsCameraLocked PlayerRef true))

(fn ConstructionScript
  (|CallParentFunction))

(fn Drag
  (params (DeltaSeconds1 :type Float%20%28double-precision%29)))