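; Interactable quest book that starts the "Between Pages" minigame.
; On interact it snaps to the player's inspect point, swaps a book material slot to the render-target first page, hides the crosshair and locks player movement and camera.
; It then hands control to a referenced minigame pawn by possession, adds the minigame input mapping context and makes itself the view target.
; No exit or gameplay logic lives here.
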(event EventBeginPlay
  (Rendering|Material|SetMaterial (Variables|Default|GetBook) 3 "/Game/Assets/Meshes/FatherAssets/ch.ch"))

(event EventOnInteract
  (params (PlayerRef :type BP%20Third%20Person%20Character%20Object%20Reference))
  (bind _returnvalue (Game|GetPlayerController 0))
  (bind _pawnref (Variables|Default|GetPawnREF))
  (|CallParentFunction PlayerRef)
  (Transformation|AttachComponentToComponent (Variables|/Game/ThirdPerson/Blueprints/BP_ThirdPersonCharacter.BP_ThirdPersonCharacter_C|GetinspectableItem PlayerRef) "None" "SnapToTarget" "SnapToTarget" "SnapToTarget" true)
  (Rendering|Material|SetMaterial (Variables|Default|GetBook) 3 "/Game/Mechanics/MiniGames/InTheBook/RednderTargets/RT_FirstPage_Mat.RT_FirstPage_Mat")
  (Widget|SetVisibility (Variables|/Game/ThirdPerson/Blueprints/BP_ThirdPersonCharacter.BP_ThirdPersonCharacter_C|GetCrosshair%20REF PlayerRef) "Hidden")
  (Variables|/Game/ThirdPerson/Blueprints/BP_ThirdPersonCharacter.BP_ThirdPersonCharacter_C|SetIsMovementLocked PlayerRef true)
  (Variables|/Game/ThirdPerson/Blueprints/BP_ThirdPersonCharacter.BP_ThirdPersonCharacter_C|SetbIsCameraLocked PlayerRef true)
  (Variables|Default|SetQuestItemREF 0)
  (Variables|/Game/Mechanics/MiniGames/InTheBook/BP_PawnSideView.BP_PawnSideView_C|SetPlayerRef _pawnref PlayerRef)
  (Pawn|Possess _returnvalue _pawnref)
  (Input|AddMappingContext _returnvalue "/Game/ThirdPerson/Input/IMC_MiniGame.IMC_MiniGame" 0 "(bIgnoreAllPressedKeysUntilRelease=True,bForceImmediately=False,bNotifyUserSettings=False)")
  (Game|Player|SetViewTargetwithBlend _returnvalue self 0.0 "VTBlend_Linear" 0.0 false))

(fn ConstructionScript
  (|CallParentFunction))