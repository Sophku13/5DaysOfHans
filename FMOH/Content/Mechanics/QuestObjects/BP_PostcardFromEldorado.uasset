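; Quest item pickup for a postcard from Eldorado that opens an inspection screen with text when the player interacts with it.
; On interact it snaps to the player's InspectableItem component, sets its item type and prints a debug message.
; After a brief delay it disables player input, shows the WBP_ObjectInspectionWithText widget with itself as the quest item, switches to UI-only input with cursor, and pauses the game.
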(event EventOnInteract
  (params (PlayerRef :type BP%20Third%20Person%20Character%20Object%20Reference))
  (bind _returnvalue (Game|GetPlayerController 0))
  (Transformation|AttachComponentToComponent self (Variables|/Game/ThirdPerson/Blueprints/BP_ThirdPersonCharacter.BP_ThirdPersonCharacter_C|GetinspectableItem PlayerRef) "None" "SnapToTarget" "SnapToTarget" "SnapToTarget" true)
  (Variables|Default|SetItemType "NewEnumerator15")
  (Development|PrintString "picked up postcard from eldoraro")
  (Utilities|FlowControl|Delay 0.1)
  (Input|DisableInput (Game|GetPlayerController 0) (Game|GetPlayerController 0))
  (bind _returnvalue_2 (UserInterface|CreateWidget "/Game/UI/ObjectInspectionWBPs/WBP_ObjectInspectionWithText.WBP_ObjectInspectionWithText_C" 0 self))
  (Variables|/Game/UI/ObjectInspectionWBPs/WBP_ObjectInspectionWithText.WBP_ObjectInspectionWithText_C|SetQuestItemREF _returnvalue_2 self)
  (UserInterface|Viewport|AddtoViewport _returnvalue_2 0)
  (Input|SetInputModeUIOnly _returnvalue 0 "DoNotLock" false)
  (Variables|/Script/Engine.PlayerController|SetbShowMouseCursor _returnvalue true)
  (Game|SetGamePaused true))

(fn ConstructionScript
  (|CallParentFunction))