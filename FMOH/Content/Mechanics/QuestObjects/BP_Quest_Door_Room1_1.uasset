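; Quest door for Room 1 that leads the player into the next room once the key is picked.
; Interaction without the key prints a placeholder inner monologue; with it, activation updates quest completion, async-loads the next room and has the current room spawn a room switcher.
; Reset calls the parent, clears completion and zeroes the hinge rotation.
; The walk-to-door cinematic and swing timeline are left unwired.
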(event Collision|EventActorBeginOverlap
  (params (OtherActor :type Actor%20Object%20Reference))
  (|CallParentFunction OtherActor) ; This node is disabled and will not be called.\nDrag off pins to build functionality.
)

(event EventOnInteract
  (params (PlayerRef :type BP%20Third%20Person%20Character%20Object%20Reference))
  (if (Variables|Default|GetbKeyIsPicked)
    (Variables|Default|SetPlayer%20Ref PlayerRef)
    (CallFunction|OnActivation PlayerRef)
    (Audio|PlaySoundatLocation 0 "0, 0, 0" "0, 0, 0" 1.0 1.0 0.0 0 0 0 0)
    (else
      ;[0 0.1127 1] Sound
      (Development|PrintString "INNER MONO: WHERE DID THEY PUT THE KEY?"))))

(event EventOnActivation
  (params (PlayerRef :type BP%20Third%20Person%20Character%20Object%20Reference))
  (|CallParentFunction PlayerRef)
  (Variables|Default|SetbIsQuestCompleted (Variables|Default|GetbIsActivated))
  (bind __nextroomref (Variables|Default|Get_NextRoomRef)
    (:then
      (Utilities|AsyncLoadAsset __nextroomref
        (:Completed
          (Default|SpawnRoomSwitcher (Variables|Default|Get_currentRoomRef) __nextroomref))))
    (:else
      (Development|PrintString "DoorNextRoomRef NOT WORKING!"))))

(event EventOnReset
  (if (not (Variables|Default|GetbIsQuestCompleted))
    (|CallParentFunction)
    (else
      (|CallParentFunction)
      (Variables|Default|SetbIsQuestCompleted false)))
  (Transformation|SetRelativeRotation (Variables|Default|GetAnchor) (Math|Rotator|MakeRotator 0.0 0.0 0.0) false false))

(event EventSaveforReset
  (|CallParentFunction))

(fn ConstructionScript
  (|CallParentFunction))

(fn CreateListOfComponents
  (return 0))