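; BP_Quest_Door is a quest door that opens on interaction and links the current room to the next.
; Interaction runs activation, plays a sound, triggers a paired second door and swings the anchor via Timeline, then hides the door and disables collision.
; Activation marks quest completion and async-loads the next room before the current room spawns a room switcher.
; Reset destroys completed death doors, otherwise restores the door if its partner is open.
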(event EventBeginPlay
  (|CallParentFunction) ; This node is disabled and will not be called.\nDrag off pins to build functionality.
)

(event Collision|EventActorBeginOverlap
  (params (OtherActor :type Actor%20Object%20Reference))
  (|CallParentFunction OtherActor) ; This node is disabled and will not be called.\nDrag off pins to build functionality.
)

(event EventTick
  (params (DeltaSeconds :type Float%20%28single-precision%29))
  (|CallParentFunction DeltaSeconds) ; This node is disabled and will not be called.\nDrag off pins to build functionality.
)

(event EventOnInteract
  (params (PlayerRef :type BP%20Third%20Person%20Character%20Object%20Reference))
  (bind _self self)
  (CallFunction|OnActivation)
  (Audio|PlaySoundatLocation "/Game/SoundSystem/Sounds/Door/SC_OpenDoor_3_Cue.SC_OpenDoor_3_Cue" "0, 0, 0" "0, 0, 0" 1.0 1.0 0.0 0 0 0 0)
  (Default|OnInteract (Variables|Default|GetSecondDoorRef))
  (bind _newtrack_0 (Timeline|Timeline Play)
    (:Update
      (Transformation|SetRelativeRotation (Variables|Default|GetAnchor) (Math|Rotator|MakeRotator 0.0 0.0 (* _newtrack_0 90)) false false))
    (:Finished
      (Rendering|SetActorHiddenInGame _self true)
      (Collision|SetCollisionEnabled (Variables|Default|GetDoor _self) "NoCollision"))))

(event EventOnActivation
  (params (PlayerRef :type BP%20Third%20Person%20Character%20Object%20Reference))
  (|CallParentFunction 0)
  (Variables|Default|SetbIsQuestCompleted (Variables|Default|GetbIsActivated))
  (bind __nextroomref (Variables|Default|Get_NextRoomRef)
    (:then
      (Utilities|AsyncLoadAsset __nextroomref
        (:Completed
          (Default|SpawnRoomSwitcher (Variables|Default|Get_currentRoomRef) __nextroomref))))
    (:else
      (Development|PrintString "DoorNextRoomRef NOT WORKING!"))))

(event EventOnReset
  (bind _seconddoorref (Variables|Default|GetSecondDoorRef))
  (if (not (and (Variables|Default|GetbIsQuestCompleted) (Variables|Default|GetbIsDeathDoor)))
    (|CallParentFunction)
    (if (Variables|/Game/Mechanics/InteractableObjects/BP_Door.BP_Door_C|GetbIsDoorOpen _seconddoorref)
      (Default|OnInteract _seconddoorref)
      (Rendering|SetActorHiddenInGame self false)
      (Collision|SetCollisionEnabled (Variables|Default|GetDoor) "QueryAndPhysics")
      (Transformation|SetRelativeRotation (Variables|Default|GetAnchor) (Math|Rotator|MakeRotator 0.0 0.0 0.0) false false))
    (else
      (Actor|DestroyActor))))

(event EventSaveforReset
  (|CallParentFunction))

(fn ConstructionScript
  (|CallParentFunction))

(fn CreateListOfComponents
  (return 0))