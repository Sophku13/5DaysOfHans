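; Draggable plate quest object that the player slides with the drag input and that breaks after falling off a table.
; A camera trace detects the "Plate" tag and locks the camera, then Tick offsets the mesh from the character's look rates while its Y stays in range.
; A downward trace enables physics over non-"Table" surfaces and arms breakage after a delay.
; The next hit hides the mesh and spawns BP_BreakablePlate_Alt in its place.
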(event OnComponentHit(PlateMesh)
  (params (HitComponent :type Primitive%20Component%20Object%20Reference) (OtherActor :type Actor%20Object%20Reference) (OtherComp :type Primitive%20Component%20Object%20Reference) (NormalImpulse :type Vector :default "0, 0, 0") (Hit :type Hit%20Result%20Structure%20%28by%20ref%29))
  (bind _platemesh (Variables|Default|GetPlateMesh))
  ;[0.4431 0 1] Spawns breakable plate upon collission
  (if (Variables|Default|GetbInAir)
    (Variables|Default|SetBreakablePlateTransform (Transformation|GetWorldTransform (Variables|Default|GetPlateMesh)))
    (Rendering|SetVisibility _platemesh false false)
    (Physics|SetSimulatePhysics _platemesh false)
    (Collision|SetCollisionEnabled _platemesh "NoCollision")
    (Game|SpawnActorfromClass "/Game/Mechanics/MiniGames/MotherRoomMinigame/BP_BreakablePlate_Alt.BP_BreakablePlate_Alt_C" (Variables|Default|GetBreakablePlateTransform) "Undefined" "MultiplyWithRoot" 0 0)))

(event Input|EnhancedActionEvents|EnhancedInputActionIA_DragObjects
  (params (ActionValue :type Boolean) (ElapsedSeconds :type Float%20%28double-precision%29) (TriggeredSeconds :type Float%20%28double-precision%29) (InputAction :type Input%20Action%20Object%20Reference :default "/Game/Character/Input/Actions/IA_DragObjects.IA_DragObjects"))
  ;[0.4431 0 1] Line trace for dragging the object
  (:Started
    (Variables|Default|SetbIsHoldingLMB true)
    (bind _asbp_third_person_character (Utilities|Casting|CastToBP_ThirdPersonCharacter (Game|GetPlayerCharacter 0)))
    (bind (_outhit _returnvalue) (Collision|LineTraceForObjects (Transformation|GetWorldLocation (Variables|/Game/ThirdPerson/Blueprints/BP_ThirdPersonCharacter.BP_ThirdPersonCharacter_C|GetFollowCamera _asbp_third_person_character)) (+ (Transformation|GetWorldLocation (Variables|/Game/ThirdPerson/Blueprints/BP_ThirdPersonCharacter.BP_ThirdPersonCharacter_C|GetFollowCamera _asbp_third_person_character)) (* (Math|Vector|GetForwardVector (Variables|/Game/ThirdPerson/Blueprints/BP_ThirdPersonCharacter.BP_ThirdPersonCharacter_C|GetFollowCamera _asbp_third_person_character)) 5e+02)) (Utilities|Array|MakeArray "ObjectTypeQuery1") false 0 "None" false))
    (if _returnvalue
      (if (== (Utilities|Array|Get(acopy) (Variables|/Script/Engine.ActorComponent|GetComponentTags (.HitComponent (Collision|BreakHitResult _outhit)))) "Plate")
        (Variables|Default|SetbLookingAtPlate true)
        (Variables|/Game/ThirdPerson/Blueprints/BP_ThirdPersonCharacter.BP_ThirdPersonCharacter_C|SetbIsCameraLocked _asbp_third_person_character true)
        (else
          (Variables|Default|SetbLookingAtPlate false :!label _label)))
      (else
        (goto _label))))
  (:Canceled
    (Variables|Default|SetbIsHoldingLMB false :!label _label_2)
    (if (Variables|Default|GetbLookingAtPlate)
      (Variables|/Game/ThirdPerson/Blueprints/BP_ThirdPersonCharacter.BP_ThirdPersonCharacter_C|SetbIsCameraLocked _asbp_third_person_character false)))
  (:Completed
    (goto _label_2)))

(event EventBeginPlay
  (Input|EnableInput (Game|GetPlayerController 0)))

(event EventTick
  (params (DeltaSeconds :type Float%20%28single-precision%29))
  (bind _platemesh (Variables|Default|GetPlateMesh))
  (bind _platemesh_2 (Variables|Default|GetPlateMesh))
  (bind _returnvalue (Transformation|GetWorldLocation _platemesh_2))
  (bind _relativelocation (Variables|/Script/Engine.SceneComponent|GetRelativeLocation _platemesh))
  ;[0.4424 0.000256 1] Handles movement while dragging
  (if (Variables|Default|GetbIsHoldingLMB)
    (if (Variables|Default|GetbLookingAtPlate)
      (if (Math|Float|NearlyEqual(Float) (.y _relativelocation) (Math|Float|ClampAngle (.y _relativelocation) -75.0 3e+01) 0.001)
        (Transformation|AddLocalOffset _platemesh (Math|Vector|MakeVector (* (Variables|/Game/ThirdPerson/Blueprints/BP_ThirdPersonCharacter.BP_ThirdPersonCharacter_C|GetTurnRate (stale Input|EnhancedActionEvents|EnhancedInputActionIA_DragObjects _asbp_third_person_character)) (Variables|Default|GetSensitivity)) (* (Variables|/Game/ThirdPerson/Blueprints/BP_ThirdPersonCharacter.BP_ThirdPersonCharacter_C|GetUpDownRate (stale Input|EnhancedActionEvents|EnhancedInputActionIA_DragObjects _asbp_third_person_character)) (Variables|Default|GetSensitivity)) 0.0) false false)
        ;[0.4431 0 1] Line trace to enable plate physics
        (Development|PrintString (Utilities|String|ToString(Vector) _returnvalue))
        (bind (_outhit _returnvalue_2) (Class|KismetSystemLibrary|LineTraceSinglebyProfile _returnvalue (+ _returnvalue (* (Math|Vector|GetUpVector _platemesh_2) -2e+02)) "BlockAll" false 0 "None" true))
        (if _returnvalue_2
          (Development|PrintString "Hello")
          (if (Utilities|Array|IsEmpty (Variables|/Script/Engine.Actor|GetTags (.HitActor (Collision|BreakHitResult _outhit))))
            (Physics|SetSimulatePhysics (Variables|Default|GetPlateMesh) true :!label _label)
            (Utilities|FlowControl|Delay 1.0)
            (Variables|Default|SetbInAir true)
            (elif (!= (Utilities|Array|Get(acopy) (Variables|/Script/Engine.Actor|GetTags (.HitActor (Collision|BreakHitResult _outhit)))) "Table")
              (goto _label))))))))

(fn ConstructionScript
  (|CallParentFunction))