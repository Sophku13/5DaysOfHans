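; BP_Prolog_Lamp is an interactable pull-chain lamp, filed under quest objects, that toggles its light when used.
; Interaction calls the parent logic and OnActivation, which sets IsActivated, then plays the MovingChain timeline unless IsTurningOn is already set.
; The timeline shifts the chain's relative Z by adding scaled track values to its current position each update.
; On finish, a FlipFlop alternates the light's visibility and the busy flag clears.
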(event EventBeginPlay
  (|CallParentFunction) ; This node is disabled and will not be called.\nDrag off pins to build functionality.
)

(event Collision|EventActorBeginOverlap
  (params (OtherActor :type Actor%20Object%20Reference))
  (|CallParentFunction OtherActor) ; This node is disabled and will not be called.\nDrag off pins to build functionality.
)

(event EventTick
  (params (DeltaSeconds :type Float%20%28single-precision%29))
  (|CallParentFunction DeltaSeconds) ; This node is disabled and will not be called.\nDrag off pins to build functionality.
)

(event EventOnInteract
  (params (PlayerRef :type BP%20Third%20Person%20Character%20Object%20Reference))
  (bind _chain (Variables|Default|GetChain))
  (bind _light (Variables|Default|GetLight))
  (bind _relativelocation (Variables|/Script/Engine.SceneComponent|GetRelativeLocation _chain))
  (|CallParentFunction PlayerRef)
  (CallFunction|OnActivation PlayerRef)
  (if (not (Variables|Default|GetbIsTurningOn))
    (Variables|Default|SetbIsTurningOn true)
    (bind _newtrack_0 (Timeline|MovingChain PlayFromStart)
      (:Update
        (Transformation|SetRelativeLocation _chain (Math|Vector|MakeVector (.x _relativelocation) (.y _relativelocation) (+ (.z _relativelocation) (* _newtrack_0 -1e+01))) false false))
      (:Finished
        (Utilities|FlowControl|FlipFlop
          (:A
            (Rendering|SetVisibility _light true false))
          (:B
            (Rendering|SetVisibility _light false false)))
        (Variables|Default|SetbIsTurningOn false)))))

(event EventOnActivation
  (params (PlayerRef :type BP%20Third%20Person%20Character%20Object%20Reference))
  (Variables|Default|SetbIsActivated true))

(fn ConstructionScript
  (|CallParentFunction))