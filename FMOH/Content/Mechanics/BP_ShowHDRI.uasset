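; BP_ShowHDRI is a trigger volume that reveals the skylight of a referenced HDRI actor.
; When something begins overlapping its box while that skylight is hidden in game, it unhides the skylight and clears a hidden-state flag.
; It then disables the box's collision so it fires once, until OnReset restores query-only collision.
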(event OnComponentBeginOverlap(Box)
  (params (OverlappedComponent :type Primitive%20Component%20Object%20Reference) (OtherActor :type Actor%20Object%20Reference) (OtherComp :type Primitive%20Component%20Object%20Reference) (OtherBodyIndex :type Integer) (bFromSweep :type Boolean) (SweepResult :type Hit%20Result%20Structure%20%28by%20ref%29))
  (if (Variables|/Script/Engine.SceneComponent|GetbHiddenInGame (Variables|/HDRIBackdrop/Blueprints/HDRIBackdrop.HDRIBackdrop_C|GetSkylight (Variables|Default|GetHDRIRef)))
    (Development|SetHiddeninGame (Variables|/HDRIBackdrop/Blueprints/HDRIBackdrop.HDRIBackdrop_C|GetSkylight (Variables|Default|GetHDRIRef)) false false)
    (Variables|Default|SetbisHDRIHidden false)
    (Collision|SetCollisionEnabled (Variables|Default|GetBox) "NoCollision")))

(event EventBeginPlay
  (|CallParentFunction) ; This node is disabled and will not be called.\nDrag off pins to build functionality.
)

(event Collision|EventActorBeginOverlap
  (params (OtherActor :type Actor%20Object%20Reference)))

(event EventTick
  (params (DeltaSeconds :type Float%20%28single-precision%29)))

(event EventOnReset
  (Collision|SetCollisionEnabled (Variables|Default|GetBox) "QueryOnly"))

(fn ConstructionScript
  (|CallParentFunction))