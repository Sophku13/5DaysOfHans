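; Chapter manager actor that tracks story progress, current chapter and current room, and restores them on BeginPlay.
; With a saved room, it loads progress from the GameInstance, re-applies completed quest items' flags and transforms, and streams in that room's level.
; Otherwise it streams the first corridor level and async-loads StartingRoom as the current room.
; ResetRoom resets the given room and saves progress through the GameInstance.
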(event Custom|ResetRoom
  (params (ResetRoom :type BP%20Room%20Object%20Reference))
  (Default|ResetRoom ResetRoom)
  (bind _progresssave (CallFunction|SaveProgress))
  (Class|BPISaveGame|SaveRoomProgress(Message) (Game|GetGameInstance) false _progresssave))

(event Custom|LoadData
  (bind _returnvalue (Game|GetGameInstance))
  (bind __startingroom (Variables|Default|Get_StartingRoom))
  (bind _gamesave (Class|BPISaveGame|GetGameData(Message) _returnvalue))
  (if (Utilities|IsValidSoftObjectReference (.currentroom (Variables|/Game/Mechanics/LoadSaveGame/BP_SaveGame.BP_SaveGame_C|GetChapterManagerSave _gamesave)))
    (bind _chaptermanagergamedata (Class|BPISaveGame|GetChapterManagerGameData(Message) _returnvalue))
    (CallFunction|LoadProgress _chaptermanagergamedata (Variables|/Game/Mechanics/LoadSaveGame/BP_SaveGame.BP_SaveGame_C|GetCompletedQuestItemList _gamesave))
    (Game|LoadStreamLevel(byName) (Variables|Default|GetCurrentRoomName) true true)
    (else
      (Game|LoadStreamLevel(byName) "FMOH_Corridor_0" true true)
      (Utilities|AsyncLoadAsset __startingroom
        (:Completed
          (Variables|Default|SetcurrentRoom __startingroom)
          (Utilities|Array|AddUnique (Variables|Default|GetStoryProgress) (Variables|/Game/Mechanics/BaseBlueprints/BP_Room.BP_Room_C|Get_RoomName (Utilities|ResolveSoftReference __startingroom))))))))

(event EventBeginPlay
  (bind _returnvalue (Game|GetGameInstance))
  (bind __startingroom (Variables|Default|Get_StartingRoom))
  (bind _gamesave (Class|BPISaveGame|GetGameData(Message) _returnvalue))
  (if (Utilities|IsValidSoftObjectReference (.currentroom (Variables|/Game/Mechanics/LoadSaveGame/BP_SaveGame.BP_SaveGame_C|GetChapterManagerSave _gamesave)))
    (bind _chaptermanagergamedata (Class|BPISaveGame|GetChapterManagerGameData(Message) _returnvalue))
    (CallFunction|LoadProgress _chaptermanagergamedata (Variables|/Game/Mechanics/LoadSaveGame/BP_SaveGame.BP_SaveGame_C|GetCompletedQuestItemList _gamesave))
    (Game|LoadStreamLevel(byName) (Variables|Default|GetCurrentRoomName) true true)
    (else
      (Game|LoadStreamLevel(byName) "FMOH_Corridor_0" true true)
      (Utilities|AsyncLoadAsset __startingroom
        (:Completed
          (Variables|Default|SetcurrentRoom __startingroom)
          (Utilities|Array|AddUnique (Variables|Default|GetStoryProgress) (Variables|/Game/Mechanics/BaseBlueprints/BP_Room.BP_Room_C|Get_RoomName (Utilities|ResolveSoftReference __startingroom))))))))

(event Collision|EventActorBeginOverlap
  (params (OtherActor :type Actor%20Object%20Reference)))

(event EventTick
  (params (DeltaSeconds :type Float%20%28single-precision%29)))

(fn ConstructionScript)

(fn LoadStart
  (params (StartRoom :type BP%20Room%20Switcher%20Object%20Reference) (StartChapter :type BP%20Chapter%20Object%20Reference)))

(fn SaveProgress
  (return (Utilities|Struct|MakeS_ChapterManagerSave (Variables|Default|GetStoryProgress) (Variables|Default|GetcurrentChapter) (Variables|Default|GetcurrentRoom) (Variables|Default|GetCurrentRoomName) (Variables|Default|GetChapterList))))

(fn LoadProgress
  (params (ProgressSave :type S%20Chapter%20Manager%20Save%20Structure) (QuestItemList :type Map%20of%20BP%20Base%20Quest%20Item%20Object%20References%20to%20Structs))
  (Variables|Default|SetStoryProgress (.storyprogress ProgressSave))
  (Variables|Default|SetcurrentChapter (.currentchapter ProgressSave))
  (Variables|Default|SetcurrentRoom (.currentroom ProgressSave))
  (Variables|Default|SetCurrentRoomName (.currentroomname ProgressSave))
  (Variables|Default|SetChapterList (.chapterlist ProgressSave))
  (bind _keys (Utilities|Map|Keys QuestItemList))
  (for _array_element _keys
    (Variables|/Game/Mechanics/BaseBlueprints/BP_BaseQuestItem.BP_BaseQuestItem_C|SetbIsQuestCompleted _array_element true)
    (Transformation|SetActorTransform _array_element (.Value (Utilities|Map|Find QuestItemList _array_element)) false true)))