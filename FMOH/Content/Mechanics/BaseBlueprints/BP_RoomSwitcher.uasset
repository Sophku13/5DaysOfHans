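; Portal actor that moves the player between rooms and advances chapter progress.
; LoadNext async-loads the next room's view material onto the portal mesh and can open a paused teleport-choice widget.
; Box overlap or TeleportToNextLevel teleports the character, suppressing camera lag, then resets the current room, updates BP_ChapterManager and saves.
; While active, Tick rotates the next switcher's PortalView with the player camera, keeping the portal image aligned.
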(event OnComponentBeginOverlap(Box)
  (params (OverlappedComponent :type Primitive%20Component%20Object%20Reference) (OtherActor :type Actor%20Object%20Reference) (OtherComp :type Primitive%20Component%20Object%20Reference) (OtherBodyIndex :type Integer) (bFromSweep :type Boolean) (SweepResult :type Hit%20Result%20Structure%20%28by%20ref%29))
  (bind _returnvalue (Game|GetPlayerController 0))
  (bind _nextroomtoload (Variables|Default|GetNextRoomToLoad))
  (bind _controlrotationvalue (Variables|Default|GetcontrolRotationValue))
  (bind _output (Utilities|ResolveSoftReference _nextroomtoload))
  (bind _teleportlocation (Variables|/Game/Mechanics/BaseBlueprints/BP_Room.BP_Room_C|GetTeleportLocation _output))
  (bind _teleportlocation_2 (Variables|/Game/Mechanics/BaseBlueprints/BP_Room.BP_Room_C|GetTeleportLocation _output))
  (bind _returnvalue_2 (Transformation|GetWorldRotation _teleportlocation))
  (bind _returnvalue_3 (Transformation|GetWorldRotation _teleportlocation_2))
  (bind _returnvalue_4 (+ (.yaw _returnvalue_3) _controlrotationvalue))
  (bind _returnvalue_5 (Math|Rotator|MakeRotator 0.0 0.0 _returnvalue_4))
  ;[1 1 1] Teleportation through Portal Frames
  (bind _asbp_third_person_character (Utilities|Casting|CastToBP_ThirdPersonCharacter OtherActor)
    (:then
      (bind _output_get (Variables|Default|SetCharacterRef _asbp_third_person_character))
      (Variables|/Script/Engine.SpringArmComponent|SetbEnableCameraRotationLag (Variables|/Game/ThirdPerson/Blueprints/BP_ThirdPersonCharacter.BP_ThirdPersonCharacter_C|GetCameraBoom (Variables|Default|GetCharacterRef)) false :!label _label)
      (Utilities|AsyncLoadAsset _nextroomtoload :!label _label_2
        (:Completed
          (Variables|Default|SetbCanTeleport false)
          (Transformation|SetActorLocationAndRotation _output_get (Transformation|GetWorldLocation _teleportlocation_2) _returnvalue_5 false true)
          (Audio|PlaySoundatLocation (Variables|Default|GetSound) (.location (Transformation|GetActorTransform _output_get)) (.rotation (Transformation|GetActorTransform _output_get)) 1.0 1.0 0.0 0 0 0 0)
          (if (Variables|/Game/ThirdPerson/Blueprints/BP_ThirdPersonCharacter.BP_ThirdPersonCharacter_C|GetbIsInProlog _output_get)
            (Transformation|SetActorTransform (Variables|Default|GetCharacterRef) (Math|Transform|MakeTransform (Transformation|GetWorldLocation _teleportlocation) _returnvalue_2 "0.800000,0.800000,0.800000") false true)
            (Pawn|SetControlRotation _returnvalue _returnvalue_2)
            (Pawn|Possess _returnvalue (Variables|Default|GetCharacterRef))
            (CallFunction|UpdateChapterManager)
            (Variables|Default|SetbCanTeleport true)
            (Variables|Default|SetbIsActive false)
            (Variables|/Game/ThirdPerson/Blueprints/BP_ThirdPersonCharacter.BP_ThirdPersonCharacter_C|SetbIsCameraLocked (Variables|Default|GetCharacterRef) false)
            (Variables|/Game/ThirdPerson/Blueprints/BP_ThirdPersonCharacter.BP_ThirdPersonCharacter_C|SetIsMovementLocked (Variables|Default|GetCharacterRef) false)
            (Variables|/Game/ThirdPerson/Blueprints/BP_ThirdPersonCharacter.BP_ThirdPersonCharacter_C|SetbIsInProlog (Variables|Default|GetCharacterRef) false)
            (Variables|/Game/ThirdPerson/Blueprints/BP_ThirdPersonCharacter.BP_ThirdPersonCharacter_C|SetFirstPersonCameraREF (Variables|Default|GetCharacterRef) (Variables|/Game/ThirdPerson/Blueprints/BP_ThirdPersonCharacter.BP_ThirdPersonCharacter_C|GetFollowCamera (Variables|Default|GetCharacterRef)))
            (Variables|/Game/ThirdPerson/Blueprints/BP_ThirdPersonCharacter.BP_ThirdPersonCharacter_C|SetbInUIMode (Variables|Default|GetCharacterRef) false)
            (Utilities|FlowControl|Delay 1.0)
            (Variables|/Script/Engine.SpringArmComponent|SetbEnableCameraRotationLag (Variables|/Game/ThirdPerson/Blueprints/BP_ThirdPersonCharacter.BP_ThirdPersonCharacter_C|GetCameraBoom (Variables|Default|GetCharacterRef)) true)
            (else
              (if (Variables|Default|GetbIsRotationNeeded)
                (Pawn|SetControlRotation (Game|GetPlayerController 0) _returnvalue_5))
              (CallFunction|UpdateChapterManager)
              (if (== (Variables|/Game/Mechanics/BaseBlueprints/BP_Room.BP_Room_C|Get_RoomName (Variables|Default|GetNextRoom)) "FMOH_Room_1_1")
                (Transformation|SetActorTransform _output_get (Math|Transform|MakeTransform (.location (Transformation|GetActorTransform _output_get)) _returnvalue_5 "0.800000,0.800000,0.800000") false true)
                (else
                  (Transformation|SetActorTransform _output_get (Math|Transform|MakeTransform (.location (Transformation|GetActorTransform _output_get)) _returnvalue_5 "1.000000,1.000000,1.000000") false true)))
              (Variables|Default|SetbCanTeleport true)
              (Variables|Default|SetbIsActive false)
              (Variables|/Game/ThirdPerson/Blueprints/BP_ThirdPersonCharacter.BP_ThirdPersonCharacter_C|SetbIsCameraLocked (Variables|Default|GetCharacterRef) false)
              (Variables|/Game/ThirdPerson/Blueprints/BP_ThirdPersonCharacter.BP_ThirdPersonCharacter_C|SetIsMovementLocked (Variables|Default|GetCharacterRef) false)
              (Variables|/Game/ThirdPerson/Blueprints/BP_ThirdPersonCharacter.BP_ThirdPersonCharacter_C|SetbIsInProlog (Variables|Default|GetCharacterRef) false)
              (Utilities|FlowControl|Delay 1.0)
              (Variables|/Script/Engine.SpringArmComponent|SetbEnableCameraRotationLag (Variables|/Game/ThirdPerson/Blueprints/BP_ThirdPersonCharacter.BP_ThirdPersonCharacter_C|GetCameraBoom (Variables|Default|GetCharacterRef)) true))))))
    (:CastFailed
      (if (Variables|Default|GetbCanTeleport)
        (Variables|Default|GetCharacterRef
          (:then
            (goto _label))
          (:else
            (goto _label_2)))))))

(event Custom|LoadNext
  (params (NextRoomToLoad :type BP%20Room%20Soft%20Object%20Reference))
  (bind _returnvalue (Game|GetPlayerController 0))
  (bind _output (Utilities|ResolveSoftReference NextRoomToLoad))
  (bind __cameraview (Variables|/Game/Mechanics/BaseBlueprints/BP_Room.BP_Room_C|Get_CameraView _output))
  ;[1 1 1] Comment
  (bind _asbp_third_person_character (Utilities|Casting|CastToBP_ThirdPersonCharacter (Game|GetPlayerCharacter 0))
    (:then
      (Variables|Default|SetCharacterRef _asbp_third_person_character))
    (:CastFailed
      _))
  (bind _output_get (Variables|Default|SetNextRoomToLoad NextRoomToLoad))
  (Utilities|AsyncLoadAsset __cameraview
    (:Completed
      (bind _output_get_2 (Variables|Default|SetNextRoom (Utilities|ResolveSoftReference _output_get)))
      (CallFunction|SpawnPortal (Utilities|ResolveSoftReference __cameraview))
      (Variables|Default|SetbIsActive true)
      (Variables|Default|SetNextRoomSwitcher (Variables|/Game/Mechanics/BaseBlueprints/BP_Room.BP_Room_C|Get_roomSwitcher _output_get_2))
      (if (Variables|Default|GetbIsRoom)
        (Variables|Default|GetTeleportFrameRef
          (:then
            (bind _characterref (Variables|Default|GetCharacterRef)
              (:then
                (Default|CloseEyes _characterref 1.0)
                (Utilities|FlowControl|Delay 2.0)
                (Game|SetGamePaused true)
                (bind _returnvalue_2 (UserInterface|CreateWidget "/Game/UI/WBP_TeleportChoice.WBP_TeleportChoice_C" 0 self))
                (UserInterface|Viewport|AddtoViewport _returnvalue_2 1)
                (Variables|/Script/Engine.PlayerController|SetbShowMouseCursor _returnvalue true)
                (Input|SetInputModeUIOnly _returnvalue 0 "DoNotLock" false))
              (:else)))
          (:else))))))

(event Custom|UpdateChapterManager
  (bind _nextroomtoload (Variables|Default|GetNextRoomToLoad))
  (bind _output (Utilities|ResolveSoftReference _nextroomtoload))
  (bind __roomname (Variables|/Game/Mechanics/BaseBlueprints/BP_Room.BP_Room_C|Get_RoomName _output))
  ;[1 1 1] Comment
  (Default|ResetRoom (Variables|Default|GetCurrentRoomRef))
  (bind _returnvalue (Actor|GetActorOfClass "/Game/Mechanics/BaseBlueprints/BP_ChapterManager.BP_ChapterManager_C"))
  (if (or (== (Variables|/Game/Mechanics/BaseBlueprints/BP_Room.BP_Room_C|GetcurrentChapter (Variables|Default|GetCurrentRoomRef)) 5) (== (Variables|/Game/Mechanics/BaseBlueprints/BP_Room.BP_Room_C|GetcurrentChapter (Variables|Default|GetCurrentRoomRef)) 0))
    (Variables|/Game/Mechanics/BaseBlueprints/BP_ChapterManager.BP_ChapterManager_C|SetcurrentChapter _returnvalue 1)
    (else
      (Variables|/Game/Mechanics/BaseBlueprints/BP_ChapterManager.BP_ChapterManager_C|SetcurrentChapter _returnvalue (+ (Variables|/Game/Mechanics/BaseBlueprints/BP_Room.BP_Room_C|GetcurrentChapter (Variables|Default|GetCurrentRoomRef)) 1))))
  (Utilities|AsyncLoadAsset _nextroomtoload
    (:Completed
      (Variables|/Game/Mechanics/BaseBlueprints/BP_ChapterManager.BP_ChapterManager_C|SetcurrentRoom _returnvalue _nextroomtoload)
      (Variables|/Game/Mechanics/BaseBlueprints/BP_ChapterManager.BP_ChapterManager_C|SetCurrentRoomName _returnvalue __roomname)
      (Utilities|Array|AddUnique (Variables|/Game/Mechanics/BaseBlueprints/BP_ChapterManager.BP_ChapterManager_C|GetStoryProgress _returnvalue) __roomname)
      (CallFunction|SaveProgress))))

(event Custom|Reset
  ;[1 1 1] Comment
  (bind __portaldoor (Variables|Default|Get_PortalDoor)
    (:then
      (Variables|/Game/Mechanics/QuestObjects/BP_Portal_Door_Base.BP_Portal_Door_Base_C|SetbCanBeOpened __portaldoor false))
    (:else
      _))
  (Development|SetHiddeninGame (Variables|Default|GetPortalMesh) true false)
  (Variables|/Script/Engine.PrimitiveComponent|SetbGenerateOverlapEvents (Variables|Default|GetBox) false))

(event Custom|SaveProgress
  (bind _returnvalue (Game|GetGameInstance))
  ;[1 1 1] SaveProgress
  (Utilities|FlowControl|Delay 1.0)
  (bind _asbp_third_person_character (Utilities|Casting|CastToBP_ThirdPersonCharacter (Game|GetPlayerCharacter 0)))
  (bind _output_get (Variables|Default|SetCharacterRef _asbp_third_person_character))
  (bind _playersave (Default|GetPlayerSaveData _output_get))
  (Class|BPISaveGame|SavePlayer(Message) _returnvalue false _playersave)
  (bind _returnvalue_2 (Actor|GetActorOfClass "/Game/Mechanics/BaseBlueprints/BP_ChapterManager.BP_ChapterManager_C"))
  (bind _progresssave (Default|SaveProgress _returnvalue_2))
  (Class|BPISaveGame|SaveRoomProgress(Message) _returnvalue false _progresssave)
  (for _array_element (Variables|/Game/Mechanics/BaseBlueprints/BP_Room.BP_Room_C|Get_QuestItemList (Variables|Default|GetCurrentRoomRef))
    (Default|SaveCompletedQuestItem _array_element)))

(event Custom|TeleportToNextLevel
  (bind _controlrotationvalue (Variables|Default|GetcontrolRotationValue))
  (bind _nextroomtoload (Variables|Default|GetNextRoomToLoad))
  (bind _output (Utilities|ResolveSoftReference _nextroomtoload))
  (bind _teleportlocation (Variables|/Game/Mechanics/BaseBlueprints/BP_Room.BP_Room_C|GetTeleportLocation _output))
  (bind _returnvalue (Transformation|GetWorldRotation _teleportlocation))
  (bind _returnvalue_2 (+ (.yaw _returnvalue) _controlrotationvalue))
  (bind _returnvalue_3 (Math|Rotator|MakeRotator 0.0 0.0 _returnvalue_2))
  ;[0 1 0.4424] Prepared for implementation
  (bind _asbp_third_person_character (Utilities|Casting|CastToBP_ThirdPersonCharacter (Game|GetPlayerCharacter 0)))
  (Variables|Default|SetCharacterRef _asbp_third_person_character)
  (Variables|/Script/Engine.SpringArmComponent|SetbEnableCameraRotationLag (Variables|/Game/ThirdPerson/Blueprints/BP_ThirdPersonCharacter.BP_ThirdPersonCharacter_C|GetCameraBoom (Variables|Default|GetCharacterRef)) false)
  (Utilities|AsyncLoadAsset _nextroomtoload
    (:Completed
      (Variables|Default|SetbCanTeleport false)
      (Transformation|SetActorTransform (Variables|Default|GetCharacterRef) (Math|Transform|MakeTransform (Transformation|GetWorldLocation _teleportlocation) _returnvalue_3 "1.000000,1.000000,1.000000") false true)
      (Audio|PlaySoundatLocation (Variables|Default|GetSound) (.location (Transformation|GetActorTransform (Variables|Default|GetCharacterRef))) (.rotation (Transformation|GetActorTransform (Variables|Default|GetCharacterRef))) 1.0 1.0 0.0 0 0 0 0)
      (if (Variables|Default|GetbIsRotationNeeded)
        (Pawn|SetControlRotation (Game|GetPlayerController 0) _returnvalue_3))
      (CallFunction|UpdateChapterManager)
      (Default|OpenEyes (Variables|Default|GetCharacterRef) 1.0)
      (Variables|Default|SetbCanTeleport true)
      (Variables|Default|SetbIsActive false)
      (Variables|/Game/ThirdPerson/Blueprints/BP_ThirdPersonCharacter.BP_ThirdPersonCharacter_C|SetbIsCameraLocked (Variables|Default|GetCharacterRef) false)
      (Variables|/Game/ThirdPerson/Blueprints/BP_ThirdPersonCharacter.BP_ThirdPersonCharacter_C|SetIsMovementLocked (Variables|Default|GetCharacterRef) false)
      (Variables|/Game/ThirdPerson/Blueprints/BP_ThirdPersonCharacter.BP_ThirdPersonCharacter_C|SetbIsInProlog (Variables|Default|GetCharacterRef) false)
      (Utilities|FlowControl|Delay 1.0)
      (Variables|/Script/Engine.SpringArmComponent|SetbEnableCameraRotationLag (Variables|/Game/ThirdPerson/Blueprints/BP_ThirdPersonCharacter.BP_ThirdPersonCharacter_C|GetCameraBoom (Variables|Default|GetCharacterRef)) true))))

(event EventBeginPlay
  (bind __portaldoor (Variables|Default|Get_PortalDoor)
    (:then
      (Variables|/Game/Mechanics/QuestObjects/BP_Portal_Door_Base.BP_Portal_Door_Base_C|SetbCanBeOpened __portaldoor true))
    (:else)))

(event EventTick
  (params (DeltaSeconds :type Float%20%28single-precision%29))
  (bind _returnvalue (Game|GetPlayerCameraManager 0))
  (bind _nextroomswitcher (Variables|Default|GetNextRoomSwitcher))
  (bind _transformcomponent (Variables|/Script/Engine.PlayerCameraManager|GetTransformComponent _returnvalue))
  (bind _portalview (Variables|BP_RoomSwitcher_C|GetPortalView _nextroomswitcher))
  (bind _returnvalue_2 (Transformation|GetWorldLocation _portalview))
  ;[1 1 1] Portal Image is moving aligned with the player in Portall 1
  (if (Variables|Default|GetbIsActive)
    (if (Variables|Default|GetbNotRotatingCamera)
      (Transformation|SetWorldLocationAndRotation _portalview _returnvalue_2 (Transformation|GetWorldRotation _transformcomponent) false false)
      (else
        (Transformation|SetWorldLocationAndRotation _portalview _returnvalue_2 (Math|Rotator|CombineRotators (Math|Rotator|MakeRotator 0.0 0.0 (.yaw (Transformation|GetWorldRotation _transformcomponent))) (Variables|/Script/Engine.SceneComponent|GetRelativeRotation (Variables|/Game/Mechanics/BaseBlueprints/BP_Room.BP_Room_C|GetTeleportLocation (Variables|BP_RoomSwitcher_C|GetCurrentRoomRef _nextroomswitcher)))) false false)))))

(fn ConstructionScript)

(fn UnloadPrev
  (params (ChapterManager :type BP%20Chapter%20Manager%20Object%20Reference) (PrevRoom :type BP%20Room%20Object%20Reference)))

(fn SpawnPortal
  (params (Portal%20Visual :type Material%20Object%20Reference))
  (Rendering|Material|SetMaterial (Variables|Default|GetPortalMesh) 0 Portal%20Visual)
  (Variables|Default|SetbCanTeleport true)
  (Development|SetHiddeninGame (Variables|Default|GetPortalMesh) false false)
  (Variables|/Script/Engine.PrimitiveComponent|SetbGenerateOverlapEvents (Variables|Default|GetBox) true)
  (bind __portaldoor (Variables|Default|Get_PortalDoor)
    (:then
      (Variables|/Game/Mechanics/QuestObjects/BP_Portal_Door_Base.BP_Portal_Door_Base_C|SetbCanBeOpened __portaldoor true))
    (:else)))