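; Base interactable drop-off spot for a quest item, shown as the item's mesh with a silhouette material.
; On interact, if the player is carrying an item and the referenced quest item is picked up, it places that item at the saved mesh transform, hides itself, disables mesh collision and plays a sound.
; The transform is saved on BeginPlay; the reset handler checks quest completion but takes no action.
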(event EventBeginPlay
  (|CallParentFunction)
  (CallFunction|SaveforReset)
  (Transformation|SetWorldTransform (Variables|Default|GetQuestItemMesh) (Variables|Default|GetObjectLocation) false false))

(event EventOnReset
  (if (Variables|/Game/Mechanics/BaseBlueprints/BP_BaseQuestItem.BP_BaseQuestItem_C|GetbIsQuestCompleted (Variables|Default|GetQuestItemRef))
    _))

(event EventSaveforReset
  (Variables|Default|SetObjectLocation (Transformation|GetWorldTransform (Variables|Default|GetQuestItemMesh))))

(event EventOnInteract
  (params (PlayerRef :type BP%20Third%20Person%20Character%20Object%20Reference))
  (if (and (Variables|/Game/ThirdPerson/Blueprints/BP_ThirdPersonCharacter.BP_ThirdPersonCharacter_C|GetbIsCarryingItem PlayerRef) (Variables|/Game/Mechanics/QuestObjects/BP_BaseQuestPickUpItem.BP_BaseQuestPickUpItem_C|GetbIsPickedUp (Variables|Default|GetQuestItemRef)))
    (Default|PlaceinQuestLocation (Variables|Default|GetQuestItemRef) (Variables|Default|GetObjectLocation))
    (Rendering|SetActorHiddenInGame self true)
    (Collision|SetCollisionEnabled (Variables|Default|GetQuestItemMesh) "NoCollision")
    (Audio|PlaySound2D "/Game/SoundSystem/Sounds/SFX/Actions/PlaceObject.PlaceObject" 1.0 1.0 0.0 0 0)))

(fn ConstructionScript
  (|CallParentFunction)
  (Components|StaticMesh|SetStaticMesh (Variables|Default|GetQuestItemMesh) (Variables|Default|GetstaticMesh_QuestItem))
  (Rendering|Material|SetMaterial (Variables|Default|GetQuestItemMesh) 0 (Variables|Default|GetSillohueteMaterial)))

(fn CreateListOfComponents
  (bind _static_mesh_array (Variables|Default|GetStatic%20Mesh%20Array))
  (Utilities|Array|Add _static_mesh_array (Variables|Default|GetQuestItemMesh))
  (return _static_mesh_array))