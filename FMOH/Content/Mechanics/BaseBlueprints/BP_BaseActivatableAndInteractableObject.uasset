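; Base Blueprint for activatable and interactable objects that can be reset to their starting state.
; BeginPlay calls SaveForReset, which stores the root component's world transform.
; OnActivation toggles the IsActivated flag, while OnInteract is an empty event.
; OnReset teleports the actor to the saved location and rotation and clears IsActivated.
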(event EventBeginPlay
  (CallFunction|SaveforReset))

(event Collision|EventActorBeginOverlap
  (params (OtherActor :type Actor%20Object%20Reference)))

(event EventTick
  (params (DeltaSeconds :type Float%20%28single-precision%29)))

(event EventOnInteract
  (params (PlayerRef :type BP%20Third%20Person%20Character%20Object%20Reference)))

(event EventOnActivation
  (params (PlayerRef :type BP%20Third%20Person%20Character%20Object%20Reference))
  (if (Variables|Default|GetbIsActivated)
    (Variables|Default|SetbIsActivated false)
    (else
      (Variables|Default|SetbIsActivated true))))

(event EventSaveforReset
  (Variables|Default|SetStartingLocation (Transformation|GetWorldTransform (Variables|Default|GetDefaultSceneRoot self))))

(event EventOnReset
  (bind _startinglocation (Variables|Default|GetStartingLocation))
  (Transformation|SetActorLocationAndRotation self (.location _startinglocation) (.rotation _startinglocation) false true)
  (Variables|Default|SetbIsActivated false))

(fn ConstructionScript)