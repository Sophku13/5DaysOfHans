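; Prototype quest button that, on interaction, marks quest completion and opens the way to the next room.
; OnInteract calls OnActivation, then briefly lowers and raises the button mesh with down and up sounds.
; OnActivation runs parent logic, copies IsActivated into IsQuestCompleted, async-loads NextRoomRef and has the current room spawn a room switcher for it.
; An invalid room reference only prints an error.
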(event EventBeginPlay
  ;[1 1 1] Comment
  (|CallParentFunction))

(event EventOnActivation
  (params (PlayerRef :type BP%20Third%20Person%20Character%20Object%20Reference))
  ;[1 1 1] Comment
  (|CallParentFunction PlayerRef)
  (Variables|Default|SetbIsQuestCompleted (Variables|Default|GetbIsActivated))
  (bind __nextroomref (Variables|Default|Get_NextRoomRef)
    (:then
      (Utilities|AsyncLoadAsset __nextroomref
        (:Completed
          (Default|SpawnRoomSwitcher (Variables|Default|Get_currentRoomRef) __nextroomref))))
    (:else
      (Development|PrintString "ButtonNextRoomRef NOT WORKING!"))))

(event EventOnInteract
  (params (PlayerRef :type BP%20Third%20Person%20Character%20Object%20Reference))
  (bind _button (Variables|Default|GetButton))
  (bind _button_2 (Variables|Default|GetButton))
  ;[1 1 1] Comment
  (CallFunction|OnActivation PlayerRef)
  (Transformation|SetWorldLocation _button_2 (- (Transformation|GetWorldLocation _button_2) "0.000000,0.000000,5.000000") false false)
  (Audio|PlaySoundatLocation "/Game/SoundSystem/Sounds/Buttons/SC_ButtonDown_Cue.SC_ButtonDown_Cue" "0, 0, 0" "0, 0, 0" 1.0 1.0 0.0 0 0 0 0)
  (Utilities|FlowControl|Delay 1.0)
  (Audio|PlaySoundatLocation "/Game/SoundSystem/Sounds/Buttons/SC_ButtonUp_Cue.SC_ButtonUp_Cue" "0, 0, 0" "0, 0, 0" 1.0 1.0 0.0 0 0 0 0)
  (Transformation|SetWorldLocation _button (+ (Transformation|GetWorldLocation _button) "0.000000,0.000000,5.000000") false false))

(fn ConstructionScript
  (|CallParentFunction))