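; Base Blueprint for quest items, layered on a parent that supplies interaction, activation and reset events.
; Most events pass straight to the parent; reset also clears the quest completion flag.
; SaveCompletedQuestItem sends completed items, with their transform, to the Game Instance through an interface message for saving.
; CreateListOfComponents is an empty stub here.
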(event EventBeginPlay
  (|CallParentFunction))

(event Collision|EventActorBeginOverlap
  (params (OtherActor :type Actor%20Object%20Reference))
  (|CallParentFunction OtherActor) ; This node is disabled and will not be called.\nDrag off pins to build functionality.
)

(event EventTick
  (params (DeltaSeconds :type Float%20%28single-precision%29))
  (|CallParentFunction DeltaSeconds) ; This node is disabled and will not be called.\nDrag off pins to build functionality.
)

(event EventOnInteract
  (params (PlayerRef :type BP%20Third%20Person%20Character%20Object%20Reference))
  (|CallParentFunction PlayerRef))

(event EventOnActivation
  (params (PlayerRef :type BP%20Third%20Person%20Character%20Object%20Reference))
  (|CallParentFunction PlayerRef))

(event EventOnReset
  (|CallParentFunction)
  (Variables|Default|SetbIsQuestCompleted false))

(event EventSaveforReset
  (|CallParentFunction))

(fn ConstructionScript
  (|CallParentFunction))

(fn SaveCompletedQuestItem
  (bind _self self)
  (if (Variables|Default|GetbIsQuestCompleted)
    (Class|BPISaveGame|SaveQuestItems(Message) (Game|GetGameInstance) false _self (Transformation|GetActorTransform _self))))

(fn CreateListOfComponents
  (return 0))