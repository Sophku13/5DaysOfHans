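; Base room Blueprint that registers itself with the Room Switcher, tints its lights and triggers the move to the next room.
; On BeginPlay it async-loads the soft-referenced switcher, sets itself as current room and applies the room colour to the point lights in ChangingColours.
; SpawnRoomSwitcher, commented as firing on quest completion, async-loads the switcher and calls LoadNext with the given room.
; The LoadLevelTest level-streaming graph never runs.
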(event Custom|SpawnRoomSwitcher
  (params (nextRoomToLoad :type BP%20Room%20Soft%20Object%20Reference))
  (bind __roomswitcher (Variables|Default|Get_roomSwitcher))
  ;[0.1216 0.902 0.6627] Spawns the Room Switcher when Quest is done
  (Utilities|AsyncLoadAsset __roomswitcher
    (:Completed
      (Default|LoadNext (Utilities|ResolveSoftReference __roomswitcher) nextRoomToLoad))))

(event EventBeginPlay
  (bind __roomswitcher (Variables|Default|Get_roomSwitcher))
  (Utilities|AsyncLoadAsset __roomswitcher
    (:Completed
      (Variables|/Game/Mechanics/BaseBlueprints/BP_RoomSwitcher.BP_RoomSwitcher_C|SetCurrentRoomRef (Utilities|ResolveSoftReference __roomswitcher) self)
      (for _array_element (Variables|Default|Get_ChangingColours)
        (Rendering|Components|Light|SetLightColor (Variables|/Script/Engine.PointLight|GetPointLightComponent _array_element) (Variables|Default|GetRoomLightColor) true)))))

(fn ConstructionScript)