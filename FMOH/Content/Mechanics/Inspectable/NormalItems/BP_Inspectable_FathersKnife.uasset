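; BP_Inspectable_FathersKnife is the inspectable father's knife, which can unlock a dialog option in the parents-fighting minigame.
; On interact it runs the parent logic, plays 2D sounds around a short delay, then spawns BP_InterMono at the player with the item's sound and subtitle.
; If AreParentsFighting is set, it adds "Hurt" to BP_ParentsFightingMinigame's DialogOptionList and clears the flag, so this happens once.
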(event EventBeginPlay
  (|CallParentFunction) ; This node is disabled and will not be called.\nDrag off pins to build functionality.
)

(event Collision|EventActorBeginOverlap
  (params (OtherActor :type Actor%20Object%20Reference))
  (|CallParentFunction OtherActor) ; This node is disabled and will not be called.\nDrag off pins to build functionality.
)

(event EventTick
  (params (DeltaSeconds :type Float%20%28single-precision%29))
  (|CallParentFunction DeltaSeconds) ; This node is disabled and will not be called.\nDrag off pins to build functionality.
)

(event EventOnInteract
  (params (PlayerRef :type BP%20Third%20Person%20Character%20Object%20Reference))
  (|CallParentFunction PlayerRef)
  (Audio|SpawnSound2D 0 1.0 1.0 0.0 0)
  (Utilities|FlowControl|Delay 0.5)
  (Audio|PlaySound2D 0 1.0 1.0 0.0 0 0)
  (bind _returnvalue (Game|SpawnActorfromClass "/Game/SoundSystem/Sounds/BP_InterMono.BP_InterMono_C" (Transformation|GetActorTransform (Game|GetPlayerCharacter 0)) "Undefined" "MultiplyWithRoot" 0 (Variables|Default|GetSound) 1.0 (Variables|Default|GetSubtitle%20Text) 1.0 true 0))
  (Default|CheckValues _returnvalue)
  (if (Variables|Default|GetbAreParentsFighting)
    (bind _returnvalue_2 (Actor|GetActorOfClass "/Game/Mechanics/MiniGames/ParentsFighting/BP_ParentsFightingMinigame.BP_ParentsFightingMinigame_C"))
    (Utilities|Map|Add (Variables|/Game/Mechanics/MiniGames/ParentsFighting/BP_ParentsFightingMinigame.BP_ParentsFightingMinigame_C|GetDialogOptionList _returnvalue_2) "Hurt" true)
    (Variables|Default|SetbAreParentsFighting false)))

(fn ConstructionScript
  (|CallParentFunction))