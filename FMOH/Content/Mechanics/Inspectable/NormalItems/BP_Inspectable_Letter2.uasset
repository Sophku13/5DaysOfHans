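; BP_Inspectable_Letter2 is an inspectable letter that plays a monologue and can unlock a dialog option in the parents-fighting minigame.
; On interact, it runs the parent logic, plays a paper sound and, after a short delay, spawns a BP_InterMono at the player with its sound and subtitle.
; If AreParentsFighting is set, it also adds "Letter" to BP_ParentsFightingMinigame's DialogOptionList and clears that flag.
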(event EventBeginPlay
  (|CallParentFunction) ; This node is disabled and will not be called.\nDrag off pins to build functionality.
)

(event Collision|EventActorBeginOverlap
  (params (OtherActor :type Actor%20Object%20Reference)))

(event EventTick
  (params (DeltaSeconds :type Float%20%28single-precision%29)))

(event EventOnInteract
  (params (PlayerRef :type BP%20Third%20Person%20Character%20Object%20Reference))
  (|CallParentFunction PlayerRef)
  (Utilities|FlowControl|Sequence
    (:then_0
      (Audio|PlaySoundatLocation "/Game/SoundSystem/Sounds/SFX/Paper/SC_Paper_1.SC_Paper_1" (Transformation|GetWorldLocation (Variables|Default|GetStaticMesh)) "0, 0, 0" 1.0 1.0 0.0 0 0 0 0)
      (Utilities|FlowControl|Delay 0.2)
      (bind _returnvalue (Game|SpawnActorfromClass "/Game/SoundSystem/Sounds/BP_InterMono.BP_InterMono_C" (Transformation|GetActorTransform (Game|GetPlayerCharacter 0)) "Undefined" "MultiplyWithRoot" 0 (Variables|Default|GetSound) 1.0 (Variables|Default|GetSubtitle%20Text) 6.0 true 0))
      (Default|CheckValues _returnvalue))
    (:then_1
      (if (Variables|Default|GetbAreParentsFighting)
        (bind _returnvalue_2 (Actor|GetActorOfClass "/Game/Mechanics/MiniGames/ParentsFighting/BP_ParentsFightingMinigame.BP_ParentsFightingMinigame_C"))
        (Utilities|Map|Add (Variables|/Game/Mechanics/MiniGames/ParentsFighting/BP_ParentsFightingMinigame.BP_ParentsFightingMinigame_C|GetDialogOptionList _returnvalue_2) "Letter" true)
        (Variables|Default|SetbAreParentsFighting false)))))

(fn ConstructionScript
  (|CallParentFunction))