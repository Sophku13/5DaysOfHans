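; Inspectable newspaper item that plays a sound and triggers an audio and subtitle response when the player interacts with it.
; On interact, it runs the parent logic, then plays the newspaper sound at its mesh location.
; It then spawns a short-lived BP_InterMono at the player character's transform, passes in its Sound and SubtitleText, and calls CheckValues on it.
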(event EventBeginPlay
  (|CallParentFunction) ; This node is disabled and will not be called.\nDrag off pins to build functionality.
)

(event Collision|EventActorBeginOverlap
  (params (OtherActor :type Actor%20Object%20Reference)))

(event EventTick
  (params (DeltaSeconds :type Float%20%28single-precision%29))
  (|CallParentFunction DeltaSeconds) ; This node is disabled and will not be called.\nDrag off pins to build functionality.
)

(event EventOnInteract
  (params (PlayerRef :type BP%20Third%20Person%20Character%20Object%20Reference))
  (|CallParentFunction PlayerRef)
  (Audio|PlaySoundatLocation "/Game/SoundSystem/Sounds/SFX/Paper/SC_Newspaper.SC_Newspaper" (Transformation|GetWorldLocation (Variables|Default|GetStaticMesh)) "0, 0, 0" 1.0 1.0 0.0 0 0 0 0)
  (bind _returnvalue (Game|SpawnActorfromClass "/Game/SoundSystem/Sounds/BP_InterMono.BP_InterMono_C" (Transformation|GetActorTransform (Game|GetPlayerCharacter 0)) "Undefined" "MultiplyWithRoot" 0 (Variables|Default|GetSound) 1.0 (Variables|Default|GetSubtitle%20Text) 5.0 true 0))
  (Default|CheckValues _returnvalue))

(fn ConstructionScript
  (|CallParentFunction))