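; Base Blueprint for inspectable clue quest items that the player finds by interacting with them.
; OnInteract sets IsFound and calls the parent's interaction, then, if CanBeFound is true, hides the actor and disables its mesh's overlap events.
; OnReset restores visibility and overlap events under the same CanBeFound check, but leaves IsFound unchanged.
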(event EventBeginPlay
  (|CallParentFunction) ; This node is disabled and will not be called.\nDrag off pins to build functionality.
)

(event Collision|EventActorBeginOverlap
  (params (OtherActor :type Actor%20Object%20Reference))
  (|CallParentFunction OtherActor) ; This node is disabled and will not be called.\nDrag off pins to build functionality.
)

(event EventTick
  (params (DeltaSeconds :type Float%20%28single-precision%29))
  (|CallParentFunction DeltaSeconds) ; This node is disabled and will not be called.\nDrag off pins to build functionality.
)

(event EventOnInteract
  (params (PlayerRef :type BP%20Third%20Person%20Character%20Object%20Reference))
  (Variables|Default|SetbIsFound true)
  (|CallParentFunction PlayerRef)
  (if (Variables|Default|GetbCanBeFound)
    (Rendering|SetActorHiddenInGame true)
    (Variables|/Script/Engine.PrimitiveComponent|SetbGenerateOverlapEvents (Variables|Default|GetStaticMesh) false)))

(event EventOnReset
  (if (Variables|Default|GetbCanBeFound)
    (Rendering|SetActorHiddenInGame false)
    (Variables|/Script/Engine.PrimitiveComponent|SetbGenerateOverlapEvents (Variables|Default|GetStaticMesh) true)))

(fn ConstructionScript
  (|CallParentFunction))