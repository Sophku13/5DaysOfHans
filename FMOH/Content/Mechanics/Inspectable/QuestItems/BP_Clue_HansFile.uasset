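; BP_Clue_HansFile is an inspectable quest clue, Hans's file, that moves the player on to the next room.
; Interacting marks it found and flags the player as moving on.
; If found, SaveforReset stops the secret wardrobe's end-level music, triggers activation and clears that flag, otherwise deferring to the parent.
; Activation sets quest completion, async-loads the next room and has the current room spawn a room switcher.
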(event EventBeginPlay)

(event Collision|EventActorBeginOverlap
  (params (OtherActor :type Actor%20Object%20Reference))
  (|CallParentFunction OtherActor) ; This node is disabled and will not be called.\nDrag off pins to build functionality.
)

(event EventTick
  (params (DeltaSeconds :type Float%20%28single-precision%29))
  (|CallParentFunction DeltaSeconds) ; This node is disabled and will not be called.\nDrag off pins to build functionality.
)

(event EventOnInteract
  (params (PlayerRef :type BP%20Third%20Person%20Character%20Object%20Reference))
  ;[0 1 0.6029] Spawning next level
  (Variables|Default|SetPlayer%20Ref PlayerRef)
  (Variables|/Game/ThirdPerson/Blueprints/BP_ThirdPersonCharacter.BP_ThirdPersonCharacter_C|SetbIsMovingOn PlayerRef true)
  (Variables|Default|SetbIsFound true)
  (|CallParentFunction PlayerRef))

(event EventOnActivation
  (params (PlayerRef :type BP%20Third%20Person%20Character%20Object%20Reference))
  ;[0 1 0.6029] Spawning next level
  (|CallParentFunction PlayerRef)
  (Variables|Default|SetbIsQuestCompleted (Variables|Default|GetbIsActivated))
  (bind __nextroomref (Variables|Default|Get_NextRoomRef)
    (:then
      (Utilities|AsyncLoadAsset __nextroomref
        (:Completed
          (Default|SpawnRoomSwitcher (Variables|Default|Get_currentRoomRef) __nextroomref))))
    (:else
      (Development|PrintString "ButtonNextRoomRef NOT WORKING!"))))

(event EventSaveforReset
  (bind _player_ref (Variables|Default|GetPlayer%20Ref))
  (if (Variables|Default|GetbIsFound)
    (bind _returnvalue (Actor|GetActorOfClass "/Game/Mechanics/ActivatableObject/BP_SecretWardrobe.BP_SecretWardrobe_C"))
    (Audio|Components|Audio|Stop (Variables|/Game/Mechanics/ActivatableObject/BP_SecretWardrobe.BP_SecretWardrobe_C|GetEndLevelMusicRef _returnvalue))
    (CallFunction|OnActivation _player_ref)
    (Variables|/Game/ThirdPerson/Blueprints/BP_ThirdPersonCharacter.BP_ThirdPersonCharacter_C|SetbIsMovingOn _player_ref false)
    (else
      (|CallParentFunction))))

(fn ConstructionScript
  (|CallParentFunction))