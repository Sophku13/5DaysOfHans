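; Inspectable quest item, apparently tied to a death room, that triggers a room switch when the player interacts with it.
; Interaction runs activation, which copies the activated state to quest completion, async loads the next room and has the current room spawn a room switcher to it.
; The item then hides and drops its mesh collision, and a reset restores both.
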(event EventBeginPlay
  (|CallParentFunction) ; This node is disabled and will not be called.\nDrag off pins to build functionality.
)

(event Collision|EventActorBeginOverlap
  (params (OtherActor :type Actor%20Object%20Reference))
  (|CallParentFunction OtherActor) ; This node is disabled and will not be called.\nDrag off pins to build functionality.
)

(event EventTick
  (params (DeltaSeconds :type Float%20%28single-precision%29))
  (|CallParentFunction DeltaSeconds) ; This node is disabled and will not be called.\nDrag off pins to build functionality.
)

(event EventOnActivation
  (params (PlayerRef :type BP%20Third%20Person%20Character%20Object%20Reference))
  ;[1 1 1] Comment
  (|CallParentFunction PlayerRef)
  (Variables|Default|SetbIsQuestCompleted (Variables|Default|GetbIsActivated))
  (bind __nextroomref (Variables|Default|Get_NextRoomRef)
    (:then
      (Utilities|AsyncLoadAsset __nextroomref
        (:Completed
          (Default|SpawnRoomSwitcher (Variables|Default|Get_currentRoomRef) __nextroomref))))
    (:else
      (Development|PrintString "DeathRoomRef NOT WORKING!"))))

(event EventOnInteract
  (params (PlayerRef :type BP%20Third%20Person%20Character%20Object%20Reference))
  ;[1 1 1] Comment
  (|CallParentFunction PlayerRef)
  (CallFunction|OnActivation PlayerRef)
  (Rendering|SetActorHiddenInGame self true)
  (Collision|SetCollisionEnabled (Variables|Default|GetStaticMesh) "NoCollision"))

(event EventSaveforReset
  (|CallParentFunction))

(event EventOnReset
  (|CallParentFunction)
  (Rendering|SetActorHiddenInGame self false)
  (Collision|SetCollisionEnabled (Variables|Default|GetStaticMesh) "QueryAndPhysics"))

(fn ConstructionScript
  (|CallParentFunction))