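; Carryable quest item, apparently a test version, that the player picks up and places at a quest location.
; Interacting attaches it to the player's ItemAttachmentArm and reveals the linked location meshes with overlap events enabled.
; Dropping detaches it and teleports it back to the mesh transform saved at BeginPlay.
; PlaceInQuestLocation moves it to the given transform and completes the quest, after which Tick destroys the linked location actors.
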(event Custom|PlaceInQuestLocation
  (params (QuestItemLocation :type Transform))
  (bind (_location _rotation) (Math|Transform|BreakTransform QuestItemLocation))
  (Transformation|DetachFromActor self "KeepRelative" "KeepRelative" "KeepRelative")
  (Variables|Default|SetbIsPickedUp false)
  (Transformation|SetActorLocationAndRotation self _location _rotation)
  (Variables|Default|SetbIsQuestCompleted true))

(event Input|EnhancedActionEvents|EnhancedInputActionIA_Drop
  (params (ActionValue :type Boolean) (ElapsedSeconds :type Float%20%28double-precision%29) (TriggeredSeconds :type Float%20%28double-precision%29) (InputAction :type Input%20Action%20Object%20Reference :default "/Game/Character/Input/Actions/IA_Drop.IA_Drop"))
  (bind _startinglocation (Variables|Default|GetstartingLocation))
  (if (Variables|Default|GetbIsPickedUp)
    (Transformation|DetachFromActor self "KeepRelative" "KeepRelative" "KeepRelative")
    (Variables|Default|SetbIsPickedUp false)
    (Transformation|SetActorLocationAndRotation self (.location _startinglocation) (.rotation _startinglocation) false true)))

(event EventBeginPlay
  (|CallParentFunction)
  (Variables|Default|SetstartingLocation (Transformation|GetWorldTransform (Variables|Default|GetQuestItemMesh))))

(event Collision|EventActorBeginOverlap
  (params (OtherActor :type Actor%20Object%20Reference))
  (|CallParentFunction OtherActor) ; This node is disabled and will not be called.\nDrag off pins to build functionality.
)

(event EventOnInteract
  (params (PlayerRef :type BP%20Third%20Person%20Character%20Object%20Reference))
  (if (and (not (Variables|Default|GetbIsQuestCompleted)) (not (Variables|/Game/ThirdPerson/Blueprints/BP_ThirdPersonCharacter.BP_ThirdPersonCharacter_C|GetbIsCarryingItem PlayerRef)))
    (Variables|/Game/ThirdPerson/Blueprints/BP_ThirdPersonCharacter.BP_ThirdPersonCharacter_C|SetbIsCarryingItem PlayerRef true)
    (Transformation|AttachComponentToComponent self (Variables|/Game/ThirdPerson/Blueprints/BP_ThirdPersonCharacter.BP_ThirdPersonCharacter_C|GetItemAttachmentArm PlayerRef) "Target" "SnapToTarget" "SnapToTarget" "KeepRelative" false)
    (Variables|Default|SetbIsPickedUp true)
    (for _array_element (Variables|Default|GetLocationBps)
      (Development|SetHiddeninGame (Variables|/Game/Mechanics/BaseBlueprints/BP_QuestItemPlaceLocation.BP_QuestItemPlaceLocation_C|GetQuestItemMesh _array_element) false false)
      (Variables|/Script/Engine.PrimitiveComponent|SetbGenerateOverlapEvents (Variables|/Game/Mechanics/BaseBlueprints/BP_QuestItemPlaceLocation.BP_QuestItemPlaceLocation_C|GetQuestItemMesh _array_element) true))))

(event EventOnActivation
  (params (PlayerRef :type BP%20Third%20Person%20Character%20Object%20Reference)))

(event EventTick
  (params (DeltaSeconds :type Float%20%28single-precision%29))
  (if (Variables|Default|GetbIsQuestCompleted)
    (for _array_element (Variables|Default|GetLocationBps)
      (Utilities|IsValid _array_element
        (:Is%20Valid
          (Actor|DestroyActor _array_element))))))

(fn ConstructionScript
  (|CallParentFunction))