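; Base piano key Blueprint that plays its key sound at the mesh location on every interaction and animates a press.
; Two chained timelines lower then raise the mesh by adding scaled track values to its current relative Z each update, so offsets accumulate rather than interpolate from a stored start.
; IsPlaying blocks animation restarts but not repeated sounds.
; The construction script applies the configurable key mesh.
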(event EventBeginPlay
  (|CallParentFunction))

(event Collision|EventActorBeginOverlap
  (params (OtherActor :type Actor%20Object%20Reference)))

(event EventTick
  (params (DeltaSeconds :type Float%20%28single-precision%29)))

(event EventOnInteract
  (params (PlayerRef :type BP%20Third%20Person%20Character%20Object%20Reference))
  (bind _keymesh (Variables|Default|GetKeyMesh))
  (bind _keymesh_2 (Variables|Default|GetKeyMesh))
  (bind _relativelocation (Variables|/Script/Engine.SceneComponent|GetRelativeLocation _keymesh))
  (bind _relativelocation_2 (Variables|/Script/Engine.SceneComponent|GetRelativeLocation _keymesh_2))
  (Audio|SpawnSoundatLocation (Variables|Default|GetKeySound) (Transformation|GetWorldLocation (Variables|Default|GetKeyMesh)) "0, 0, 0" 1.0 1.0 0.0 0 0)
  (if (not (Variables|Default|GetbIsPlaying))
    (Variables|Default|SetbIsPlaying true)
    (bind _newtrack_0 (Timeline|Timeline PlayFromStart)
      (:Update
        (Transformation|SetRelativeLocation _keymesh (Math|Vector|MakeVector (.x _relativelocation) (.y _relativelocation) (+ (.z _relativelocation) (* _newtrack_0 -0.08))) false false))
      (:Finished
        (bind _newtrack_0_2 (Timeline|Timeline_0 PlayFromStart)
          (:Update
            (Transformation|SetRelativeLocation _keymesh_2 (Math|Vector|MakeVector (.x _relativelocation_2) (.y _relativelocation_2) (+ (.z _relativelocation_2) (* _newtrack_0_2 0.08))) false false))
          (:Finished
            (Variables|Default|SetbIsPlaying false)))))))

(fn ConstructionScript
  (|CallParentFunction)
  (Components|StaticMesh|SetStaticMesh (Variables|Default|GetKeyMesh) (Variables|Default|GetInputKeyMesh)))