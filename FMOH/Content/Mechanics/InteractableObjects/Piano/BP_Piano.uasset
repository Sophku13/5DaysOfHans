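; Interactable piano that toggles a playable view, locking player movement and camera, switching view target and showing the cursor.
; BeginPlay assigns each key its sound from KeySetup, and left clicks trace from the cursor to forward interaction to the hit actor.
; Interacting also spawns a one-time BP_InterMono chosen by PianoNumber, with sound and subtitle set only for the first.
; While AreParentsFighting is set, it adds a "Piano" dialog option to the parents-fighting minigame, then clears the flag.
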(event EventBeginPlay
  (|CallParentFunction)
  (bind _values (Utilities|Map|Values (Variables|Default|GetKeySetup)))
  (for _array_element _values
    (Variables|/Game/Mechanics/InteractableObjects/Piano/BP_Piano_Key_Base.BP_Piano_Key_Base_C|SetKeySound (.reference _array_element) (.sound _array_element))))

(event EventOnInteract
  (params (PlayerRef :type BP%20Third%20Person%20Character%20Object%20Reference))
  (bind _returnvalue (Game|GetPlayerController 0))
  (bind _returnvalue_2 (Game|GetPlayerController 0))
  (bind _returnvalue_3 (Game|GetPlayerController 0))
  ;[1 1 1] Entering and leaving the PianoView
  (Utilities|FlowControl|Sequence
    (:then_0
      (|CollapseGraph))
    (:then_1
      (bind _output_get (Variables|Default|SetPlayer%20Ref PlayerRef))
      (if (not (Variables|Default|GetbIsPlayingPiano))
        (Variables|/Game/ThirdPerson/Blueprints/BP_ThirdPersonCharacter.BP_ThirdPersonCharacter_C|SetIsMovementLocked _output_get true)
        (Variables|/Game/ThirdPerson/Blueprints/BP_ThirdPersonCharacter.BP_ThirdPersonCharacter_C|SetbIsCameraLocked _output_get true)
        (Variables|/Script/Engine.PlayerController|SetbShowMouseCursor _returnvalue true)
        (Game|Player|SetViewTargetwithBlend _returnvalue self 0.0 "VTBlend_Linear" 0.0 false)
        (Input|EnableInput _returnvalue_2)
        (Variables|Default|SetbIsPlayingPiano true)
        (Input|SetInputModeGameandUI _returnvalue_2 0 "LockInFullscreen" true false)
        (Variables|/Game/ThirdPerson/Blueprints/BP_ThirdPersonCharacter.BP_ThirdPersonCharacter_C|SetbIsInMinigame (Variables|Default|GetPlayer%20Ref) true)
        (Variables|/Game/ThirdPerson/Blueprints/BP_ThirdPersonCharacter.BP_ThirdPersonCharacter_C|SetActiveMinigameName (Variables|Default|GetPlayer%20Ref) "Clicker")
        (else
          (Variables|/Game/ThirdPerson/Blueprints/BP_ThirdPersonCharacter.BP_ThirdPersonCharacter_C|SetIsMovementLocked _output_get false)
          (Variables|/Game/ThirdPerson/Blueprints/BP_ThirdPersonCharacter.BP_ThirdPersonCharacter_C|SetbIsCameraLocked _output_get false)
          (Variables|/Script/Engine.PlayerController|SetbShowMouseCursor _returnvalue_3 false)
          (Game|Player|SetViewTargetwithBlend _returnvalue_3 (Variables|Default|GetPlayer%20Ref) 0.0 "VTBlend_Linear" 0.0 false)
          (Input|DisableInput (Game|GetPlayerController 0))
          (Variables|Default|SetbIsPlayingPiano false)
          (Input|SetInputModeGameOnly _returnvalue_2 false)
          (Variables|/Game/ThirdPerson/Blueprints/BP_ThirdPersonCharacter.BP_ThirdPersonCharacter_C|SetbIsInMinigame (Variables|Default|GetPlayer%20Ref) false))))
    (:then_2
      (if (Variables|Default|GetbAreParentsFighting)
        (bind _returnvalue_4 (Actor|GetActorOfClass "/Game/Mechanics/MiniGames/ParentsFighting/BP_ParentsFightingMinigame.BP_ParentsFightingMinigame_C"))
        (Utilities|Map|Add (Variables|/Game/Mechanics/MiniGames/ParentsFighting/BP_ParentsFightingMinigame.BP_ParentsFightingMinigame_C|GetDialogOptionList _returnvalue_4) "Piano" true)
        (Variables|Default|SetbAreParentsFighting false)))))

(event Input|MouseEvents|LeftMouseButton
  (params (Key :type Key%20Structure :default "None"))
  (bind _returnvalue (Game|GetPlayerController 0))
  (bind (_worldlocation _worlddirection) (Game|Player|ConvertMouseLocationToWorldSpace _returnvalue))
  ;[1 1 1] Comment
  (:Pressed
    (bind _outhit (Collision|LineTraceByChannel _worldlocation (+ _worldlocation (* _worlddirection (Math|Conversions|ToVector(Float) 5e+02))) "TraceTypeQuery1" false 0 "None" false))
    (Class|BPIInteractable|OnInteract(Message) (.HitActor (Collision|BreakHitResult _outhit)) (Variables|Default|GetPlayer%20Ref))))

(fn ConstructionScript
  (|CallParentFunction))