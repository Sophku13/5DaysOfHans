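; Interactable door Blueprint that toggles open and closed on each interaction.
; A FlipFlop plays or reverses the OpenDoor timeline, which yaws the Anchor component up to 90 degrees, with open and close sounds played at world origin.
; OnReset re-runs OnInteract to close the door if it is open.
; CreateListOfComponents returns a list containing the Door component.
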(event EventOnReset
  (if (Variables|Default|GetbIsDoorOpen)
    (CallFunction|OnInteract)))

(event EventOnInteract
  (params (PlayerRef :type BP%20Third%20Person%20Character%20Object%20Reference))
  ;[1 1 1] Comment
  (Utilities|FlowControl|FlipFlop
    (:A
      (Variables|Default|SetbIsDoorOpen true)
      (Audio|PlaySoundatLocation "/Game/SoundSystem/Sounds/Door/SC_OpenDoor_3_Cue.SC_OpenDoor_3_Cue" "0, 0, 0" "0, 0, 0" 1.0 1.0 0.0 0 0 0 0)
      (bind _newtrack_0 (Timeline|OpenDoor Play)
        (:Update
          (Transformation|SetRelativeRotation (Variables|Default|GetAnchor) (Math|Rotator|MakeRotator 0.0 0.0 (* _newtrack_0 90)) false false))))
    (:B
      (Variables|Default|SetbIsDoorOpen false)
      (Audio|PlaySoundatLocation "/Game/SoundSystem/Sounds/Door/CloseDoor_3_Cue.CloseDoor_3_Cue" "0, 0, 0" "0, 0, 0" 1.0 1.0 0.0 0 0 0 0)
      (Timeline|OpenDoor Reverse))))

(fn ConstructionScript
  (|CallParentFunction))

(fn CreateListOfComponents
  (Utilities|Array|Add (LocalVariables|GetDoorVar) (Variables|Default|GetDoor))
  (return (LocalVariables|GetDoorVar)))