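; Interactable door that stays locked until OnActivation marks its key as acquired.
; Interacting then toggles it, playing a sound and swinging Anchor 90 degrees through a forward or reversed timeline, and OnReset closes it if open.
; While locked, it plays a locked sound and, after a short delay, spawns a one-time BP_InterMono monologue with subtitles.
; Mouse-drag rotation and try-counter logic remain in the graph but never run.
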(event Input|EnhancedActionEvents|EnhancedInputActionIA_DragObjects
  (params (ActionValue :type Boolean) (ElapsedSeconds :type Float%20%28double-precision%29) (TriggeredSeconds :type Float%20%28double-precision%29) (InputAction :type Input%20Action%20Object%20Reference :default "/Game/Character/Input/Actions/IA_DragObjects.IA_DragObjects"))
  ;[1 1 1] Comment
  ;;[1 1 1] Comment
)

(event EventBeginPlay
  (|CallParentFunction))

(event EventOnReset
  (if (Variables|Default|GetbIsDoorOpen)
    (CallFunction|OnInteract)))

(event EventOnInteract
  (params (PlayerRef :type BP%20Third%20Person%20Character%20Object%20Reference))
  ;[1 1 1] Comment
  (if (Variables|Default|GetbIsDoorKeyAquired)
    (if (not (Variables|Default|GetbIsDoorOpen))
      (Variables|Default|SetbIsDoorOpen true)
      (Audio|PlaySoundatLocation "/Game/SoundSystem/Sounds/SFX/Door/SC_OpenDoor_3_Cue.SC_OpenDoor_3_Cue" "0, 0, 0" "0, 0, 0" 1.0 1.0 0.0 0 0 0 0)
      (bind _newtrack_0 (Timeline|Timeline PlayFromStart)
        (:Update
          (Transformation|SetRelativeRotation (Variables|Default|GetAnchor) (Math|Rotator|MakeRotator 0.0 0.0 (* _newtrack_0 90)) false false)))
      (else
        (Variables|Default|SetbIsDoorOpen false)
        (Audio|PlaySoundatLocation "/Game/SoundSystem/Sounds/SFX/Door/CloseDoor_3_Cue.CloseDoor_3_Cue" "0, 0, 0" "0, 0, 0" 1.0 1.0 0.0 0 0 0 0)
        (Timeline|Timeline ReverseFromEnd)))
    (elif (not (Variables|Default|GetbIsPlayingSound))
      (Audio|PlaySound2D (Variables|Default|Getlocked_door_sound) 1.0 1.0 0.0 0 0)
      (Utilities|FlowControl|Delay 0.2)
      (Utilities|FlowControl|DoOnce false
        (:Completed
          (bind _returnvalue (Game|SpawnActorfromClass "/Game/SoundSystem/Sounds/BP_InterMono.BP_InterMono_C" (Transformation|GetActorTransform (Game|GetPlayerCharacter 0)) "Undefined" "MultiplyWithRoot" 0 (Variables|Default|GetMonolog) 1.0 (Variables|Default|GetSubtitle%20Text) 5.0 true 0))
          (Default|CheckValues _returnvalue))))))

(event Collision|EventActorBeginOverlap
  (params (OtherActor :type Actor%20Object%20Reference))
  (|CallParentFunction OtherActor) ; This node is disabled and will not be called.\nDrag off pins to build functionality.
)

(event EventSaveforReset
  (|CallParentFunction))

(event EventOnActivation
  (params (PlayerRef :type BP%20Third%20Person%20Character%20Object%20Reference))
  (Variables|Default|SetbIsDoorKeyAquired true))

(event EventTick
  (params (DeltaSeconds :type Float%20%28single-precision%29))
  ;[1 1 1] Comment
  ;;[1 1 1] Comment
)

(fn ConstructionScript
  (|CallParentFunction))