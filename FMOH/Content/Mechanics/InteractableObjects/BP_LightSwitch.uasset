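; Interactable light switch actor that toggles a list of linked lamps.
; Each interaction alternates through a FlipFlop, setting the LightsOn flag and rolling the switch component 60 degrees one way or back.
; Both branches send the same OnActivationMessage to every entry in LampList, with no on/off state passed.
; On reset, it calls the parent logic and re-runs the interaction if the lights are on, returning the switch to off.
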(event EventBeginPlay
  (|CallParentFunction) ; This node is disabled and will not be called.\nDrag off pins to build functionality.
)

(event Collision|EventActorBeginOverlap
  (params (OtherActor :type Actor%20Object%20Reference))
  (|CallParentFunction OtherActor) ; This node is disabled and will not be called.\nDrag off pins to build functionality.
)

(event EventTick
  (params (DeltaSeconds :type Float%20%28single-precision%29))
  (|CallParentFunction DeltaSeconds) ; This node is disabled and will not be called.\nDrag off pins to build functionality.
)

(event EventOnInteract
  (params (PlayerRef :type BP%20Third%20Person%20Character%20Object%20Reference))
  (bind _lightswitch (Variables|Default|GetLightSwitch))
  (bind _relativerotation (Variables|/Script/Engine.SceneComponent|GetRelativeRotation _lightswitch))
  (Utilities|FlowControl|FlipFlop
    (:A
      (Variables|Default|SetbLightsOn true)
      (Transformation|SetRelativeRotation _lightswitch (Math|Rotator|MakeRotator (+ (.roll _relativerotation) 6e+01) (.pitch _relativerotation) (.yaw _relativerotation)) false false)
      (for _array_element (Variables|Default|GetLampList)
        (Class|BPIActivatable|OnActivation(Message) _array_element)))
    (:B
      (Variables|Default|SetbLightsOn false)
      (Transformation|SetRelativeRotation _lightswitch (Math|Rotator|MakeRotator (- (.roll _relativerotation) 6e+01) (.pitch _relativerotation) (.yaw _relativerotation)) false false)
      (for _array_element_2 (Variables|Default|GetLampList)
        (Class|BPIActivatable|OnActivation(Message) _array_element_2)))))

(event EventOnReset
  (|CallParentFunction)
  (if (Variables|Default|GetbLightsOn)
    (CallFunction|OnInteract)))

(fn ConstructionScript
  (|CallParentFunction))