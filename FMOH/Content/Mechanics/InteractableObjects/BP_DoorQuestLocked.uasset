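; A quest-locked door that the player can swing by hand once every referenced quest item reports its quest completed.
; Interacting checks those quests, then toggles open state with sounds, or reports it locked and plays a monologue on the first of every three attempts.
; While drag input is held and a camera trace hits this door class, Tick rotates the anchor by the character's turn rate within angle limits.
; The timeline-driven opening is disconnected.
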(event Input|EnhancedActionEvents|EnhancedInputActionIA_DragObjects
  (params (ActionValue :type Boolean) (ElapsedSeconds :type Float%20%28double-precision%29) (TriggeredSeconds :type Float%20%28double-precision%29) (InputAction :type Input%20Action%20Object%20Reference :default "/Game/Character/Input/Actions/IA_DragObjects.IA_DragObjects"))
  ;[1 1 1] Comment
  ;;[1 1 1] Comment
  (:Triggered
    (Variables|Default|SetbIsHoldingLMB true)
    (bind _asbp_third_person_character (Utilities|Casting|CastToBP_ThirdPersonCharacter (Game|GetPlayerCharacter 0)))
    (bind (_outhit _returnvalue) (Collision|LineTraceForObjects (Transformation|GetWorldLocation (Variables|/Game/ThirdPerson/Blueprints/BP_ThirdPersonCharacter.BP_ThirdPersonCharacter_C|GetFollowCamera _asbp_third_person_character)) (+ (Transformation|GetWorldLocation (Variables|/Game/ThirdPerson/Blueprints/BP_ThirdPersonCharacter.BP_ThirdPersonCharacter_C|GetFollowCamera _asbp_third_person_character)) (* (Math|Vector|GetForwardVector (Variables|/Game/ThirdPerson/Blueprints/BP_ThirdPersonCharacter.BP_ThirdPersonCharacter_C|GetFollowCamera _asbp_third_person_character)) 5e+02)) (Utilities|Array|MakeArray "ObjectTypeQuery1") false 0 "None" false))
    (if _returnvalue
      (Utilities|Casting|CastToBP_DoorQuestLocked (.HitActor (Collision|BreakHitResult _outhit)))
      (Variables|Default|SetbLookingAtDoor true)
      (else
        (Variables|Default|SetbLookingAtDoor false))))
  (:Completed
    (Variables|Default|SetbIsHoldingLMB false)))

(event EventBeginPlay
  ;[1 1 1] Comment
  (|CallParentFunction)
  (Input|EnableInput (Game|GetPlayerController 0)))

(event EventOnReset
  (if (Variables|Default|GetbIsDoorOpen)
    (CallFunction|OnInteract))
  (Variables|Default|SetbIsDoorQuestComplete false))

(event EventOnInteract
  (params (PlayerRef :type BP%20Third%20Person%20Character%20Object%20Reference))
  ;[1 1 1] Comment
  (bind (_array_element _array_index) (Utilities|Array|ForEachLoopwithBreak (Variables|Default|GetQuestItemRef) :!label _label)
    (:LoopBody
      (if (Variables|/Game/Mechanics/BaseBlueprints/BP_BaseQuestItem.BP_BaseQuestItem_C|GetbIsQuestCompleted _array_element)
        (if (== _array_index 0)
          (Variables|Default|SetbIsDoorQuestComplete true)
          (else
            (Variables|Default|SetbIsDoorQuestComplete (and (Variables|/Game/Mechanics/BaseBlueprints/BP_BaseQuestItem.BP_BaseQuestItem_C|GetbIsQuestCompleted _array_element) (Variables|Default|GetbIsDoorQuestComplete)))))
        (else
          (Variables|Default|SetbIsDoorQuestComplete false)
          (goto _label Break))))
    (:Completed
      (if (Variables|Default|GetbIsDoorQuestComplete)
        (Utilities|FlowControl|FlipFlop
          (:A
            (Variables|Default|SetbIsDoorOpen true)
            (Audio|PlaySoundatLocation "/Game/SoundSystem/Sounds/SFX/Door/SC_OpenDoor_3_Cue.SC_OpenDoor_3_Cue" "0, 0, 0" "0, 0, 0" 1.0 1.0 0.0 0 0 0 0))
          (:B
            (Variables|Default|SetbIsDoorOpen false)
            (Audio|PlaySoundatLocation "/Game/SoundSystem/Sounds/SFX/Door/CloseDoor_3_Cue.CloseDoor_3_Cue" "0, 0, 0" "0, 0, 0" 1.0 1.0 0.0 0 0 0 0)))
        (else
          (Math|Integer|IncrementInt (Variables|Default|GetOpenThreeTimes)
            (:%20%20
              (Development|PrintString "Door is Locked")
              (if (== (Variables|Default|GetOpenThreeTimes) 1)
                (Audio|PlaySound2D "/Game/SoundSystem/Sounds/VoiceRecordings/InnerMonologue/SC_Monologue_01.SC_Monologue_01" 1.0 1.0 0.0 0 0)
                (elif (== (Variables|Default|GetOpenThreeTimes) 3)
                  (Variables|Default|SetOpenThreeTimes 0))))))))))

(event EventTick
  (params (DeltaSeconds :type Float%20%28single-precision%29))
  (bind _anchor (Variables|Default|GetAnchor))
  (bind _openangle (Variables|Default|GetOpenAngle))
  (bind _openangle_2 (Variables|Default|GetOpenAngle))
  (bind _returnvalue (Transformation|GetWorldRotation _anchor))
  ;[1 1 1] Comment
  ;;[1 1 1] Comment
  (if (Variables|Default|GetbIsDoorQuestComplete)
    (if (Variables|Default|GetbIsHoldingLMB)
      (if (Variables|Default|GetbLookingAtDoor)
        (if (not (== (.yaw _returnvalue) (Math|Float|ClampAngle (.yaw _returnvalue) _openangle (* _openangle -1.0))))
          (Transformation|AddLocalRotation _anchor (Math|Rotator|MakeRotator 0.0 0.0 (* (Variables|/Game/ThirdPerson/Blueprints/BP_ThirdPersonCharacter.BP_ThirdPersonCharacter_C|GetTurnRate (stale Input|EnhancedActionEvents|EnhancedInputActionIA_DragObjects _asbp_third_person_character)) (Variables|Default|GetSensitivity))) false false)
          (elif (>= (.yaw _returnvalue) _openangle_2)
            (Transformation|SetRelativeRotation _anchor (Math|Rotator|MakeRotator 0.0 0.0 (- _openangle_2 1.0)) false false)
            (else
              (Transformation|SetRelativeRotation _anchor (Math|Rotator|MakeRotator 0.0 0.0 (+ (* _openangle_2 -1.0) 1.0)) false false))))))))

(fn ConstructionScript
  (|CallParentFunction))

(fn CreateListOfComponents
  (Utilities|Array|Add (LocalVariables|GetDoorVar) (Variables|Default|GetDoor))
  (return (LocalVariables|GetDoorVar)))