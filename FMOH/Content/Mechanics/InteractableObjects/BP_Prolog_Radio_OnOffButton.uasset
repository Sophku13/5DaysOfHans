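; An interactable on/off button for the prologue radio that calls OnOff on its referenced radio actor.
; OnInteract and TurnOff pass opposite booleans to that call, then share the same button feedback.
; A FlipFlop alternates button up and down sounds at the button's location.
; A timeline, gated by an IsMoving flag, offsets the button along its local Y axis to animate the press.
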(event Custom|TurnOff
  (bind _button (Variables|Default|GetButton))
  (bind _relativelocation (Variables|/Script/Engine.SceneComponent|GetRelativeLocation _button))
  (Default|OnOff (Variables|Default|GetRadioRef) true)
  (Development|PrintString "ButtonSound")
  (Utilities|FlowControl|FlipFlop
    (:A
      (Audio|PlaySoundatLocation "/Game/SoundSystem/Sounds/SFX/Buttons/SC_ButtonUp_Cue.SC_ButtonUp_Cue" (Transformation|GetWorldLocation (Variables|Default|GetButton)) "0, 0, 0" 1.0 1.0 0.0 0 0 0 0))
    (:B
      (Audio|PlaySoundatLocation "/Game/SoundSystem/Sounds/SFX/Buttons/SC_ButtonDown_Cue.SC_ButtonDown_Cue" (Transformation|GetWorldLocation (Variables|Default|GetButton)) "0, 0, 0" 1.0 1.0 0.0 0 0 0 0)))
  (if (Variables|Default|GetbIsMoving)
    (Variables|Default|SetbIsMoving true)
    (bind _newtrack_0 (Timeline|Timeline PlayFromStart)
      (:Update
        (Transformation|SetRelativeLocation _button (Math|Vector|MakeVector (.x _relativelocation) (+ (.y _relativelocation) (* _newtrack_0 -0.5)) (.z _relativelocation)) false false))
      (:Finished
        (Variables|Default|SetbIsMoving false)))))

(event EventBeginPlay
  (|CallParentFunction) ; This node is disabled and will not be called.\nDrag off pins to build functionality.
)

(event Collision|EventActorBeginOverlap
  (params (OtherActor :type Actor%20Object%20Reference)))

(event EventTick
  (params (DeltaSeconds :type Float%20%28single-precision%29)))

(event EventOnInteract
  (params (PlayerRef :type BP%20Third%20Person%20Character%20Object%20Reference))
  (bind _button (Variables|Default|GetButton))
  (bind _relativelocation (Variables|/Script/Engine.SceneComponent|GetRelativeLocation _button))
  (Default|OnOff (Variables|Default|GetRadioRef) false)
  (Development|PrintString "ButtonSound")
  (Utilities|FlowControl|FlipFlop
    (:A
      (Audio|PlaySoundatLocation "/Game/SoundSystem/Sounds/SFX/Buttons/SC_ButtonUp_Cue.SC_ButtonUp_Cue" (Transformation|GetWorldLocation (Variables|Default|GetButton)) "0, 0, 0" 1.0 1.0 0.0 0 0 0 0))
    (:B
      (Audio|PlaySoundatLocation "/Game/SoundSystem/Sounds/SFX/Buttons/SC_ButtonDown_Cue.SC_ButtonDown_Cue" (Transformation|GetWorldLocation (Variables|Default|GetButton)) "0, 0, 0" 1.0 1.0 0.0 0 0 0 0)))
  (if (Variables|Default|GetbIsMoving)
    (Variables|Default|SetbIsMoving true)
    (bind _newtrack_0 (Timeline|Timeline PlayFromStart)
      (:Update
        (Transformation|SetRelativeLocation _button (Math|Vector|MakeVector (.x _relativelocation) (+ (.y _relativelocation) (* _newtrack_0 -0.5)) (.z _relativelocation)) false false))
      (:Finished
        (Variables|Default|SetbIsMoving false)))))

(fn ConstructionScript
  (|CallParentFunction))