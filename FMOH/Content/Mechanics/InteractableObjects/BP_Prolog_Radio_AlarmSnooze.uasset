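; Interactable snooze button for the prologue radio alarm that switches off the alarm on the referenced radio when interacted with.
; OnInteract calls AlarmOff, prints a debug string and plays button up and down sounds at the button, separated by a short delay.
; A timeline then offsets the button's Z cumulatively each update, but as wired it only starts if IsMoving is already true, clearing that flag when finished.
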(event EventBeginPlay
  (|CallParentFunction) ; This node is disabled and will not be called.\nDrag off pins to build functionality.
)

(event Collision|EventActorBeginOverlap
  (params (OtherActor :type Actor%20Object%20Reference)))

(event EventTick
  (params (DeltaSeconds :type Float%20%28single-precision%29)))

(event EventOnInteract
  (params (PlayerRef :type BP%20Third%20Person%20Character%20Object%20Reference))
  (bind _button (Variables|Default|GetButton))
  (bind _relativelocation (Variables|/Script/Engine.SceneComponent|GetRelativeLocation _button))
  (Default|AlarmOff (Variables|Default|GetRadioRef))
  (Development|PrintString "ButtonSound")
  (Audio|PlaySoundatLocation "/Game/SoundSystem/Sounds/SFX/Buttons/SC_ButtonUp_Cue.SC_ButtonUp_Cue" (Transformation|GetWorldLocation (Variables|Default|GetButton)) "0, 0, 0" 1.0 1.0 0.0 0 0 0 0)
  (Utilities|FlowControl|Delay 0.1)
  (Audio|PlaySoundatLocation "/Game/SoundSystem/Sounds/SFX/Buttons/SC_ButtonDown_Cue.SC_ButtonDown_Cue" (Transformation|GetWorldLocation (Variables|Default|GetButton)) "0, 0, 0" 1.0 1.0 0.0 0 0 0 0)
  (if (Variables|Default|GetbIsMoving)
    (Variables|Default|SetbIsMoving true)
    (bind _newtrack_0 (Timeline|Timeline PlayFromStart)
      (:Update
        (Transformation|SetRelativeLocation _button (Math|Vector|MakeVector (.x _relativelocation) (.y _relativelocation) (+ (.z _relativelocation) (* _newtrack_0 -2.0))) false false))
      (:Finished
        (Variables|Default|SetbIsMoving false)))))

(fn ConstructionScript
  (|CallParentFunction))