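; BP_TeleportationFrame is an interactable actor that opens a teleport choice menu for the player.
; On interact it closes the player's eyes, waits, pauses the game and shows WBP_TeleportChoice with mouse-driven UI-only input, passing in the room switcher reference.
; StayingInLevel unhides the frame and reopens the character's eyes, while OnReset hides the frame again.
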(event Custom|StayingInLevel
  (Rendering|SetActorHiddenInGame false)
  (bind _asbp_third_person_character (Utilities|Casting|CastToBP_ThirdPersonCharacter (Game|GetPlayerCharacter 0)))
  (Default|OpenEyes _asbp_third_person_character 1.0))

(event EventBeginPlay
  (|CallParentFunction) ; This node is disabled and will not be called.\nDrag off pins to build functionality.
)

(event Collision|EventActorBeginOverlap
  (params (OtherActor :type Actor%20Object%20Reference)))

(event EventTick
  (params (DeltaSeconds :type Float%20%28single-precision%29)))

(event EventOnInteract
  (params (PlayerRef :type BP%20Third%20Person%20Character%20Object%20Reference))
  (bind _returnvalue (Game|GetPlayerController 0))
  (Default|CloseEyes PlayerRef 2.0)
  (Utilities|FlowControl|Delay 2.5)
  (Game|SetGamePaused true)
  (bind _returnvalue_2 (UserInterface|CreateWidget "/Game/UI/WBP_TeleportChoice.WBP_TeleportChoice_C" 0 (Variables|Default|GetRoomSwitcherRef)))
  (UserInterface|Viewport|AddtoViewport _returnvalue_2 1)
  (Variables|/Script/Engine.PlayerController|SetbShowMouseCursor _returnvalue true)
  (Input|SetInputModeUIOnly _returnvalue 0 "DoNotLock" false))

(event EventOnReset
  (Rendering|SetActorHiddenInGame true))

(fn ConstructionScript
  (|CallParentFunction))