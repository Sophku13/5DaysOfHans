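; BP_LookAtObject is an interactable, apparently a poster, that the player can toggle a close look at.
; Each interaction toggles IsLookingAtPoster, locking or unlocking the player's camera and movement while blending the view target between this actor and the player.
; The first interaction also spawns a BP_InterMono at the player's transform with a hardcoded Room1 anatomical-scheme sound cue, then calls CheckValues on it.
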(event EventBeginPlay
  (|CallParentFunction))

(event EventOnInteract
  (params (PlayerRef :type BP%20Third%20Person%20Character%20Object%20Reference))
  (Utilities|FlowControl|Sequence
    (:then_0
      (Utilities|FlowControl|DoOnce false
        (:Completed
          (bind _returnvalue (Game|SpawnActorfromClass "/Game/SoundSystem/Sounds/BP_InterMono.BP_InterMono_C" (Transformation|GetActorTransform (Game|GetPlayerCharacter 0)) "Undefined" "MultiplyWithRoot" 0 "/Game/SoundSystem/Sounds/VoiceRecordings/NewMonologue/Room1_AtAnatomicalScheme_Cue.Room1_AtAnatomicalScheme_Cue" 1.0 "" 0.0 true 0))
          (Default|CheckValues _returnvalue))))
    (:then_1
      (if (Variables|Default|GetbIsLookingAtPoster)
        ;[0.1274 1 0.6626] OFF
        (Variables|/Game/ThirdPerson/Blueprints/BP_ThirdPersonCharacter.BP_ThirdPersonCharacter_C|SetbIsCameraLocked (Variables|Default|GetPlayerRef) false)
        (Variables|/Game/ThirdPerson/Blueprints/BP_ThirdPersonCharacter.BP_ThirdPersonCharacter_C|SetIsMovementLocked (Variables|Default|GetPlayerRef) false)
        (Game|Player|SetViewTargetwithBlend (Game|GetPlayerController 0) (Variables|Default|GetPlayerRef) 1.0 "VTBlend_Linear" 0.0 false)
        (Variables|Default|SetbIsLookingAtPoster false)
        (else
          ;[0.1274 1 0.6626] ON
          (bind _output_get (Variables|Default|SetPlayerRef PlayerRef))
          (Variables|/Game/ThirdPerson/Blueprints/BP_ThirdPersonCharacter.BP_ThirdPersonCharacter_C|SetbIsCameraLocked (Variables|Default|GetPlayerRef) true)
          (Variables|/Game/ThirdPerson/Blueprints/BP_ThirdPersonCharacter.BP_ThirdPersonCharacter_C|SetIsMovementLocked _output_get true)
          (Game|Player|SetViewTargetwithBlend (Game|GetPlayerController 0) self 1.0 "VTBlend_Linear" 0.0 false)
          (Variables|Default|SetbIsLookingAtPoster true))))))

(event Input|KeyboardEvents|B
  (params (Key :type Key%20Structure :default "None")))

(fn ConstructionScript
  (|CallParentFunction))