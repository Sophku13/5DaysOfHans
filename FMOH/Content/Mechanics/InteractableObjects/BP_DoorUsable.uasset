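; Interactable hinged door that toggles open and closed on each interaction and plays a scripted monologue the first time it is used.
; A FlipFlop drives the OpenDoor timeline forward or backward to yaw the Anchor, with open and close sounds.
; A DoOnce chain spawns four timed BP_InterMono actors carrying voice and subtitles.
; OnReset closes an open door; mouse-drag and portal-door logic remain disconnected.
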(event Input|EnhancedActionEvents|EnhancedInputActionIA_DragObjects
  (params (ActionValue :type Boolean) (ElapsedSeconds :type Float%20%28double-precision%29) (TriggeredSeconds :type Float%20%28double-precision%29) (InputAction :type Input%20Action%20Object%20Reference :default "/Game/Character/Input/Actions/IA_DragObjects.IA_DragObjects"))
  ;[1 1 1] Comment
  ;;[1 1 1] Comment
)

(event EventBeginPlay
  ;[1 1 1] Comment
  (|CallParentFunction))

(event EventOnReset
  (if (Variables|Default|GetbIsDoorOpen)
    (CallFunction|OnInteract)))

(event EventOnInteract
  (params (PlayerRef :type BP%20Third%20Person%20Character%20Object%20Reference))
  ;[1 1 1] Comment
  (Utilities|FlowControl|Sequence
    (:then_0
      (Utilities|FlowControl|DoOnce false
        (:Completed
          (Utilities|FlowControl|Delay 0.5)
          (bind _returnvalue (Game|SpawnActorfromClass "/Game/SoundSystem/Sounds/BP_InterMono.BP_InterMono_C" (Transformation|GetActorTransform (Game|GetPlayerCharacter 0)) "Undefined" "MultiplyWithRoot" 0 (Variables|Default|GetMonolog%20Sound) 1.0 (Variables|Default|GetSubtitle%20Text%201) 3.0 true 0))
          (Default|CheckValues _returnvalue)
          (Utilities|FlowControl|Delay 3.0)
          (bind _returnvalue_2 (Game|SpawnActorfromClass "/Game/SoundSystem/Sounds/BP_InterMono.BP_InterMono_C" (Transformation|GetActorTransform (Game|GetPlayerCharacter 0)) "Undefined" "MultiplyWithRoot" 0 (Variables|Default|GetSound%202) 1.0 (Variables|Default|GetSubtitle%20Text_2) 13.0 true 0))
          (Default|CheckValues _returnvalue_2)
          (Utilities|FlowControl|Delay 13.5)
          (bind _returnvalue_3 (Game|SpawnActorfromClass "/Game/SoundSystem/Sounds/BP_InterMono.BP_InterMono_C" (Transformation|GetActorTransform (Game|GetPlayerCharacter 0)) "Undefined" "MultiplyWithRoot" 0 (Variables|Default|GetSound%203) 1.0 (Variables|Default|GetSubtitle%20Text_3) 7.0 true 0))
          (Default|CheckValues _returnvalue_3)
          (Utilities|FlowControl|Delay 7.5)
          (bind _returnvalue_4 (Game|SpawnActorfromClass "/Game/SoundSystem/Sounds/BP_InterMono.BP_InterMono_C" (Transformation|GetActorTransform (Game|GetPlayerCharacter 0)) "Undefined" "MultiplyWithRoot" 0 (Variables|Default|GetSound%204) 1.0 (Variables|Default|GetSubtitle%20Text%204) 15.0 true 0))
          (Default|CheckValues _returnvalue_4))))
    (:then_1
      (Utilities|FlowControl|FlipFlop
        (:A
          (Audio|PlaySoundatLocation (Variables|Default|GetOpenDoorSound) (Transformation|GetWorldLocation (Variables|Default|GetDoor)) "0, 0, 0" 1.0 1.0 0.0 0 0 0 0)
          (Variables|Default|SetbIsDoorOpen true)
          (Audio|PlaySoundatLocation 0 "0, 0, 0" "0, 0, 0" 1.0 1.0 0.0 0 0 0 0)
          (bind _newtrack_0 (Timeline|OpenDoor PlayFromStart)
            (:Update
              (Transformation|SetRelativeRotation (Variables|Default|GetAnchor) (Math|Rotator|MakeRotator 0.0 0.0 (* _newtrack_0 90)) false false))))
        (:B
          (Audio|PlaySoundatLocation (Variables|Default|GetCloseDoorSound) (Transformation|GetWorldLocation (Variables|Default|GetDoor)) "0, 0, 0" 1.0 1.0 0.0 0 0 0 0)
          (Variables|Default|SetbIsDoorOpen false)
          (Audio|PlaySoundatLocation 0 "0, 0, 0" "0, 0, 0" 1.0 1.0 0.0 0 0 0 0)
          (Timeline|OpenDoor ReverseFromEnd))))))

(event EventTick
  (params (DeltaSeconds :type Float%20%28single-precision%29))
  ;[1 1 1] Comment
  ;;[1 1 1] Comment
)

(fn ConstructionScript
  (|CallParentFunction))

(fn CreateListOfComponents
  (Utilities|Array|Add (LocalVariables|GetDoorVar) (Variables|Default|GetDoor))
  (return (LocalVariables|GetDoorVar)))