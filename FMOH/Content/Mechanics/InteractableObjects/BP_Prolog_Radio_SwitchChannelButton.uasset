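; Interactable button for the prologue radio that switches the radio's channel when the player interacts with it.
; OnInteract calls SwitchChannel on RadioRef and prints "ButtonSound" as a debug string, with no audio played.
; A Timeline then nudges the button along local Y, offsetting from its current location each update.
; The animation runs only if IsMoving is already true, and clears that flag on finish.
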(event EventBeginPlay
  (|CallParentFunction) ; This node is disabled and will not be called.\nDrag off pins to build functionality.
)

(event Collision|EventActorBeginOverlap
  (params (OtherActor :type Actor%20Object%20Reference)))

(event EventTick
  (params (DeltaSeconds :type Float%20%28single-precision%29)))

(event EventOnInteract
  (params (PlayerRef :type BP%20Third%20Person%20Character%20Object%20Reference))
  (bind _button (Variables|Default|GetButton))
  (bind _relativelocation (Variables|/Script/Engine.SceneComponent|GetRelativeLocation _button))
  (Default|SwitchChannel (Variables|Default|GetRadioRef))
  (Development|PrintString "ButtonSound")
  (if (Variables|Default|GetbIsMoving)
    (Variables|Default|SetbIsMoving true)
    (bind _newtrack_0 (Timeline|Timeline PlayFromStart)
      (:Update
        (Transformation|SetRelativeLocation _button (Math|Vector|MakeVector (.x _relativelocation) (+ (.y _relativelocation) (* _newtrack_0 -0.5)) (.z _relativelocation)) false false))
      (:Finished
        (Variables|Default|SetbIsMoving false)))))

(fn ConstructionScript
  (|CallParentFunction))