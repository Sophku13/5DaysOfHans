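; BP_SpaceDistortion warps space by rescaling a set of actors based on the player's movement direction.
; While the player's world Y velocity is negative, Tick multiplies each ActorsToDistort scale by ScaleRange, compounding per frame; otherwise it snaps them to unit scale.
; BeginPlay stores ActorToMove locations in one unused variable, keeping only the last.
; The logic that offsets those actors by MoveRange is disconnected and never runs.
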(event EventBeginPlay
  (for _array_element (Variables|Default|GetActorToMove)
    (Variables|Default|SetObjOriginalLocation (Transformation|GetActorLocation _array_element))))

(event EventTick
  (params (DeltaSeconds :type Float%20%28single-precision%29))
  (if (< (.y (Transformation|GetVelocity (Game|GetPlayerCharacter 0))) 0.0)
    ;[1 1 1] Scaling Objects With Movement
    (for _array_element (Variables|Default|GetActorsToDistort)
      (Transformation|SetActorScale3D _array_element (* (Transformation|GetActorScale3D _array_element) (Variables|Default|GetScaleRange))))
    (else
      (for _array_element_2 (Variables|Default|GetActorsToDistort)
        (Transformation|SetActorScale3D _array_element_2 "1.000000,1.000000,1.000000")))))

(fn ConstructionScript)