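; Trigger volume that turns on camera rotation lag for the third-person character.
; When BP_ThirdPersonCharacter overlaps the Box, it sets the flag on the CameraBoom and never clears it.
; OnReset sets the Box collision to query-only.
; BeginPlay caches the HDRI skylight intensity, but the timeline fade that uses it and the collision-disable node are unwired leftovers.
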(event OnComponentBeginOverlap(Box)
  (params (OverlappedComponent :type Primitive%20Component%20Object%20Reference) (OtherActor :type Actor%20Object%20Reference) (OtherComp :type Primitive%20Component%20Object%20Reference) (OtherBodyIndex :type Integer) (bFromSweep :type Boolean) (SweepResult :type Hit%20Result%20Structure%20%28by%20ref%29))
  (bind _asbp_third_person_character (Utilities|Casting|CastToBP_ThirdPersonCharacter OtherActor))
  (Variables|/Script/Engine.SpringArmComponent|SetbEnableCameraRotationLag (Variables|/Game/ThirdPerson/Blueprints/BP_ThirdPersonCharacter.BP_ThirdPersonCharacter_C|GetCameraBoom _asbp_third_person_character) true))

(event EventBeginPlay
  (|CallParentFunction)
  (Variables|Default|SetOriginalIntensity (Variables|/Script/Engine.LightComponentBase|GetIntensity (Variables|/HDRIBackdrop/Blueprints/HDRIBackdrop.HDRIBackdrop_C|GetSkylight (Variables|Default|GetHDRIRef)))))

(event Collision|EventActorBeginOverlap
  (params (OtherActor :type Actor%20Object%20Reference)))

(event EventTick
  (params (DeltaSeconds :type Float%20%28single-precision%29)))

(event EventOnReset
  (Collision|SetCollisionEnabled (Variables|Default|GetBox) "QueryOnly"))

(fn ConstructionScript
  (|CallParentFunction))