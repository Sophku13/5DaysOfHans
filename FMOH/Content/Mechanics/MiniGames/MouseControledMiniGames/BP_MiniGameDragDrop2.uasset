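; BP_MiniGameDragDrop2 is an interactable actor that acts as the entry point to a mouse-controlled drag-and-drop minigame.
; On interact, it passes the player reference to its referenced pawn, has the first player controller possess that pawn, and blends the view to itself.
; The activation event is empty, and this graph holds no drag-and-drop logic or return to the player.
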(event EventBeginPlay
  (|CallParentFunction) ; This node is disabled and will not be called.\nDrag off pins to build functionality.
)

(event Collision|EventActorBeginOverlap
  (params (OtherActor :type Actor%20Object%20Reference))
  (|CallParentFunction OtherActor) ; This node is disabled and will not be called.\nDrag off pins to build functionality.
)

(event EventTick
  (params (DeltaSeconds :type Float%20%28single-precision%29))
  (|CallParentFunction DeltaSeconds) ; This node is disabled and will not be called.\nDrag off pins to build functionality.
)

(event EventOnActivation
  (params (PlayerRef :type BP%20Third%20Person%20Character%20Object%20Reference)))

(event EventOnInteract
  (params (PlayerRef :type BP%20Third%20Person%20Character%20Object%20Reference))
  (bind _returnvalue (Game|GetPlayerController 0))
  (bind _pawnref (Variables|Default|GetPawnRef))
  ;[1 1 1] Switch the Pawns and the View
  (Variables|/Game/Mechanics/MiniGames/MouseControledMiniGames/BP_GrabPawn.BP_GrabPawn_C|SetPlayerRef _pawnref PlayerRef)
  (Pawn|Possess _returnvalue _pawnref)
  (Game|Player|SetViewTargetwithBlend _returnvalue self 1.0 "VTBlend_Linear" 0.0 false))

(fn ConstructionScript
  (|CallParentFunction))