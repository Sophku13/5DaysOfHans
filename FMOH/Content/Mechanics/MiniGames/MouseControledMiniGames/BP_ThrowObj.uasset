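; Throwing minigame actor that takes over the player's view and moves its camera along a spline to track the thrown object.
; On BeginPlay it caches BP_GrabPawn; once that pawn's object is released, Tick clears GrabMode and interpolates the camera toward the spline point closest to ObjToThrow.
; An older follow-distance path using GetClosestPointOnSpline is disconnected; that function's comparison keeps the farthest sample, despite its name.
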(event EventBeginPlay
  (Game|Player|SetViewTargetwithBlend (Game|GetPlayerController 0) self 0.0 "VTBlend_Linear" 0.0 false)
  (Actor|Tick|SetActorTickEnabled true)
  (bind _returnvalue (Actor|GetActorOfClass "/Game/Mechanics/MiniGames/MouseControledMiniGames/BP_GrabPawn.BP_GrabPawn_C"))
  (Variables|Default|SetGarbPawnRef _returnvalue))

(event EventTick
  (params (DeltaSeconds :type Float%20%28single-precision%29))
  (bind _garbpawnref (Variables|Default|GetGarbPawnRef))
  (bind _camera (Variables|Default|GetCamera))
  (if (Variables|/Game/Mechanics/MiniGames/MouseControledMiniGames/BP_GrabPawn.BP_GrabPawn_C|GetObjIsReleased _garbpawnref)
    (Variables|/Game/Mechanics/MiniGames/MouseControledMiniGames/BP_GrabPawn.BP_GrabPawn_C|SetbGrabMode _garbpawnref false)
    (Transformation|SetWorldLocation _camera (Math|Interpolation|VInterpTo (Transformation|GetWorldLocation _camera) (Spline|FindLocationClosesttoWorldLocation (Variables|Default|GetSpline) (Transformation|GetWorldLocation (Variables|Default|GetObjToThrow)) "World") (Utilities|Time|GetWorldDeltaSeconds) 1.0) false false)))

(fn ConstructionScript)

(fn GetClosestPointonSpline
  (params (WhereIsTheObj :type Vector))
  (bind _spline (Variables|Default|GetSpline))
  (if (< (LocalVariables|GetCheckLength) (Spline|GetSplineLength _spline)) :!label _label
    (if (> (Math|Vector|Distance(Vector) (Spline|GetLocationatDistanceAlongSpline _spline (LocalVariables|GetCheckLength) "World") (Variables|Default|GetWhere%20Is%20the%20Obj)) (LocalVariables|GetClosestDistance))
      (LocalVariables|SetClosestDistance (Math|Vector|Distance(Vector) (Spline|GetLocationatDistanceAlongSpline _spline (LocalVariables|GetCheckLength) "World") (Variables|Default|GetWhere%20Is%20the%20Obj)))
      (LocalVariables|SetLengthAtClosestDistance (LocalVariables|GetCheckLength)))
    (LocalVariables|SetCheckLength (+ (LocalVariables|GetCheckLength) 5.0))
    (goto _label)
    (else
      (return (LocalVariables|GetLengthAtClosestDistance)))))