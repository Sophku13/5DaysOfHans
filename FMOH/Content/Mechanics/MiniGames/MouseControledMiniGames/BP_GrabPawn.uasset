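; Free-moving pawn that lets the player drag objects with the mouse, with G toggling between mouse look and a cursor-driven grab mode.
; Left click in grab mode traces under the cursor for a Movable component and stores its hit distance.
; Tick holds it at that distance along the cursor ray, using a PhysicsHandle for simulating bodies (bone-aware on skeletal meshes) and SetWorldLocation with the stored grab offset otherwise.
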(event EventTick
  (params (DeltaSeconds :type Float%20%28single-precision%29))
  (bind _returnvalue (Game|GetPlayerController 0))
  (bind _grabbedobj (Variables|Default|GetGrabbedObj))
  (bind _originaldistance (Variables|Default|GetOriginalDistance))
  (bind (_worldlocation _worlddirection) (Game|Player|ConvertMouseLocationToWorldSpace _returnvalue))
  (bind _returnvalue_2 (* _worlddirection _originaldistance))
  (bind _returnvalue_3 (+ _worldlocation _returnvalue_2))
  (if (Variables|Default|GetbGrabMode)
    (Utilities|IsValid _grabbedobj
      (:Is%20Valid
        (if (Physics|IsSimulatingPhysics _grabbedobj "None")
          (Physics|Components|PhysicsHandle|SetTargetLocation (Variables|Default|GetPhysicsHandle) _returnvalue_3)
          (else
            (Transformation|SetWorldLocation (Variables|Default|GetGrabbedObj) (Math|Transform|InverseTransformLocation (Math|Conversions|ToTransform(Vector) (Variables|Default|GetRelativeGrabLocation)) _returnvalue_3) false false)))))))

(event Input|AxisEvents|InputAxisLookUp/DownMouse
  (params (AxisValue :type Float%20%28single-precision%29))
  ;[1 1 1] ReturnTheCameraInput
  (if (not (Variables|Default|GetbGrabMode))
    (Pawn|Input|AddControllerPitchInput AxisValue)))

(event Input|AxisEvents|InputAxisTurnRight/LeftMouse
  (params (AxisValue :type Float%20%28single-precision%29))
  ;[1 1 1] ReturnTheCameraInput
  (if (not (Variables|Default|GetbGrabMode))
    (Pawn|Input|AddControllerYawInput AxisValue)))

(event Input|AxisEvents|InputAxisMoveForward/Backward
  (params (AxisValue :type Float%20%28single-precision%29))
  (Transformation|AddActorWorldOffset (* (Math|Vector|GetForwardVector (Transformation|GetActorRotation (Pawn|GetController))) (* AxisValue 1e+01))))

(event Input|AxisEvents|InputAxisMoveRight/Left
  (params (AxisValue :type Float%20%28single-precision%29))
  (Transformation|AddActorWorldOffset (* (Math|Vector|GetRightVector (Transformation|GetActorRotation (Pawn|GetController))) (* AxisValue 1e+01))))

(event Input|KeyboardEvents|G
  (params (Key :type Key%20Structure :default "None"))
  (bind _returnvalue (Game|GetPlayerController 0))
  ;[1 1 1] SwitchGrabMode
  (:Pressed
    (Variables|Default|SetbGrabMode (not (Variables|Default|GetbGrabMode)))
    (Variables|/Script/Engine.PlayerController|SetbShowMouseCursor _returnvalue (not (Variables|/Script/Engine.PlayerController|GetbShowMouseCursor _returnvalue)))))

(event Input|MouseEvents|LeftMouseButton
  (params (Key :type Key%20Structure :default "None"))
  (bind _returnvalue (Game|GetPlayerController 0))
  (bind _bgrabmode (Variables|Default|GetbGrabMode))
  (bind (_worldlocation _worlddirection) (Game|Player|ConvertMouseLocationToWorldSpace _returnvalue))
  (:Pressed
    (if _bgrabmode
      ;[1 1 1] LookAtComponentUnderTheMouse
      (bind (_outhit _returnvalue_2) (Collision|LineTraceByChannel _worldlocation (+ _worldlocation (* _worlddirection (Math|Conversions|ToVector(Float) 1e+05))) "TraceTypeQuery1" false 0 "ForDuration"))
      (if _returnvalue_2
        (if (Utilities|Enum|Equal(Enum) (Variables|/Script/Engine.SceneComponent|GetMobility (.HitComponent (Collision|BreakHitResult _outhit))) "Movable")
          ;[1 1 1] RemeberDistanceAndComponent
          (Variables|Default|SetOriginalDistance (.Distance (Collision|BreakHitResult _outhit)))
          (Variables|Default|SetGrabbedObj (.HitComponent (Collision|BreakHitResult _outhit)))
          (if (Physics|IsSimulatingPhysics (.HitComponent (Collision|BreakHitResult _outhit)) "None")
            (Utilities|Casting|CastToSkeletalMeshComponent (Variables|Default|GetGrabbedObj)
              (:then
                (Variables|Default|SetName (.HitBoneName (Collision|BreakHitResult _outhit))))
              (:CastFailed
                _))
            (Class|PhysicsHandleComponent|GrabComponentatLocation (Variables|Default|GetPhysicsHandle) (Variables|Default|GetGrabbedObj) (Variables|Default|GetName) (.Location (Collision|BreakHitResult _outhit)))
            (else
              (Variables|Default|SetRelativeGrabLocation (Math|Transform|InverseTransformLocation (Math|Conversions|ToTransform(Vector) (Transformation|GetWorldLocation (.HitComponent (Collision|BreakHitResult _outhit)))) (.Location (Collision|BreakHitResult _outhit))))))))))
  (:Released
    (if _bgrabmode
      ;[1 1 1] Release component
      (Variables|Default|SetGrabbedObj 0)
      (Physics|Components|PhysicsHandle|ReleaseComponent (Variables|Default|GetPhysicsHandle)))))

(fn ConstructionScript)