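; BP_AnatomicalMinigame is a minigame actor that penalizes contact with its Box collision by sending a Sphere back to a Start transform.
; On overlap, the Sphere turns red, the PointLight goes black, and the Sphere resets after a short delay if the overlap flag is still set.
; Ending the overlap clears the flag, then restores the blue material and white light after a delay.
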(event OnComponentBeginOverlap(Box)
  (params (OverlappedComponent :type Primitive%20Component%20Object%20Reference) (OtherActor :type Actor%20Object%20Reference) (OtherComp :type Primitive%20Component%20Object%20Reference) (OtherBodyIndex :type Integer) (bFromSweep :type Boolean) (SweepResult :type Hit%20Result%20Structure%20%28by%20ref%29))
  (bind _start (Variables|Default|GetStart))
  (bind _returnvalue (Transformation|GetWorldTransform _start))
  (Variables|Default|SetIs%20overlappong true)
  (Rendering|Material|SetMaterial (Variables|Default|GetSphere) 0 "/Engine/EngineDebugMaterials/VertexColorViewMode_RedOnly.VertexColorViewMode_RedOnly")
  (Rendering|Components|Light|SetLightColor (Variables|Default|GetPointLight) "(R=0.000000,G=0.000000,B=0.000000,A=1.000000)" true)
  (Utilities|FlowControl|Delay 1.0)
  (if (Variables|Default|GetIs%20overlappong)
    (Transformation|SetWorldLocationAndRotation (Variables|Default|GetSphere) (.location _returnvalue) (.rotation _returnvalue) false false)))

(event OnComponentEndOverlap(Box)
  (params (OverlappedComponent :type Primitive%20Component%20Object%20Reference) (OtherActor :type Actor%20Object%20Reference) (OtherComp :type Primitive%20Component%20Object%20Reference) (OtherBodyIndex :type Integer))
  (Variables|Default|SetIs%20overlappong false)
  (Utilities|FlowControl|Delay 0.5)
  (Rendering|Material|SetMaterial (Variables|Default|GetSphere) 0 "/Engine/EngineDebugMaterials/VertexColorViewMode_BlueOnly.VertexColorViewMode_BlueOnly")
  (Rendering|Components|Light|SetLightColor (Variables|Default|GetPointLight) "(R=1.000000,G=1.000000,B=1.000000,A=1.000000)" true))

(event EventBeginPlay)

(event Collision|EventActorBeginOverlap
  (params (OtherActor :type Actor%20Object%20Reference)))

(event EventTick
  (params (DeltaSeconds :type Float%20%28single-precision%29)))

(fn ConstructionScript)