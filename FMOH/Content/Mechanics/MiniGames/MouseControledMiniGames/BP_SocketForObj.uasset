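; BP_SocketForObj is a socket actor for the mouse-controlled minigames that detects when the object held by BP_GrabPawn is near it.
; On BeginPlay it caches the BP_GrabPawn in the level.
; Its Sphere overlap sets IsNearSocket when the grabbed component enters while the pawn's SocketIsTaken is false, printing a debug string, and clears it when that component leaves.
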(event OnComponentBeginOverlap(Sphere)
  (params (OverlappedComponent :type Primitive%20Component%20Object%20Reference) (OtherActor :type Actor%20Object%20Reference) (OtherComp :type Primitive%20Component%20Object%20Reference) (OtherBodyIndex :type Integer) (bFromSweep :type Boolean) (SweepResult :type Hit%20Result%20Structure%20%28by%20ref%29))
  (bind _grabpawnref (Variables|Default|GetGrabPawnRef))
  (if (not (Variables|/Game/Mechanics/MiniGames/MouseControledMiniGames/BP_GrabPawn.BP_GrabPawn_C|GetSocketIsTaken _grabpawnref))
    (if (== OtherComp (Variables|/Game/Mechanics/MiniGames/MouseControledMiniGames/BP_GrabPawn.BP_GrabPawn_C|GetGrabbedObj _grabpawnref))
      (Variables|Default|SetIsNearSocket true)
      (Development|PrintString "Socket is Near"))))

(event OnComponentEndOverlap(Sphere)
  (params (OverlappedComponent :type Primitive%20Component%20Object%20Reference) (OtherActor :type Actor%20Object%20Reference) (OtherComp :type Primitive%20Component%20Object%20Reference) (OtherBodyIndex :type Integer))
  (if (== OtherComp (Variables|/Game/Mechanics/MiniGames/MouseControledMiniGames/BP_GrabPawn.BP_GrabPawn_C|GetGrabbedObj (Variables|Default|GetGrabPawnRef)))
    (Variables|Default|SetIsNearSocket false)))

(event EventBeginPlay
  (bind _returnvalue (Actor|GetActorOfClass "/Game/Mechanics/MiniGames/MouseControledMiniGames/BP_GrabPawn.BP_GrabPawn_C"))
  (Variables|Default|SetGrabPawnRef _returnvalue))

(event Collision|EventActorBeginOverlap
  (params (OtherActor :type Actor%20Object%20Reference)))

(event EventTick
  (params (DeltaSeconds :type Float%20%28single-precision%29)))

(fn ConstructionScript)