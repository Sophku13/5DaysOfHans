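; Interactable door for the parents-fighting minigame, which plays a locked sound and a one-time monologue when the parents are not fighting.
; During an unfinished fight, interaction locks the player, blends to this actor's view, reveals a video and opens WBP_ParentsFighting with options from DialogOptionList.
; SetSelectedOption marks used options false, and OnActivation restores control, stopping the arguing sound if the quest is complete.
; OpenDoor swings the Anchor via Timeline.
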(event Custom|OpenDoor
  (Audio|PlaySoundatLocation "/Game/SoundSystem/Sounds/SFX/Door/SC_OpenDoor_3_Cue.SC_OpenDoor_3_Cue" "0, 0, 0" "0, 0, 0" 1.0 1.0 0.0 0 0 0 0)
  (bind _newtrack_0 (Timeline|Timeline PlayFromStart)
    (:Update
      (Transformation|SetRelativeRotation (Variables|Default|GetAnchor) (Math|Rotator|MakeRotator 0.0 0.0 (* _newtrack_0 -90)) false false))))

(event Custom|MakeVisible
  (Development|SetHiddeninGame (Variables|Default|GetVideo) false false))

(event Custom|MakeHidden
  (Development|SetHiddeninGame (Variables|Default|GetVideo) false false))

(event Custom|SetSelectedOption
  (params (ActionName :type Name))
  (Utilities|Map|Add (Variables|Default|GetDialogOptionList) ActionName false))

(event Custom|MovePlayer
  (bind _hanslocation (Variables|Default|GetHansLocation))
  (Transformation|SetActorLocationAndRotation (Variables|Default|GetPlayer%20Ref) (Transformation|GetWorldLocation _hanslocation) (Transformation|GetWorldRotation _hanslocation) false true))

(event EventTick
  (params (DeltaSeconds :type Float%20%28single-precision%29)))

(event EventOnActivation
  (params (PlayerRef :type BP%20Third%20Person%20Character%20Object%20Reference))
  (bind _returnvalue (Game|GetPlayerController 0))
  (bind _output_get (Variables|Default|SetPlayer%20Ref PlayerRef))
  (Variables|/Game/ThirdPerson/Blueprints/BP_ThirdPersonCharacter.BP_ThirdPersonCharacter_C|SetIsMovementLocked _output_get false)
  (Variables|/Game/ThirdPerson/Blueprints/BP_ThirdPersonCharacter.BP_ThirdPersonCharacter_C|SetbIsCameraLocked _output_get false)
  (Variables|/Script/Engine.PlayerController|SetbShowMouseCursor _returnvalue false)
  (Input|SetInputModeGameOnly _returnvalue false)
  (Game|Player|SetViewTargetwithBlend _returnvalue (Game|GetPlayerCharacter 0) 1.0 "VTBlend_Linear" 0.0 false)
  (CallFunction|MakeHidden)
  (if (Variables|Default|GetbQuestCompleted)
    (bind _returnvalue_2 (Actor|GetActorOfClass "/Game/SoundSystem/Sounds/VoiceRecordings/Parents/BP_ParentsArguingSound.BP_ParentsArguingSound_C"))
    (Default|EventStopShouting _returnvalue_2)))

(event EventOnInteract
  (params (PlayerRef :type BP%20Third%20Person%20Character%20Object%20Reference))
  (bind _returnvalue (Game|GetPlayerController 0))
  (bind _returnvalue_2 (Game|GetPlayerController 0))
  (bind _dialogoptionlist (Variables|Default|GetDialogOptionList))
  ;[1 1 1] Switch the Pawns and the View
  (if (Variables|Default|GetbParentsAreFighting)
    (if (not (Variables|Default|GetbQuestCompleted))
      (bind _output_get (Variables|Default|SetPlayer%20Ref PlayerRef))
      (Variables|/Game/ThirdPerson/Blueprints/BP_ThirdPersonCharacter.BP_ThirdPersonCharacter_C|SetIsMovementLocked _output_get true)
      (Variables|/Game/ThirdPerson/Blueprints/BP_ThirdPersonCharacter.BP_ThirdPersonCharacter_C|SetbIsCameraLocked _output_get true)
      (Variables|/Game/Mechanics/BaseBlueprints/BP_RoomSwitcher.BP_RoomSwitcher_C|SetCharacterRef (Variables|Default|GetRoomSwitcherRef) _output_get)
      (Variables|/Script/Engine.PlayerController|SetbShowMouseCursor _returnvalue_2 true)
      (Game|Player|SetViewTargetwithBlend _returnvalue_2 self 1.0 "VTBlend_Linear" 0.0 false)
      (bind _returnvalue_3 (UserInterface|CreateWidget "/Game/Mechanics/MiniGames/ParentsFighting/WBP_ParentsFighting.WBP_ParentsFighting_C" _returnvalue self (Variables|Default|GetPlayer%20Ref) (.Value (Utilities|Map|Find _dialogoptionlist "Break")) (.Value (Utilities|Map|Find _dialogoptionlist "Hurt")) (.Value (Utilities|Map|Find _dialogoptionlist "Letter")) (.Value (Utilities|Map|Find _dialogoptionlist "Piano")) (.Value (Utilities|Map|Find _dialogoptionlist "Play")) (.Value (Utilities|Map|Find _dialogoptionlist "Shout")) (.Value (Utilities|Map|Find _dialogoptionlist "Sing"))))
      (UserInterface|Viewport|AddtoViewport _returnvalue_3 0)
      (Input|SetInputModeUIOnly _returnvalue 0 "DoNotLock" false)
      (CallFunction|MakeVisible)
      (CallFunction|MovePlayer))
    (else
      (Audio|PlaySound2D (Variables|Default|Getlocked_door_sound) 1.0 1.0 0.0 0 0)
      (Utilities|FlowControl|Delay 0.2)
      (Utilities|FlowControl|DoOnce false
        (:Completed
          (bind _returnvalue_4 (Game|SpawnActorfromClass "/Game/SoundSystem/Sounds/BP_InterMono.BP_InterMono_C" (Transformation|GetActorTransform (Game|GetPlayerCharacter 0)) "Undefined" "MultiplyWithRoot" 0 (Variables|Default|GetMonolog) 1.0 (Variables|Default|GetSubtitle%20Text) 5.0 true 0))
          (Default|CheckValues _returnvalue_4))))))

(fn ConstructionScript
  (|CallParentFunction))