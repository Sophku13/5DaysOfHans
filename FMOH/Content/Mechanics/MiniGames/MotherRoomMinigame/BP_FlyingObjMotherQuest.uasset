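; BP_FlyingObjMotherQuest is an actor for the Mother Room minigame, set up as an object that flies from a spawn point toward the character.
; A timeline with play rate 1/Speed lerps its transform from SpawnLocation1 to CharacterLocation on MiniGameRef, then destroys the actor.
; The location lerp targets CharacterLocation's scale rather than its location.
; This flight logic is unconnected and never runs, and BeginPlay is empty.
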(event EventBeginPlay)

(fn ConstructionScript)