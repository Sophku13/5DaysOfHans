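; Shooting minigame in the mother's bedroom, started by interacting with it, that plays out Hans's dialogue with his mother.
; Interaction locks the player in place, sets the train targets moving along splines and shows a counter widget; left click fires projectiles.
; Each hit lowers a countdown and spawns subtitle exchanges.
; At zero it stops the trains, teleports the player behind closed eyes, restores movement, stops music, unlocks a door and shows a closing monologue.
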(event Custom|SpawnObjects
  ;[1 1 1] MakingObjsMOve
  (bind _outactors (Actor|GetAllActorsOfClass "/Game/Mechanics/InteractableObjects/Train/BP_Train2.BP_Train2_C"))
  (bind _output_get (Variables|Default|SetTrainRef _outactors))
  (Class|BPISplineTrain|MoveObjAlongSpline(Message) _output_get))

(event Custom|GameIsOver
  (bind _lockeddoorref (Variables|Default|GetLockedDoorRef))
  (bind _playerref (Variables|Default|GetPlayerRef))
  ;[1 1 1] Finish Minigame
  (Default|CloseEyes _playerref 1.0)
  (Utilities|FlowControl|Delay 1.0)
  (Transformation|SetActorLocation (Game|GetPlayerCharacter 0) (Transformation|GetWorldLocation (Variables|/Game/Mechanics/MiniGames/MotherRoomMinigame/BP_MothersRoom.BP_MothersRoom_C|GetTP_DestinationEnd (Variables|Default|GetMother'sRoomRef))) false true)
  (Variables|/Game/ThirdPerson/Blueprints/BP_ThirdPersonCharacter.BP_ThirdPersonCharacter_C|SetbIsInMinigame _playerref false)
  ;[1 0 0] Trying To Set movement bakc to unlocked in Third Person
  (Variables|/Game/ThirdPerson/Blueprints/BP_ThirdPersonCharacter.BP_ThirdPersonCharacter_C|SetIsMovementLocked _playerref false)
  (Default|TurnMusicOff (Variables|Default|GetMiniGameMusicRef))
  (Variables|/Game/Mechanics/InteractableObjects/BP_DoorKeyLocked.BP_DoorKeyLocked_C|SetbIsDoorKeyAquired _lockeddoorref true)
  (Default|OnInteract _lockeddoorref)
  (Input|DisableInput (Game|GetPlayerController 0))
  (Utilities|FlowControl|Delay 0.5)
  (Default|OpenEyes (Variables|Default|GetPlayerRef) 1.0)
  (Utilities|FlowControl|Delay 2.0)
  (bind _returnvalue (Game|SpawnActorfromClass "/Game/SoundSystem/Sounds/BP_InterMono.BP_InterMono_C" (Transformation|GetActorTransform (Game|GetPlayerCharacter 0)) "Undefined" "MultiplyWithRoot" 0 0 1.0 "Life with her was like a war. It flared up and faded away, leaving Hans in the dark. In which he could barely make out his own silhouette." 7.0 true 0))
  (Default|CheckValues _returnvalue))

(event EventObjectIsHit
  ;[1 1 1] CountingObjects in the Array
  (Development|PrintString "Hello")
  (bind _result (Math|Integer|DecrementInt (Variables|Default|GetCountOfAllObjects))
    (:%20%20
      (if (> _result 0)
        (bind _output_get (Variables|Default|SetCountOfAllObjects _result))
        (Development|PrintString (Utilities|String|ToString(Integer) _output_get))
        ;[0 1 0.5634] We are counting down so start at 4 after first one got hit
        (switch int _output_get
          (:1
            (Development|PrintString "Audio after Hit #4")
            (bind _returnvalue (Game|SpawnActorfromClass "/Game/SoundSystem/Sounds/BP_InterMono.BP_InterMono_C" (Transformation|GetActorTransform (Game|GetPlayerCharacter 0)) "Undefined" "MultiplyWithRoot" 0 0 1.0 "Mother: You have the most beautiful eyes." 0.0 true 0))
            (Default|CheckValues _returnvalue)
            (Utilities|FlowControl|Delay 0.5)
            (bind _returnvalue_2 (Game|SpawnActorfromClass "/Game/SoundSystem/Sounds/BP_InterMono.BP_InterMono_C" (Transformation|GetActorTransform (Game|GetPlayerCharacter 0)) "Undefined" "MultiplyWithRoot" 0 0 1.0 "Hans: Mama, eat. You haven't eaten in days." 0.0 true 0))
            (Default|CheckValues _returnvalue_2))
          (:2
            (Development|PrintString "Audio after Hit #3")
            (bind _returnvalue_3 (Game|SpawnActorfromClass "/Game/SoundSystem/Sounds/BP_InterMono.BP_InterMono_C" (Transformation|GetActorTransform (Game|GetPlayerCharacter 0)) "Undefined" "MultiplyWithRoot" 0 0 1.0 "Mother: You're the most beautiful boy in the world, Hans." 0.0 true 0))
            (Default|CheckValues _returnvalue_3)
            (Utilities|FlowControl|Delay 0.5)
            (bind _returnvalue_4 (Game|SpawnActorfromClass "/Game/SoundSystem/Sounds/BP_InterMono.BP_InterMono_C" (Transformation|GetActorTransform (Game|GetPlayerCharacter 0)) "Undefined" "MultiplyWithRoot" 0 0 1.0 "Hans: Mama, it's too loud in here." 0.0 true 0))
            (Default|CheckValues _returnvalue_4))
          (:3
            (Development|PrintString "Audio after Hit #2")
            (bind _returnvalue_5 (Game|SpawnActorfromClass "/Game/SoundSystem/Sounds/BP_InterMono.BP_InterMono_C" (Transformation|GetActorTransform (Game|GetPlayerCharacter 0)) "Undefined" "MultiplyWithRoot" 0 0 1.0 "Mother: Stop whining, baby. We've got all night." 0.0 true 0))
            (Default|CheckValues _returnvalue_5)
            (Utilities|FlowControl|Delay 0.5)
            (bind _returnvalue_6 (Game|SpawnActorfromClass "/Game/SoundSystem/Sounds/BP_InterMono.BP_InterMono_C" (Transformation|GetActorTransform (Game|GetPlayerCharacter 0)) "Undefined" "MultiplyWithRoot" 0 0 1.0 "Hans: Mama, get dressed." 0.0 true 0))
            (Default|CheckValues _returnvalue_6))
          (:4
            (Development|PrintString "Audio after Hit #1")
            (bind _returnvalue_7 (Game|SpawnActorfromClass "/Game/SoundSystem/Sounds/BP_InterMono.BP_InterMono_C" (Transformation|GetActorTransform (Game|GetPlayerCharacter 0)) "Undefined" "MultiplyWithRoot" 0 0 1.0 "Mother: I love you, Hans." 0.0 true 0))
            (Default|CheckValues _returnvalue_7)
            (Utilities|FlowControl|Delay 0.5)
            (bind _returnvalue_8 (Game|SpawnActorfromClass "/Game/SoundSystem/Sounds/BP_InterMono.BP_InterMono_C" (Transformation|GetActorTransform (Game|GetPlayerCharacter 0)) "Undefined" "MultiplyWithRoot" 0 0 1.0 "Hans: Mama, I want to go home." 0.0 true 0))
            (Default|CheckValues _returnvalue_8)))
        (else
          (for _array_element (Variables|Default|GetTrainRef)
            (Default|StopMovementAlongSpline _array_element))
          (Widget|RemovefromParent (Variables|Default|GetCountWidgetRef))
          (Default|StartBlink (Variables|Default|GetPlayerRef) 1.0 1.0)
          (Utilities|FlowControl|Delay 1.0)
          (CallFunction|GameIsOver))))))

(event EventOnInteract
  (params (PlayerRef :type BP%20Third%20Person%20Character%20Object%20Reference))
  (bind _characterlocation (Variables|Default|GetCharacterLocation))
  (bind _returnvalue (Transformation|GetWorldTransform _characterlocation))
  ;[1 1 1] Teleporting player to the position
  (Variables|Default|SetPlayerRef PlayerRef)
  (Transformation|SetActorLocationAndRotation PlayerRef (.location _returnvalue) (.rotation _returnvalue))
  (Variables|/Game/ThirdPerson/Blueprints/BP_ThirdPersonCharacter.BP_ThirdPersonCharacter_C|SetIsMovementLocked PlayerRef true)
  (CallFunction|SpawnObjects)
  (Input|EnableInput (Game|GetPlayerController 0))
  (bind _returnvalue_2 (Actor|GetActorOfClass "/Game/Mechanics/MiniGames/MotherRoomMinigame/BP_MothersRoom.BP_MothersRoom_C"))
  (Variables|Default|SetMother'sRoomRef _returnvalue_2)
  (bind _returnvalue_3 (UserInterface|CreateWidget "/Game/UI/WBP_MotherRoomCount.WBP_MotherRoomCount_C" (Game|GetPlayerController 0) self))
  (bind _output_get (Variables|Default|SetCountWidgetRef _returnvalue_3))
  (UserInterface|Viewport|AddtoViewport _output_get 0)
  (Variables|/Game/ThirdPerson/Blueprints/BP_ThirdPersonCharacter.BP_ThirdPersonCharacter_C|SetbIsInMinigame (Variables|Default|GetPlayerRef) true)
  (Variables|/Game/ThirdPerson/Blueprints/BP_ThirdPersonCharacter.BP_ThirdPersonCharacter_C|SetActiveMinigameName (Variables|Default|GetPlayerRef) "Shoot"))

(event Input|MouseEvents|LeftMouseButton
  (params (Key :type Key%20Structure :default "None"))
  ;[1 1 1] Shoot
  (:Pressed
    (Game|SpawnActorfromClass "/Game/Mechanics/MiniGames/MotherRoomMinigame/BP_ProjectileMother.BP_ProjectileMother_C" (Math|Transform|MakeTransform (.location (Transformation|GetWorldTransform (Variables|/Game/ThirdPerson/Blueprints/BP_ThirdPersonCharacter.BP_ThirdPersonCharacter_C|GetItemArrow (stale EventOnInteract PlayerRef)))) (.rotation (Transformation|GetWorldTransform (Variables|/Game/ThirdPerson/Blueprints/BP_ThirdPersonCharacter.BP_ThirdPersonCharacter_C|GetItemArrow (stale EventOnInteract PlayerRef)))) "1.000000,1.000000,1.000000") "AlwaysSpawn" "MultiplyWithRoot" 0 0)))

(fn ConstructionScript
  (|CallParentFunction))