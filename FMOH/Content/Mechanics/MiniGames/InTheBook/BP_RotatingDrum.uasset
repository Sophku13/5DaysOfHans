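; Rotating drum actor for the InTheBook minigame that turns while the player's pawn is jumping.
; BeginPlay caches the level's BP_ControlablePawn, and Tick checks its PawnIsJumping flag.
; While the flag is set, Tick adds a fixed one-degree step to the actor's rotation each frame, so speed depends on frame rate.
; A RotateDrum timeline for a full-turn lerp is present but never runs.
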(event EventBeginPlay
  (bind _returnvalue (Actor|GetActorOfClass "/Game/Mechanics/MiniGames/InTheBook/BP_ControlablePawn.BP_ControlablePawn_C"))
  (Variables|Default|SetControlablePawn _returnvalue))

(event Collision|EventActorBeginOverlap
  (params (OtherActor :type Actor%20Object%20Reference)))

(event EventTick
  (params (DeltaSeconds :type Float%20%28single-precision%29))
  (if (Variables|/Game/Mechanics/MiniGames/InTheBook/BP_ControlablePawn.BP_ControlablePawn_C|GetbPawnIsJumping (Variables|Default|GetControlablePawn))
    (Transformation|SetActorRotation (Math|Rotator|CombineRotators (Transformation|GetWorldRotation (Variables|Default|GetDefaultSceneRoot)) "1.000000,0.000000,0.000000"))))

(fn ConstructionScript)