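; Interactable rotating drum minigame actor that hands the player control of its own pawn.
; On interact, it passes the player reference to ControlablePawn, has the player controller possess it and blends the camera to this actor.
; While that pawn is jumping, Tick turns Base by a fixed one-degree step per frame, independent of DeltaSeconds, feeding its world rotation back in as relative rotation.
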(event EventBeginPlay
  (|CallParentFunction) ; This node is disabled and will not be called.\nDrag off pins to build functionality.
)

(event Collision|EventActorBeginOverlap
  (params (OtherActor :type Actor%20Object%20Reference))
  (|CallParentFunction OtherActor) ; This node is disabled and will not be called.\nDrag off pins to build functionality.
)

(event EventTick
  (params (DeltaSeconds :type Float%20%28single-precision%29))
  (|CallParentFunction DeltaSeconds)
  (if (Variables|/Game/Mechanics/MiniGames/InTheBook/BP_ControlablePawn.BP_ControlablePawn_C|GetbPawnIsJumping (Variables|Default|GetControlablePawn))
    (Transformation|SetRelativeRotation (Variables|Default|GetBase) (Math|Rotator|CombineRotators (Transformation|GetWorldRotation (Variables|Default|GetBase)) "1.000000,0.000000,0.000000") false false)))

(event EventOnActivation
  (params (PlayerRef :type BP%20Third%20Person%20Character%20Object%20Reference)))

(event EventOnInteract
  (params (PlayerRef :type BP%20Third%20Person%20Character%20Object%20Reference))
  (bind _returnvalue (Game|GetPlayerController 0))
  (bind _controlablepawn (Variables|Default|GetControlablePawn))
  ;[1 1 1] Switch the Pawns and the View
  (Variables|/Game/Mechanics/MiniGames/InTheBook/BP_ControlablePawn.BP_ControlablePawn_C|SetPlayerRef _controlablepawn PlayerRef)
  (Pawn|Possess _returnvalue _controlablepawn)
  (Game|Player|SetViewTargetwithBlend _returnvalue self 1.0 "VTBlend_Linear" 0.0 false))

(fn ConstructionScript
  (|CallParentFunction))