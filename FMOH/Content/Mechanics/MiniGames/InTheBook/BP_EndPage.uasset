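; BP_EndPage is a trigger at the end of a page in the in-book side-view minigame.
; When BP_PawnSideView overlaps its box, it teleports the pawn to TeleportTo, with location relative to the actor.
; It then applies a render-target material to the book of BP_BetweenPagesMinigame and detaches the book if IsEnd is set.
; A camera-switch branch is left unconnected, marked for replacement.
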(event OnComponentBeginOverlap(Box)
  (params (OverlappedComponent :type Primitive%20Component%20Object%20Reference) (OtherActor :type Actor%20Object%20Reference) (OtherComp :type Primitive%20Component%20Object%20Reference) (OtherBodyIndex :type Integer) (bFromSweep :type Boolean) (SweepResult :type Hit%20Result%20Structure%20%28by%20ref%29))
  (bind _teleportto (Variables|Default|GetTeleportTo))
  ;[1 1 1] TeleportPawnToNextPage
  (bind _asbp_pawn_side_view (Utilities|Casting|CastToBP_PawnSideView OtherActor))
  (Transformation|SetActorLocationAndRotation _asbp_pawn_side_view (Math|Transform|TransformLocation (Transformation|GetActorTransform) (.location _teleportto)) (.rotation _teleportto))
  ;[1 1 1] Change PageMaterial
  (bind _returnvalue (Actor|GetActorOfClass "/Game/Mechanics/QuestObjects/BP_BetweenPagesMinigame.BP_BetweenPagesMinigame_C"))
  (Rendering|Material|SetMaterial (Variables|/Game/Mechanics/QuestObjects/BP_BetweenPagesMinigame.BP_BetweenPagesMinigame_C|GetBookMinigame _returnvalue) 0 (Variables|Default|GetRenderTargetMaterial))
  (if (Variables|Default|GetbIsEnd)
    (Default|DetachBook (Variables|Default|GetBookMinigame))))

(fn ConstructionScript)