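; BP_InBookMinigame is an interactable actor that launches the in-book minigame.
; On interact, it hands the player reference to its referenced minigame pawn, has the first player controller possess that pawn, then switches the view target to itself.
; BeginPlay, overlap and Tick are disabled stubs, so all behavior lives in the interact event.
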(event EventBeginPlay
  (|CallParentFunction) ; This node is disabled and will not be called.\nDrag off pins to build functionality.
)

(event Collision|EventActorBeginOverlap
  (params (OtherActor :type Actor%20Object%20Reference))
  (|CallParentFunction OtherActor) ; This node is disabled and will not be called.\nDrag off pins to build functionality.
)

(event EventTick
  (params (DeltaSeconds :type Float%20%28single-precision%29))
  (|CallParentFunction DeltaSeconds) ; This node is disabled and will not be called.\nDrag off pins to build functionality.
)

(event EventOnInteract
  (params (PlayerRef :type BP%20Third%20Person%20Character%20Object%20Reference))
  (bind _returnvalue (Game|GetPlayerController 0))
  (bind _pawnreference (Variables|Default|GetPawnReference))
  (Variables|/Game/Mechanics/MiniGames/InTheBook/BP_PawnSideView.BP_PawnSideView_C|SetPlayerRef _pawnreference PlayerRef)
  (Pawn|Possess _returnvalue _pawnreference)
  (Game|Player|SetViewTargetwithBlend _returnvalue self 0.0 "VTBlend_Linear" 0.0 false))

(fn ConstructionScript
  (|CallParentFunction))