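; BP_TargetForLuciusMiniGame is an interactable target in the Lucius minigame that triggers figure movement.
; On interact, it passes its TargetNumber to the minigame's MoveFigures and immediately destroys whatever ConnectedTargetsRef references.
; After a short delay, it hides and destroys itself.
; A SpawnTargets call on the minigame is left unwired and never runs.
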(event EventBeginPlay
  (|CallParentFunction) ; This node is disabled and will not be called.\nDrag off pins to build functionality.
)

(event Collision|EventActorBeginOverlap
  (params (OtherActor :type Actor%20Object%20Reference)))

(event EventTick
  (params (DeltaSeconds :type Float%20%28single-precision%29)))

(event EventOnInteract
  (params (PlayerRef :type BP%20Third%20Person%20Character%20Object%20Reference))
  (Default|MoveFigures (Variables|Default|GetMiniGameRef) (Variables|Default|GetTargetNumber))
  (Actor|DestroyActor (Variables|Default|GetConnectedTargetsRef))
  (Utilities|FlowControl|Delay 3.0)
  (Rendering|SetActorHiddenInGame true)
  (Actor|DestroyActor))

(fn ConstructionScript
  (|CallParentFunction))