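; Lucius mini-game actor where up to four two-option decisions move Hans and Lucius figures toward a shared meeting point.
; Interacting blends the view to the board, enables mouse input and spawns two linked targets with materials from DecisionMap.
; Clicks line-trace to interact with hit actors; MoveFigures uses the chosen target's step value to slide both figures along six stored positions via timeline.
; Reaching the meeting point returns the view to the player.
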(event Custom|SpawnTargets
  (bind _returnvalue (Game|GetPlayerController 0))
  (bind _location1 (Variables|Default|GetLocation1))
  (bind _location2 (Variables|Default|GetLocation2))
  (bind _returnvalue_2 (Transformation|GetWorldTransform _location2))
  (bind _returnvalue_3 (Transformation|GetWorldTransform _location1))
  ;[1 1 1] Spawn Targets
  (if (< (Variables|Default|GetDecisionCount) 4)
    (if (not (Variables|Default|GetReachedTheMeetPoint))
      (bind _returnvalue_4 (Game|SpawnActorfromClass "/Game/Mechanics/MiniGames/LuciusMiniGame/BP_TargetForLuciusMiniGame.BP_TargetForLuciusMiniGame_C" (Math|Transform|MakeTransform (.location _returnvalue_3) (.rotation _returnvalue_3) "1.000000,1.000000,1.000000") "AlwaysSpawn" "MultiplyWithRoot" 0 0))
      (bind _output_get (Variables|Default|SetTarget1Ref _returnvalue_4))
      (bind _returnvalue_5 (Game|SpawnActorfromClass "/Game/Mechanics/MiniGames/LuciusMiniGame/BP_TargetForLuciusMiniGame.BP_TargetForLuciusMiniGame_C" (Math|Transform|MakeTransform (.location _returnvalue_2) (.rotation _returnvalue_2) "1.000000,1.000000,1.000000") "AlwaysSpawn" "MultiplyWithRoot" 0 0))
      (bind _output_get_2 (Variables|Default|SetTarget2Ref _returnvalue_5))
      (Variables|/Game/Mechanics/MiniGames/LuciusMiniGame/BP_TargetForLuciusMiniGame.BP_TargetForLuciusMiniGame_C|SetConnectedTargetsRef _output_get_2 _output_get)
      (Variables|/Game/Mechanics/MiniGames/LuciusMiniGame/BP_TargetForLuciusMiniGame.BP_TargetForLuciusMiniGame_C|SetConnectedTargetsRef _output_get _output_get_2)
      (Variables|/Game/Mechanics/MiniGames/LuciusMiniGame/BP_TargetForLuciusMiniGame.BP_TargetForLuciusMiniGame_C|SetMiniGameRef _output_get self)
      (Variables|/Game/Mechanics/MiniGames/LuciusMiniGame/BP_TargetForLuciusMiniGame.BP_TargetForLuciusMiniGame_C|SetMiniGameRef _output_get_2 self)
      (Rendering|Material|SetMaterial (Variables|/Game/Mechanics/MiniGames/LuciusMiniGame/BP_TargetForLuciusMiniGame.BP_TargetForLuciusMiniGame_C|GetTarget (Variables|Default|GetTarget1Ref)) 0 (.target1material (.Value (Utilities|Map|Find (Variables|Default|GetDecisionMap) (Variables|Default|GetDecisionCount)))))
      (Rendering|Material|SetMaterial (Variables|/Game/Mechanics/MiniGames/LuciusMiniGame/BP_TargetForLuciusMiniGame.BP_TargetForLuciusMiniGame_C|GetTarget (Variables|Default|GetTarget2Ref)) 0 (.target2material (.Value (Utilities|Map|Find (Variables|Default|GetDecisionMap) (Variables|Default|GetDecisionCount)))))
      (Variables|/Game/Mechanics/MiniGames/LuciusMiniGame/BP_TargetForLuciusMiniGame.BP_TargetForLuciusMiniGame_C|SetTargetNumber (Variables|Default|GetTarget1Ref) 1)
      (Variables|/Game/Mechanics/MiniGames/LuciusMiniGame/BP_TargetForLuciusMiniGame.BP_TargetForLuciusMiniGame_C|SetTargetNumber (Variables|Default|GetTarget2Ref) 2)
      (else
        (Variables|/Script/Engine.PlayerController|SetbShowMouseCursor _returnvalue false :!label _label)
        ;[1 1 1] LookAtComponentUnderTheMouse
        (Game|Player|SetViewTargetwithBlend _returnvalue (Game|GetPlayerCharacter 0) 0.0 "VTBlend_Linear" 0.0 false)))
    (else
      (goto _label))))

(event Custom|MoveFigures
  (params (TargetNumber :type Integer))
  (bind _hans (Variables|Default|GetHans))
  (bind _lucius (Variables|Default|GetLucius))
  (bind _relativelocation (Variables|/Script/Engine.SceneComponent|GetRelativeLocation _lucius))
  (bind _relativelocation_2 (Variables|/Script/Engine.SceneComponent|GetRelativeLocation _hans))
  ;[0.1152 1 0.6715] Move Figures
  ;;[0.1152 1 0.6715] Move Hans Figure
  (bind _newtrack_0 (Timeline|Timeline PlayFromStart)
    (:Update
      (Transformation|SetRelativeLocation _hans (Math|Vector|MakeVector (.x _relativelocation_2) (Math|Float|Lerp (.y _relativelocation_2) (.y (.location (.Value (Utilities|Map|Find (Variables|Default|GetHansLocations) (Math|Integer|Clamp(Integer) (+ (Variables|Default|GetcurrentFigureLocation) (.Value (Utilities|Map|Find (.targetdata (.Value (Utilities|Map|Find (Variables|Default|GetDecisionMap) (Variables|Default|GetDecisionCount)))) TargetNumber))) 1 6))))) _newtrack_0) (.z _relativelocation_2)) false false)
      ;;[0.1152 1 0.6715] Move Lucius Figure
      (Transformation|SetRelativeLocation _lucius (Math|Vector|MakeVector (.x _relativelocation) (Math|Float|Lerp (.y _relativelocation) (.y (.location (.Value (Utilities|Map|Find (Variables|Default|GetLuciusLocations) (Math|Integer|Clamp(Integer) (+ (Variables|Default|GetcurrentFigureLocation) (.Value (Utilities|Map|Find (.targetdata (.Value (Utilities|Map|Find (Variables|Default|GetDecisionMap) (Variables|Default|GetDecisionCount)))) TargetNumber))) 1 6))))) _newtrack_0) (.z _relativelocation)) false false))
    (:Finished
      (CallFunction|CheckQuestStatus)
      (Variables|Default|SetcurrentFigureLocation (Math|Integer|Clamp(Integer) (+ (Variables|Default|GetcurrentFigureLocation) (.Value (Utilities|Map|Find (.targetdata (.Value (Utilities|Map|Find (Variables|Default|GetDecisionMap) (Variables|Default|GetDecisionCount)))) TargetNumber))) 1 6))
      (Math|Integer|IncrementInt (Variables|Default|GetDecisionCount)))))

(event Custom|CheckQuestStatus
  ;[1 1 1] Check quest completion
  (if (<= (.y (Variables|/Script/Engine.SceneComponent|GetRelativeLocation (Variables|Default|GetHans))) 0.0)
    (if (>= (.y (Variables|/Script/Engine.SceneComponent|GetRelativeLocation (Variables|Default|GetLucius))) 0.0)
      (Variables|Default|SetReachedTheMeetPoint true)
      (CallFunction|OnInteract))))

(event EventBeginPlay
  (|CallParentFunction)
  ;[0.02824 1 0.5689] Saving the Locations
  (|SetFigureLocationsInMap))

(event Collision|EventActorBeginOverlap
  (params (OtherActor :type Actor%20Object%20Reference))
  (|CallParentFunction OtherActor) ; This node is disabled and will not be called.\nDrag off pins to build functionality.
)

(event EventTick
  (params (DeltaSeconds :type Float%20%28single-precision%29))
  (|CallParentFunction DeltaSeconds) ; This node is disabled and will not be called.\nDrag off pins to build functionality.
)

(event EventOnActivation
  (params (PlayerRef :type BP%20Third%20Person%20Character%20Object%20Reference)))

(event EventOnInteract
  (params (PlayerRef :type BP%20Third%20Person%20Character%20Object%20Reference))
  (bind _returnvalue (Game|GetPlayerController 0))
  (bind _returnvalue_2 (Game|GetPlayerController 0))
  ;[1 1 1] Switch the Pawns and the View
  (if (not (Variables|Default|GetReachedTheMeetPoint))
    (Variables|/Script/Engine.PlayerController|SetbShowMouseCursor _returnvalue_2 true)
    (Game|Player|SetViewTargetwithBlend _returnvalue_2 self 1.0 "VTBlend_Linear" 0.0 false)
    (Input|EnableInput (Game|GetPlayerController 0))
    (CallFunction|SpawnTargets)
    (else
      (Variables|/Script/Engine.PlayerController|SetbShowMouseCursor _returnvalue false)
      (Game|Player|SetViewTargetwithBlend _returnvalue (Game|GetPlayerCharacter 0) 1.0 "VTBlend_Linear" 0.0 false))))

(event Input|MouseEvents|LeftMouseButton
  (params (Key :type Key%20Structure :default "None"))
  (bind _returnvalue (Game|GetPlayerController 0))
  (bind (_worldlocation _worlddirection) (Game|Player|ConvertMouseLocationToWorldSpace _returnvalue))
  ;[1 1 1] LookAtComponentUnderTheMouse
  (:Pressed
    (bind _outhit (Collision|LineTraceByChannel _worldlocation (+ _worldlocation (* _worlddirection (Math|Conversions|ToVector(Float) 5e+02))) "TraceTypeQuery1" false 0 "ForDuration" false))
    (Class|BPIInteractable|OnInteract(Message) (.HitActor (Collision|BreakHitResult _outhit)))))

(fn ConstructionScript
  (|CallParentFunction))