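; Marble maze minigame actor that hands control to its pawn and switches the camera to itself when the player interacts.
; The player reference is passed to the pawn before possession.
; A looping-style rolling cue starts on BeginPlay, and each hit scales its volume by the Cube's physics speed.
; Hits with upward Cube velocity also play a marble impact sound, throttled by a DoOnce that resets after a short delay.
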(event EventBeginPlay
  (|CallParentFunction)
  (Audio|Components|Audio|Play (Variables|Default|GetRolling_Cue) 0.0))

(event Collision|EventActorBeginOverlap
  (params (OtherActor :type Actor%20Object%20Reference)))

(event EventTick
  (params (DeltaSeconds :type Float%20%28single-precision%29)))

(event EventOnInteract
  (params (PlayerRef :type BP%20Third%20Person%20Character%20Object%20Reference))
  (bind _returnvalue (Game|GetPlayerController 0))
  (bind _pawnref (Variables|Default|GetPawnRef))
  (Variables|/Game/Mechanics/MiniGames/MarbleMaze/BP_MarbleMazePawn.BP_MarbleMazePawn_C|SetPlayerRef _pawnref PlayerRef)
  (Pawn|Possess _returnvalue _pawnref)
  (Game|Player|SetViewTargetwithBlend _returnvalue self 0.0 "VTBlend_Linear" 0.0 false))

(event Collision|EventHit
  (params (MyComp :type Primitive%20Component%20Object%20Reference) (Other :type Actor%20Object%20Reference) (OtherComp :type Primitive%20Component%20Object%20Reference) (bSelfMoved :type Boolean) (HitLocation :type Vector :default "0, 0, 0") (HitNormal :type Vector :default "0, 0, 0") (NormalImpulse :type Vector :default "0, 0, 0") (Hit :type Hit%20Result%20Structure%20%28by%20ref%29))
  (bind _returnvalue (Physics|GetPhysicsLinearVelocity (Variables|Default|GetCube) "None"))
  (Utilities|FlowControl|Sequence
    (:then_0
      (Math|Float|CompareFloat (.Z (Math|Vector|BreakVector _returnvalue)) 0.0
        (:>
          (Utilities|FlowControl|DoOnce false :!label _label
            (:Completed
              (Audio|PlaySoundatLocation "/Game/SoundSystem/Sounds/SFX/Marble/MS_MarbleHit.MS_MarbleHit" (Transformation|GetWorldLocation (Variables|Default|GetCube)) "0, 0, 0" 1.0 1.0 0.0 0 0 0 0)
              (Utilities|FlowControl|Delay 1.0)
              (goto _label Reset))))))
    (:then_1
      (Audio|Components|Audio|SetVolumeMultiplier (Variables|Default|GetRolling_Cue) (/ (Math|Vector|VectorLength _returnvalue) 3e+02) :!class /Script/Engine.AudioComponent))))

(fn ConstructionScript
  (|CallParentFunction))