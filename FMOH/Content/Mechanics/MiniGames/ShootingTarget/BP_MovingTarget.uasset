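; Shooting-gallery target for the gun minigame that slides back and forth and falls when hit by a BP_Projectile.
; MiniGameStarted starts paired timelines that lerp the Cube between its start location and a RangeOfMovement offset in a continuous loop, timed by SpeedOfMovement.
; A projectile overlapping the Box plays a tip-over rotation, then adds a point to the player's BP_ContolableGunPawn and destroys the target.
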(event OnComponentBeginOverlap(Box)
  (params (OverlappedComponent :type Primitive%20Component%20Object%20Reference) (OtherActor :type Actor%20Object%20Reference) (OtherComp :type Primitive%20Component%20Object%20Reference) (OtherBodyIndex :type Integer) (bFromSweep :type Boolean) (SweepResult :type Hit%20Result%20Structure%20%28by%20ref%29))
  (bind _playerref (Variables|Default|GetPlayerRef))
  (bind _originalrotation (Variables|Default|GetOriginalRotation))
  ;[1 1 1] Destroying the Target on Overlap and adding Points to the Count
  (Utilities|Casting|CastToBP_Projectile OtherActor)
  (bind _newtrack_0 (Timeline|Timeline PlayFromStart)
    (:Update
      (Transformation|SetWorldRotation (Variables|Default|GetCube) (Math|Rotator|Lerp(Rotator) _originalrotation (Math|Rotator|CombineRotators _originalrotation (Variables|Default|GetDirectionOfFall)) _newtrack_0) false false))
    (:Finished
      (Variables|/Game/Mechanics/MiniGames/ShootingTarget/BP_ContolableGunPawn.BP_ContolableGunPawn_C|SetPointsScoure _playerref (+ (Variables|/Game/Mechanics/MiniGames/ShootingTarget/BP_ContolableGunPawn.BP_ContolableGunPawn_C|GetPointsScoure _playerref) 1))
      (Actor|DestroyActor))))

(event EventBeginPlay
  (bind _returnvalue (Transformation|GetActorLocation))
  (Variables|Default|SetStartLocation _returnvalue)
  (Variables|Default|SetEndLocation (+ _returnvalue (Variables|Default|GetRangeOfMovement)))
  (Variables|Default|SetOriginalRotation (Transformation|GetWorldRotation (Variables|Default|GetCube)))
  (bind _asbp_contolable_gun_pawn (Utilities|Casting|CastToBP_ContolableGunPawn (Game|GetPlayerCharacter 0)))
  (Variables|Default|SetPlayerRef _asbp_contolable_gun_pawn))

(event EventMiniGameStarted
  (bind _speedofmovement (Variables|Default|GetSpeedOfMovement))
  (bind _returnvalue (/ 1.0 _speedofmovement))
  ;[1 1 1] Move the Target
  (Components|Timeline|SetPlayRate (Variables|Default|GetMoveTarget) _returnvalue)
  (bind _newtrack_0 (Timeline|MoveTarget PlayFromStart)
    (:Update
      (Transformation|SetWorldLocation (Variables|Default|GetCube) (Math|Vector|Lerp(Vector) (Variables|Default|GetStartLocation) (Variables|Default|GetEndLocation) _newtrack_0) false false))
    (:Finished
      (Components|Timeline|SetPlayRate (Variables|Default|GetTimeline_0) _returnvalue)
      (bind _newtrack_0_2 (Timeline|Timeline_0 ReverseFromEnd)
        (:Update
          (Transformation|SetWorldLocation (Variables|Default|GetCube) (Math|Vector|Lerp(Vector) (Variables|Default|GetStartLocation) (Variables|Default|GetEndLocation) _newtrack_0_2) false false))
        (:Finished
          (Timeline|MoveTarget PlayFromStart))))))

(fn ConstructionScript)