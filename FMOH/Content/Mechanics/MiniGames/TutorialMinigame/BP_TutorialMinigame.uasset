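; BP_TutorialMinigame is the tutorial minigame actor, a click-to-interact view that ends once every item in ItemToWaitFor is activated.
; OnInteract locks the player, plays a frame-taking montage with a camera animation, then blends the view to itself and shows the cursor.
; Mouse clicks line-trace and forward interaction to hit actors while Tick polls completion.
; OnActivation silences the radio, restores player control and plays the hanging montage with its camera animation.
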(event EventTick
  (params (DeltaSeconds :type Float%20%28single-precision%29))
  ;[0 1 0.6563] CheckingForTutorialCompletion
  (Variables|Default|SetbQuestCompleted false)
  (for (_array_element _array_index) (Variables|Default|GetItemToWaitFor)
    (if (== _array_index 0)
      (Variables|Default|SetbQuestCompleted (Variables|/Game/Mechanics/BaseBlueprints/BP_BaseActivatableAndInteractableObject.BP_BaseActivatableAndInteractableObject_C|GetbIsActivated _array_element))
      (elif (Variables|Default|GetbQuestCompleted)
        (Variables|Default|SetbQuestCompleted (Variables|/Game/Mechanics/BaseBlueprints/BP_BaseActivatableAndInteractableObject.BP_BaseActivatableAndInteractableObject_C|GetbIsActivated _array_element)))))
  (if (Variables|Default|GetbQuestCompleted)
    (CallFunction|OnActivation (Variables|Default|GetPlayer%20Ref))
    (Actor|Tick|SetActorTickEnabled false)))

(event EventOnActivation
  (params (PlayerRef :type BP%20Third%20Person%20Character%20Object%20Reference))
  (bind _returnvalue (Game|GetPlayerController 0))
  (bind _returnvalue_2 (Game|GetPlayerCharacter 0))
  (bind _returnvalue_3 (Transformation|GetActorTransform _returnvalue_2))
  ;[1 1 1] Switch the Pawns and the View
  (Default|TurnOff (Variables|Default|GetRadioRef))
  (Variables|Default|SetPlayer%20Ref PlayerRef)
  (Variables|/Script/Engine.PlayerController|SetbShowMouseCursor _returnvalue false)
  (Input|SetInputModeGameOnly _returnvalue false)
  (Game|Player|SetViewTargetwithBlend _returnvalue (Game|GetPlayerCharacter 0) 1.0 "VTBlend_Linear" 0.0 false)
  (Input|DisableInput (Game|GetPlayerController 0))
  (Variables|/Game/ThirdPerson/Blueprints/BP_ThirdPersonCharacter.BP_ThirdPersonCharacter_C|SetIsMovementLocked (Variables|Default|GetPlayer%20Ref) false)
  ;;[1 0.1752 0] GETTING UP FROM TABLE ANIMATION HERE
  (Variables|/Game/ThirdPerson/Blueprints/BP_ThirdPersonCharacter.BP_ThirdPersonCharacter_C|SetbIsCameraLocked (Variables|Default|GetPlayer%20Ref) false)
  (Animation|Montage|PlayMontage (Variables|/Script/Engine.Character|GetMesh _returnvalue_2) "/Game/Characters/Mannequins/Animations/Arys_folder/other_animations/hanging_cut/AM_HangingFirstPart.AM_HangingFirstPart"
    (:then
      (bind _returnvalue_4 (Game|SpawnActorfromClass "/Game/Characters/Mannequins/Animations/Arys_folder/other_animations/BP_HangingCameraAnimation.BP_HangingCameraAnimation_C" (Math|Transform|MakeTransform (.location _returnvalue_3) (.rotation _returnvalue_3) "1.000000,1.000000,1.000000") "Undefined" "MultiplyWithRoot" 0 0))
      (Default|PlayCameraAnimation _returnvalue_4)
      (Utilities|FlowControl|Delay 6.0)
      (Default|EndCameraAnimation _returnvalue_4))))

(event EventOnInteract
  (params (PlayerRef :type BP%20Third%20Person%20Character%20Object%20Reference))
  (bind _returnvalue (Game|GetPlayerController 0))
  (bind _returnvalue_2 (Game|GetPlayerCharacter 0))
  (bind _returnvalue_3 (Transformation|GetActorTransform _returnvalue_2))
  ;[1 1 1] Switch the Pawns and the View
  (bind _output_get (Variables|Default|SetPlayer%20Ref PlayerRef))
  (Variables|/Game/ThirdPerson/Blueprints/BP_ThirdPersonCharacter.BP_ThirdPersonCharacter_C|SetIsMovementLocked _output_get true)
  (Variables|/Game/ThirdPerson/Blueprints/BP_ThirdPersonCharacter.BP_ThirdPersonCharacter_C|SetbIsCameraLocked _output_get true)
  ;;[1 0.3298 0.03993] Animation of frame taking
  (Animation|Montage|PlayMontage (Variables|/Script/Engine.Character|GetMesh _returnvalue_2) "/Game/Characters/Mannequins/Animations/Arys_folder/other_animations/AM_frame_full_animation_Montage.AM_frame_full_animation_Montage"
    (:then
      (bind _returnvalue_4 (Game|SpawnActorfromClass "/Game/Characters/Mannequins/Animations/Arys_folder/other_animations/BP_HangingCameraAnimationFrame.BP_HangingCameraAnimationFrame_C" (Math|Transform|MakeTransform (.location _returnvalue_3) (.rotation _returnvalue_3) "1.000000,1.000000,1.000000") "Undefined" "MultiplyWithRoot" 0 0))
      (Default|PlayCameraAnimation _returnvalue_4)
      (Variables|/Game/Mechanics/BaseBlueprints/BP_RoomSwitcher.BP_RoomSwitcher_C|SetCharacterRef (Variables|Default|GetRoomSwitcherRef) _output_get)
      (if true
        (Variables|/Script/Engine.PlayerController|SetbShowMouseCursor _returnvalue true)
        (Game|Player|SetViewTargetwithBlend _returnvalue self 1.0 "VTBlend_Linear" 0.0 false)
        (Input|EnableInput (Game|GetPlayerController 0))))))

(event Input|MouseEvents|LeftMouseButton
  (params (Key :type Key%20Structure :default "None"))
  (bind _returnvalue (Game|GetPlayerController 0))
  (bind (_worldlocation _worlddirection) (Game|Player|ConvertMouseLocationToWorldSpace _returnvalue))
  ;[1 1 1] Comment
  (:Pressed
    (bind _outhit (Collision|LineTraceByChannel _worldlocation (+ _worldlocation (* _worlddirection (Math|Conversions|ToVector(Float) 5e+02))) "TraceTypeQuery1" false 0 "None" false))
    (Class|BPIInteractable|OnInteract(Message) (.HitActor (Collision|BreakHitResult _outhit)) (Variables|Default|GetPlayer%20Ref))))

(fn ConstructionScript
  (|CallParentFunction))