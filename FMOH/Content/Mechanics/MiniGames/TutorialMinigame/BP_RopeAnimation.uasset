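; Interactable rope for the tutorial minigame that runs the prologue's scripted hanging sequence.
; On interact it locks the player, glides them to a start point via a distance-scaled timeline, then plays rope, character and spawned-camera animations.
; After a timed teleport it waits for any key to trigger the death camera sequence.
; A blink then covers hiding the listed objects before the player is locked to BP_PrologSpline and set walking.
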(event Custom|CallRopeAnimation
  ;[0 1 0.6231] Calling the Rope Animation
  (Components|Animation|PlayAnimation (Variables|Default|GetSkeletalMesh) "/Game/Characters/Mannequins/Animations/Arys_folder/other_animations/hanging_cut/rope/rope_death_3_skeleton_centered.rope_death_3_skeleton_centered" false))

(event Custom|MoveCharacterIntoPosition
  (bind _returnvalue (Game|GetPlayerController 0))
  (bind _player_ref (Variables|Default|GetPlayer%20Ref))
  (bind _animationstartlocation (Variables|Default|GetAnimationStartLocation))
  (bind _returnvalue_2 (Transformation|GetDistanceTo _player_ref))
  ;[0.5454 1 0.7155] Change the speed of the timline depeding o how far the player is from the door
  (if (< _returnvalue_2 1e+02)
    (Variables|Default|SetDynamicPlayrate 1.0)
    (elif (> _returnvalue_2 2.5e+02)
      (Variables|Default|SetDynamicPlayrate 0.3)
      (else
        (Variables|Default|SetDynamicPlayrate 0.5))))
  ;[0.5454 1 0.7155] Move character to the door
  (Game|Feedback|ClientStartCameraShake _returnvalue "/Game/Mechanics/CameraBPs/BP_Walk.BP_Walk_C" 1.0 "CameraLocal" "0, 0, 0")
  (Components|Timeline|SetPlayRate (Variables|Default|GetTimeline) (Variables|Default|GetDynamicPlayrate))
  (bind (_direction _newtrack_0 _newtrack_1) (Timeline|Timeline PlayFromStart)
    (:Update
      (Pawn|SetControlRotation _returnvalue (Math|Rotator|Lerp(Rotator) (Pawn|GetControlRotation _returnvalue :!class /Script/Engine.Controller) (* (Transformation|GetWorldRotation _animationstartlocation) -1.0) _newtrack_1 true))
      (Transformation|SetActorLocation (Variables|Default|GetPlayer%20Ref) (Math|Vector|MakeVector (.x (Math|Vector|Lerp(Vector) (Transformation|GetActorLocation (Game|GetPlayerCharacter 0)) (Transformation|GetWorldLocation _animationstartlocation) _newtrack_0)) (.y (Math|Vector|Lerp(Vector) (Transformation|GetActorLocation (Game|GetPlayerCharacter 0)) (Transformation|GetWorldLocation _animationstartlocation) _newtrack_0)) (.z (Math|Vector|Lerp(Vector) (Transformation|GetActorLocation (Game|GetPlayerCharacter 0)) (Transformation|GetWorldLocation _animationstartlocation) _newtrack_0))) false false))
    (:Finished
      ;[1 0.4133 0] Calling the Animation when player is in position
      (CallFunction|PlayHangingStartAnimation))))

(event Custom|PlayHangingStartAnimation
  (bind _returnvalue (Game|GetPlayerCharacter 0))
  (bind _returnvalue_2 (Game|GetPlayerController 0))
  (bind _returnvalue_3 (Game|GetPlayerController 0))
  (bind _returnvalue_4 (Transformation|GetActorTransform _returnvalue))
  ;[1 0.3592 0] GOING UP THE STEPS TO GE TTO THE ROPE AND PUT IT AROUND MY NECK ANIMATION HERE
  (bind _returnvalue_5 (Game|SpawnActorfromClass "/Game/Characters/Mannequins/Animations/Arys_folder/other_animations/BP_HangingCameraAnimationSecond.BP_HangingCameraAnimationSecond_C" (Math|Transform|MakeTransform (.location _returnvalue_4) (Math|Rotator|MakeRotator (.roll (.rotation _returnvalue_4)) (.pitch (.rotation _returnvalue_4)) (+ (.yaw (.rotation _returnvalue_4)) 1.8e+02)) "1.000000,1.000000,1.000000") "Undefined" "MultiplyWithRoot" 0 0))
  (Default|PlayCameraAnimation _returnvalue_5)
  ;;[1 0.02257 0.02257] Turn Mesh to compensate animation rotation
  (Pawn|SetControlRotation _returnvalue_3 (* (Transformation|GetActorRotation _returnvalue_3) -1.0))
  (CallFunction|CallRopeAnimation)
  (Animation|Montage|PlayMontage (Variables|/Script/Engine.Character|GetMesh _returnvalue) "/Game/Characters/Mannequins/Animations/Arys_folder/other_animations/hanging_cut/AM_hanging_11_02_secondpart_Montage.AM_hanging_11_02_secondpart_Montage"
    (:then
      (Utilities|FlowControl|Delay 19.4)
      ;[1 0 0] Teleport the Player to Location before the leap and compensate rotation again
      (Transformation|SetActorLocation (Variables|Default|GetPlayer%20Ref) (Transformation|GetWorldLocation (Variables|Default|GetAnimationEndLocation1)) false true)
      (Pawn|SetControlRotation _returnvalue_2 (* (Pawn|GetControlRotation _returnvalue_2 :!class /Script/Engine.Controller) -1.0))
      (Pawn|Components|CharacterMovement|SetMovementMode (Variables|/Script/Engine.Character|GetCharacterMovement (Variables|Default|GetPlayer%20Ref)) "MOVE_Flying" 0)
      ;[0 1 0.6222] When the Animation is finished this will activate the players ability to activate the rest of the animation
      (Variables|Default|SetbIsWaitingForInput true)
      (Development|PrintString "Waiting for input")
      (Input|EnableInput (Game|GetPlayerController 0)))))

(event Custom|PlayDyingAnimation
  (bind _returnvalue (Game|GetPlayerCharacter 0))
  (bind _returnvalue_2 (Transformation|GetActorTransform _returnvalue))
  ;[1 0.3592 0] Taking the leap and dying Animation HERE
  (bind _returnvalue_3 (Game|SpawnActorfromClass "/Game/Characters/Mannequins/Animations/Arys_folder/other_animations/BP_HangingCameraAnimationLastPart.BP_HangingCameraAnimationLastPart_C" (Math|Transform|MakeTransform (.location _returnvalue_2) (Math|Rotator|MakeRotator (.roll (.rotation _returnvalue_2)) (.pitch (.rotation _returnvalue_2)) (+ (.yaw (.rotation _returnvalue_2)) 1.8e+02)) "1.000000,1.000000,1.000000") "Undefined" "MultiplyWithRoot" 0 0))
  (Default|PlayCameraAnimation _returnvalue_3)
  (Utilities|FlowControl|Delay 16.2)
  ;[0.03154 1 0] make wall dissapear
  (Default|StartBlink (Variables|Default|GetPlayer%20Ref) 1.0 1.0)
  (Utilities|FlowControl|Delay 1.0)
  (for _array_element (Variables|Default|GetObjects%20to%20destroy)
    (Rendering|SetActorHiddenInGame _array_element true)
    (Utilities|FlowControl|Delay 3.0)
    ;[0.01239 1 0.5672] Locking the player on the Spline when regaining control and moving towards the portal
    (Default|LockPlayer (Variables|Default|GetPrologSplineRef) (Variables|Default|GetPlayer%20Ref))
    (Pawn|Components|CharacterMovement|SetMovementMode (Variables|/Script/Engine.Character|GetCharacterMovement (Variables|Default|GetPlayer%20Ref)) "MOVE_Walking" 0)))

(event EventOnInteract
  (params (PlayerRef :type BP%20Third%20Person%20Character%20Object%20Reference))
  ;[0 1 0.6519] OnInteract
  (bind _output_get (Variables|Default|SetPlayer%20Ref PlayerRef))
  (CallFunction|MoveCharacterIntoPosition)
  (Variables|/Game/ThirdPerson/Blueprints/BP_ThirdPersonCharacter.BP_ThirdPersonCharacter_C|SetIsMovementLocked _output_get true)
  (Variables|/Game/ThirdPerson/Blueprints/BP_ThirdPersonCharacter.BP_ThirdPersonCharacter_C|SetbIsCameraLocked _output_get true))

(event EventBeginPlay
  ;[0 1 0.6065] BeginPlay
  (bind _returnvalue (Actor|GetActorOfClass "/Game/Mechanics/MiniGames/Prologue/BP_PrologSpline.BP_PrologSpline_C"))
  (Variables|Default|SetPrologSplineRef _returnvalue))

(event Input|KeyboardEvents|AnyKey
  (params (Key :type Key%20Structure :default "None"))
  ;[0 1 0.6726] Only reacts when the boolean is activated and will deactivate itself again after calling the animation event once
  (:Pressed
    (if (Variables|Default|GetbIsWaitingForInput)
      (Development|PrintString "Input Made")
      (CallFunction|PlayDyingAnimation)
      (Variables|Default|SetbIsWaitingForInput false)
      (Input|DisableInput (Game|GetPlayerController 0)))))

(fn ConstructionScript)