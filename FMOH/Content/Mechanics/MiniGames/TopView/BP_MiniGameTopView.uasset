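; Top-view minigame actor that, on interaction, hands player control to a referenced pawn and blends the camera to itself.
; It passes the player reference to that pawn, moves it to the Start point and tells a referenced spline to begin moving its object.
; It then spawns five quarter-scale BP_Collectable actors at fixed spawn components.
; OnActivation is empty and the collectable cleanup logic is unconnected.
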(event Custom|SetToStart
  ;[1 1 1] ResetingPawnTo Start
  (Transformation|SetWorldLocation (Variables|/Script/Engine.Actor|GetRootComponent (Variables|Default|GetPawnReference)) (.location (Transformation|GetWorldTransform (Variables|Default|GetStart))) false false)
  (bind _returnvalue (Actor|GetActorOfClass "/Game/Mechanics/MiniGames/TopView/BP_Collectable.BP_Collectable_C"))
  (Variables|Default|SetCollectableRef _returnvalue))

(event Custom|SetCollectables
  (bind _spawnlocation5 (Variables|Default|GetSpawnLocation5))
  (bind _spawnlocation1 (Variables|Default|GetSpawnLocation1))
  (bind _spawnlocation2 (Variables|Default|GetSpawnLocation2))
  (bind _spawnlocation3 (Variables|Default|GetSpawnLocation3))
  (bind _spawnlocation4 (Variables|Default|GetSpawnLocation4))
  (bind _returnvalue (Transformation|GetWorldTransform _spawnlocation2))
  (bind _returnvalue_2 (Transformation|GetWorldTransform _spawnlocation3))
  (bind _returnvalue_3 (Transformation|GetWorldTransform _spawnlocation5))
  (bind _returnvalue_4 (Transformation|GetWorldTransform _spawnlocation4))
  (bind _returnvalue_5 (Transformation|GetWorldTransform _spawnlocation1))
  ;[1 1 1] CollectableSpawn
  (Game|SpawnActorfromClass "/Game/Mechanics/MiniGames/TopView/BP_Collectable.BP_Collectable_C" (Math|Transform|MakeTransform (.location _returnvalue_5) (.rotation _returnvalue_5) "0.250000,0.250000,0.250000") "Undefined" "MultiplyWithRoot" 0 0)
  (Game|SpawnActorfromClass "/Game/Mechanics/MiniGames/TopView/BP_Collectable.BP_Collectable_C" (Math|Transform|MakeTransform (.location _returnvalue) (.rotation _returnvalue) "0.250000,0.250000,0.250000") "Undefined" "MultiplyWithRoot" 0 0)
  (Game|SpawnActorfromClass "/Game/Mechanics/MiniGames/TopView/BP_Collectable.BP_Collectable_C" (Math|Transform|MakeTransform (.location _returnvalue_2) (.rotation _returnvalue_2) "0.250000,0.250000,0.250000") "Undefined" "MultiplyWithRoot" 0 0)
  (Game|SpawnActorfromClass "/Game/Mechanics/MiniGames/TopView/BP_Collectable.BP_Collectable_C" (Math|Transform|MakeTransform (.location _returnvalue_4) (.rotation _returnvalue_4) "0.250000,0.250000,0.250000") "Undefined" "MultiplyWithRoot" 0 0)
  (Game|SpawnActorfromClass "/Game/Mechanics/MiniGames/TopView/BP_Collectable.BP_Collectable_C" (Math|Transform|MakeTransform (.location _returnvalue_3) (.rotation _returnvalue_3) "0.250000,0.250000,0.250000") "Undefined" "MultiplyWithRoot" 0 0))

(event EventBeginPlay
  (|CallParentFunction))

(event Collision|EventActorBeginOverlap
  (params (OtherActor :type Actor%20Object%20Reference))
  (|CallParentFunction OtherActor) ; This node is disabled and will not be called.\nDrag off pins to build functionality.
)

(event EventOnActivation
  (params (PlayerRef :type BP%20Third%20Person%20Character%20Object%20Reference)))

(event EventOnInteract
  (params (PlayerRef :type BP%20Third%20Person%20Character%20Object%20Reference))
  (bind _returnvalue (Game|GetPlayerController 0))
  (bind _pawnreference (Variables|Default|GetPawnReference))
  ;[1 1 1] Switch the Pawns and the View
  (Variables|/Game/Mechanics/MiniGames/TopView/BP_ControlablePawnTop.BP_ControlablePawnTop_C|SetPlayerRef _pawnreference PlayerRef)
  (Pawn|Possess _returnvalue _pawnreference)
  (Game|Player|SetViewTargetwithBlend _returnvalue self 0.0 "VTBlend_Linear" 0.0 false)
  (CallFunction|SettoStart)
  (Class|BPISplineTrain|MoveObjAlongSpline(Message) (Variables|Default|GetSplineRef))
  (CallFunction|SetCollectables))

(fn ConstructionScript
  (|CallParentFunction))