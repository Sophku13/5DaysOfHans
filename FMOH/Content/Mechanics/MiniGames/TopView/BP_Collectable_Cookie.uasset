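; BP_Collectable_Cookie is a pickup for the top-view minigame that the player's pawn collects by overlap.
; It finds BP_MiniGameTopView on BeginPlay and destroys itself when a BP_ControlablePawnTop enters its collision.
; Each pickup increments and prints the minigame's shared Count until it reaches four.
; The next pickup instead flags food as collected on the pawn and calls its MinigameIsFinished.
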(event OnComponentBeginOverlap(Collision)
  (params (OverlappedComponent :type Primitive%20Component%20Object%20Reference) (OtherActor :type Actor%20Object%20Reference) (OtherComp :type Primitive%20Component%20Object%20Reference) (OtherBodyIndex :type Integer) (bFromSweep :type Boolean) (SweepResult :type Hit%20Result%20Structure%20%28by%20ref%29))
  (bind _minigameref (Variables|Default|GetMiniGameRef))
  (bind _asbp_controlable_pawn_top (Utilities|Casting|CastToBP_ControlablePawnTop OtherActor))
  (Actor|DestroyActor)
  (if (< (Variables|/Game/Mechanics/MiniGames/TopView/BP_MiniGameTopView.BP_MiniGameTopView_C|GetCount _minigameref) 4)
    (bind _result (Math|Integer|IncrementInt (Variables|/Game/Mechanics/MiniGames/TopView/BP_MiniGameTopView.BP_MiniGameTopView_C|GetCount _minigameref))
      (:%20%20
        (bind _output_get (Variables|/Game/Mechanics/MiniGames/TopView/BP_MiniGameTopView.BP_MiniGameTopView_C|SetCount _minigameref _result))
        (Development|PrintString (Utilities|String|ToString(Integer) _output_get))))
    (else
      (Variables|/Game/Mechanics/MiniGames/TopView/BP_ControlablePawnTop.BP_ControlablePawnTop_C|SetbIsFoodCollected _asbp_controlable_pawn_top true)
      (Default|MinigameIsFinished _asbp_controlable_pawn_top))))

(event EventBeginPlay
  (bind _returnvalue (Actor|GetActorOfClass "/Game/Mechanics/MiniGames/TopView/BP_MiniGameTopView.BP_MiniGameTopView_C"))
  (Variables|Default|SetMiniGameRef _returnvalue))

(fn ConstructionScript)