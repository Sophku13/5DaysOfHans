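; Spline actor for the top-view minigame that moves an array of actors, likely inspection lights, along its path in a continuous loop.
; Construction script spaces them by a fixed offset; BeginPlay or MoveObjAlongSpline sets timeline rates from TimeOfCompleting and starts playback.
; Forward or reverse timelines drive wrapped spline distances and restart on finish.
; StopMovementAlongSpline hides the actors but stops only the forward timeline.
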(event Custom|PlayTimeline
  (bind _spline (Variables|Default|GetSpline))
  (bind _spline_2 (Variables|Default|GetSpline))
  (bind _spline_3 (Variables|Default|GetSpline))
  (bind _spline_4 (Variables|Default|GetSpline))
  (bind _returnvalue (Spline|GetSplineLength _spline_2))
  (bind _returnvalue_2 (Spline|GetSplineLength _spline))
  ;[1 1 1] Using On Interact to start movement
  ;[1 1 1] Moving Obj Along Spline
  (if (Variables|Default|GetReverseMovement)
    ;[1 1 1] ReversedMovement
    (bind _newtrack_0 (Timeline|Timeline PlayFromStart)
      (:Update
        (for (_array_element _array_index) (Variables|Default|GetObjectForSpLine)
          (Rendering|SetActorHiddenInGame _array_element false)
          (bind _output_get (Variables|Default|SetDistanceAlongSpline (+ (Math|Float|Lerp (Spline|GetSplineLength (Variables|Default|GetSpline)) 0.0 _newtrack_0) (* _array_index (Variables|Default|GetOffsetBetweenActors)))))
          (if (> _output_get _returnvalue)
            (Variables|Default|SetDistanceAlongSpline (- (Variables|Default|GetDistanceAlongSpline) _returnvalue)))
          (Transformation|SetActorLocationAndRotation _array_element (Spline|GetLocationatDistanceAlongSpline _spline_4 (Variables|Default|GetDistanceAlongSpline) "World") (Spline|GetRotationatDistanceAlongSpline _spline_4 (Variables|Default|GetDistanceAlongSpline) "World"))))
      (:Finished
        (CallFunction|PlayTimeline)))
    (else
      (bind _newtrack_0_2 (Timeline|MoveTrain_T PlayFromStart)
        (:Update
          (for (_array_element_2 _array_index_2) (Variables|Default|GetObjectForSpLine)
            (Rendering|SetActorHiddenInGame _array_element_2 false)
            (bind _output_get_2 (Variables|Default|SetDistanceAlongSpline (+ (Math|Float|Lerp 0.0 (Spline|GetSplineLength (Variables|Default|GetSpline)) _newtrack_0_2) (* _array_index_2 (Variables|Default|GetOffsetBetweenActors)))))
            (if (> _output_get_2 _returnvalue_2)
              (Variables|Default|SetDistanceAlongSpline (- (Variables|Default|GetDistanceAlongSpline) _returnvalue_2)))
            (Transformation|SetActorLocationAndRotation _array_element_2 (Spline|GetLocationatDistanceAlongSpline _spline_3 (Variables|Default|GetDistanceAlongSpline) "World") (Spline|GetRotationatDistanceAlongSpline _spline_3 (Variables|Default|GetDistanceAlongSpline) "World"))))
        (:Finished
          (CallFunction|PlayTimeline))))))

(event EventBeginPlay
  (|CallParentFunction)
  ;[1 1 1] Using On Interact to start movement
  (Components|Timeline|SetPlayRate (Variables|Default|GetMoveTrain_T) (/ 1.0 (Variables|Default|GetTimeOfCompleting)))
  (CallFunction|PlayTimeline))

(event Collision|EventActorBeginOverlap
  (params (OtherActor :type Actor%20Object%20Reference)))

(event EventStopMovementAlongSpline
  (bind _spline (Variables|Default|GetSpline))
  (bind _spline_2 (Variables|Default|GetSpline))
  (bind _returnvalue (Spline|GetSplineLength _spline))
  ;[1 1 1] Stop movement
  (for _array_element (Variables|Default|GetObjectForSpLine)
    (Rendering|SetActorHiddenInGame _array_element true)
    ;[1 1 1] Moving Obj Along Spline
    (bind _newtrack_0 (Timeline|MoveTrain_T Stop)
      (:Update
        (for (_array_element_2 _array_index) (Variables|Default|GetObjectForSpLine)
          (Rendering|SetActorHiddenInGame _array_element_2 false)
          (bind _output_get (Variables|Default|SetDistanceAlongSpline (+ (Math|Float|Lerp 0.0 (Spline|GetSplineLength (Variables|Default|GetSpline)) _newtrack_0) (* _array_index (Variables|Default|GetOffsetBetweenActors)))))
          (if (> _output_get _returnvalue)
            (Variables|Default|SetDistanceAlongSpline (- (Variables|Default|GetDistanceAlongSpline) _returnvalue)))
          (Transformation|SetActorLocationAndRotation _array_element_2 (Spline|GetLocationatDistanceAlongSpline _spline_2 (Variables|Default|GetDistanceAlongSpline) "World") (Spline|GetRotationatDistanceAlongSpline _spline_2 (Variables|Default|GetDistanceAlongSpline) "World"))))
      (:Finished
        (CallFunction|PlayTimeline)))))

(event EventOnInteract
  (params (PlayerRef :type BP%20Third%20Person%20Character%20Object%20Reference))
  ;[1 1 1] Using On Interact to start movement
)

(event EventMoveObjAlongSpline
  ;[1 1 1] Call Outside of Blueprint
  ;[1 1 1] Using On Interact to start movement
  (Components|Timeline|SetPlayRate (Variables|Default|GetMoveTrain_T) (/ 1.0 (Variables|Default|GetTimeOfCompleting)))
  (CallFunction|PlayTimeline))

(fn ConstructionScript
  (bind _spline (Variables|Default|GetSpline))
  (|CallParentFunction)
  (for (_array_element _array_index) (Variables|Default|GetObjectForSpLine)
    (Transformation|SetActorLocationAndRotation _array_element (Spline|GetLocationatDistanceAlongSpline _spline (* _array_index (Variables|Default|GetOffsetBetweenActors)) "World") (Spline|GetRotationatDistanceAlongSpline _spline (* _array_index (Variables|Default|GetOffsetBetweenActors)) "World"))))