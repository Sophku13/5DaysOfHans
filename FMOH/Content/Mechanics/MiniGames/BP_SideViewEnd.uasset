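; BP_SideViewEnd is the end point of the side-view minigame, offering two overlap boxes that lead to different choices or rooms.
; When a BP_PawnSideView enters ChoiceA or ChoiceB, it stores the pawn, calls DetachBook on it and records the matching choice number.
; It then passes that number and the pawn's player reference to the minigame listener through ActivateChoice.
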(event OnComponentBeginOverlap(ChoiceB)
  (params (OverlappedComponent :type Primitive%20Component%20Object%20Reference) (OtherActor :type Actor%20Object%20Reference) (OtherComp :type Primitive%20Component%20Object%20Reference) (OtherBodyIndex :type Integer) (bFromSweep :type Boolean) (SweepResult :type Hit%20Result%20Structure%20%28by%20ref%29))
  ;[0 1 0.67] Two Boxes that lead to different choices/rooms
  (bind _asbp_pawn_side_view (Utilities|Casting|CastToBP_PawnSideView OtherActor))
  (bind _output_get (Variables|Default|SetPawnRef _asbp_pawn_side_view))
  (Default|DetachBook _output_get)
  (bind _output_get_2 (Variables|Default|SetChoiceNumber 2))
  (Default|ActivateChoice (Variables|Default|GetMinigameListenerRef) _output_get_2 (Variables|/Game/Mechanics/MiniGames/InTheBook/BP_PawnSideView.BP_PawnSideView_C|GetPlayerRef _output_get)))

(event OnComponentBeginOverlap(ChoiceA)
  (params (OverlappedComponent :type Primitive%20Component%20Object%20Reference) (OtherActor :type Actor%20Object%20Reference) (OtherComp :type Primitive%20Component%20Object%20Reference) (OtherBodyIndex :type Integer) (bFromSweep :type Boolean) (SweepResult :type Hit%20Result%20Structure%20%28by%20ref%29))
  ;[0 1 0.67] Two Boxes that lead to different choices/rooms
  (bind _asbp_pawn_side_view (Utilities|Casting|CastToBP_PawnSideView OtherActor))
  (bind _output_get (Variables|Default|SetPawnRef _asbp_pawn_side_view))
  (Default|DetachBook _output_get)
  (bind _output_get_2 (Variables|Default|SetChoiceNumber 1))
  (Default|ActivateChoice (Variables|Default|GetMinigameListenerRef) _output_get_2 (Variables|/Game/Mechanics/MiniGames/InTheBook/BP_PawnSideView.BP_PawnSideView_C|GetPlayerRef _output_get)))

(event EventBeginPlay)

(event Collision|EventActorBeginOverlap
  (params (OtherActor :type Actor%20Object%20Reference)))

(event EventTick
  (params (DeltaSeconds :type Float%20%28single-precision%29)))

(fn ConstructionScript)