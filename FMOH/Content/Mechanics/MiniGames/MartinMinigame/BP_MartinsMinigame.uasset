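; Controller actor for Martin's minigame that drives every BP_Train2 spline actor in the level.
; On BeginPlay it enables player input and caches all those trains.
; InitiateEnd tells each train to move its object along its spline, while pressing N makes each fall from it.
; An unconnected leftover branch would enable physics on spline objects and destroy the trains.
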(event Custom|InitiateEnd
  (for _array_element (Variables|Default|GetSplinesRef)
    (Class|BPISplineTrain|MoveObjAlongSpline(Message) _array_element)))

(event EventBeginPlay
  (Input|EnableInput (Game|GetPlayerController 0))
  (bind _outactors (Actor|GetAllActorsOfClass "/Game/Mechanics/InteractableObjects/Train/BP_Train2.BP_Train2_C"))
  (Variables|Default|SetSplinesRef _outactors))

(event Input|KeyboardEvents|N
  (params (Key :type Key%20Structure :default "None"))
  (:Pressed
    (for _array_element (Variables|Default|GetSplinesRef)
      (Default|FallfromSpline _array_element))))

(event Input|KeyboardEvents|C
  (params (Key :type Key%20Structure :default "None")))

(fn ConstructionScript)