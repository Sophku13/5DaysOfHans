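; BP_SwitchHDRILight is a trigger actor in the Martin minigame that toggles the level's HDRI backdrop on and off.
; On BeginPlay it finds and caches the HDRIBackdrop actor.
; Each time a BP_ThirdPersonCharacter begins overlapping its Box, it flips the visibility of the backdrop's scene component and children, tracking the state in a boolean.
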(event OnComponentBeginOverlap(Box)
  (params (OverlappedComponent :type Primitive%20Component%20Object%20Reference) (OtherActor :type Actor%20Object%20Reference) (OtherComp :type Primitive%20Component%20Object%20Reference) (OtherBodyIndex :type Integer) (bFromSweep :type Boolean) (SweepResult :type Hit%20Result%20Structure%20%28by%20ref%29))
  (Utilities|Casting|CastToBP_ThirdPersonCharacter OtherActor)
  (if (not (Variables|Default|GetHDRISwitchedOff))
    (Rendering|SetVisibility (Variables|/HDRIBackdrop/Blueprints/HDRIBackdrop.HDRIBackdrop_C|GetSceneComponent (Variables|Default|GetHDRIref)) false true)
    (Variables|Default|SetHDRISwitchedOff true)
    (else
      (Rendering|SetVisibility (Variables|/HDRIBackdrop/Blueprints/HDRIBackdrop.HDRIBackdrop_C|GetSceneComponent (Variables|Default|GetHDRIref)) true true)
      (Variables|Default|SetHDRISwitchedOff false))))

(event EventBeginPlay
  (bind _returnvalue (Actor|GetActorOfClass "/HDRIBackdrop/Blueprints/HDRIBackdrop.HDRIBackdrop_C"))
  (Variables|Default|SetHDRIref _returnvalue))

(fn ConstructionScript)