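; Clue-hunt minigame board where the player finds items left by Hans's mother, ending in a secret door.
; Tick counts found items, moves the figure along saved platform transforms, lights the path, reveals matching board items and updates the room manager.
; Interacting toggles a locked board camera; BP_InterMono actors deliver narrative audio and subtitles.
; Five finds trigger the door, music and closing monologue; reset restores the figure, board items and snow.
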(event EventBeginPlay
  ;[0.07059 1 0.6196] Begin Play - Save Locations
  (|CallParentFunction)
  (Utilities|Map|Add (Variables|Default|GetQuestProgressLocations) 1 (Transformation|GetWorldTransform (Variables|Default|GetFigureLocation1)))
  (Utilities|Map|Add (Variables|Default|GetQuestProgressLocations) 2 (Transformation|GetWorldTransform (Variables|Default|GetFigureLocation2)))
  (Utilities|Map|Add (Variables|Default|GetQuestProgressLocations) 3 (Transformation|GetWorldTransform (Variables|Default|GetFigureLocation3)))
  (Utilities|Map|Add (Variables|Default|GetQuestProgressLocations) 4 (Transformation|GetWorldTransform (Variables|Default|GetFigureLocation4)))
  (Utilities|Map|Add (Variables|Default|GetQuestProgressLocations) 5 (Transformation|GetWorldTransform (Variables|Default|GetFigureLocation5)))
  (Utilities|Map|Add (Variables|Default|GetQuestProgressLocations) 6 (Transformation|GetWorldTransform (Variables|Default|GetFigureLocation6))))

(event EventOnActivation
  (params (PlayerRef :type BP%20Third%20Person%20Character%20Object%20Reference))
  (bind _secretdoorref (Variables|Default|GetSecretDoorRef))
  ;[0.07059 1 0.6196] OnActivation
  (|CallParentFunction PlayerRef)
  (Variables|Default|SetbIsQuestCompleted (Variables|Default|GetbIsActivated))
  (Default|OnActivation _secretdoorref PlayerRef)
  (Variables|/Script/Engine.Actor|SetTags _secretdoorref (Variables|Default|GetTag))
  ;[0 0.04734 1] Comment
  (bind _returnvalue (Audio|SpawnSound2D "/Game/SoundSystem/Sounds/GameMusic/Janáček-Idyll.Janáček-Idyll" 1.0 1.0 0.0 0))
  (bind _returnvalue_2 (Game|SpawnActorfromClass "/Game/SoundSystem/Sounds/BP_InterMono.BP_InterMono_C" (Transformation|GetActorTransform (Game|GetPlayerCharacter 0)) "Undefined" "MultiplyWithRoot" 0 "/Game/SoundSystem/Sounds/VoiceRecordings/Mother/1947/YourHeartIsAsBigAsMountain.YourHeartIsAsBigAsMountain" 1.0 "Hans: I remember hiding in the closet when I was a kid. I imagined a whole world behind. I never thought it would become real." 19.0 true 0))
  (Default|CheckValues _returnvalue_2)
  (Utilities|FlowControl|Delay 19.5)
  (bind _returnvalue_3 (Game|SpawnActorfromClass "/Game/SoundSystem/Sounds/BP_InterMono.BP_InterMono_C" (Transformation|GetActorTransform (Game|GetPlayerCharacter 0)) "Undefined" "MultiplyWithRoot" 0 "/Game/SoundSystem/Sounds/VoiceRecordings/Mother/1947/YourHeartIsAsBigAsMountain.YourHeartIsAsBigAsMountain" 1.0 "Mother: Tonight, I know we’ll have visitors. I know they’re coming for us. I also know that if I leave now—if I surrender to them—they’ll send me where they sent you. I know I’m taking a risk. But so many have died because of him. Someone should die against him." 24.0 true 0))
  (Default|CheckValues _returnvalue_3))

(event EventOnInteract
  (params (PlayerRef :type BP%20Third%20Person%20Character%20Object%20Reference))
  ;[0.07059 1 0.6196] On Interact
  (Variables|Default|SetPlayer%20Ref PlayerRef)
  (if (not (Variables|Default|GetbIsViewingBoard))
    (Game|Player|SetViewTargetwithBlend (Game|GetPlayerController 0) self 1.0 "VTBlend_Linear" 0.0 false)
    (Pawn|Components|CharacterMovement|SetMovementMode (Variables|/Script/Engine.Character|GetCharacterMovement (Variables|Default|GetPlayer%20Ref)) "MOVE_Flying" 0)
    (Variables|/Game/ThirdPerson/Blueprints/BP_ThirdPersonCharacter.BP_ThirdPersonCharacter_C|SetIsMovementLocked (Variables|Default|GetPlayer%20Ref) true)
    (Variables|/Game/ThirdPerson/Blueprints/BP_ThirdPersonCharacter.BP_ThirdPersonCharacter_C|SetbIsCameraLocked (Variables|Default|GetPlayer%20Ref) true)
    (Variables|Default|SetbIsViewingBoard true)
    (Utilities|FlowControl|DoOnce false
      (:Completed
        (bind _returnvalue (Game|SpawnActorfromClass "/Game/SoundSystem/Sounds/BP_InterMono.BP_InterMono_C" (Transformation|GetActorTransform (Game|GetPlayerCharacter 0)) "Undefined" "MultiplyWithRoot" 0 "/Game/SoundSystem/Sounds/VoiceRecordings/Hans/IShouldLookAround_2.IShouldLookAround_2" 1.0 "Hans: I should look around. Maybe she left something for me to find her." 4.0 true 0))
        (Default|CheckValues _returnvalue)
        (Utilities|FlowControl|Delay 4.5)
        (bind _returnvalue_2 (Game|SpawnActorfromClass "/Game/SoundSystem/Sounds/BP_InterMono.BP_InterMono_C" (Transformation|GetActorTransform (Game|GetPlayerCharacter 0)) "Undefined" "MultiplyWithRoot" 0 "/Game/SoundSystem/Sounds/VoiceRecordings/Narrator/AfterTheyKilledLucius_3.AfterTheyKilledLucius_3" 1.0 "Narrator: After they killed Lucius he stopped thinking about home. But sometimes he thought about her. Is she alright? Did she end up in the other camp?" 11.0 true 0))
        (Default|CheckValues _returnvalue_2)
        (Utilities|FlowControl|Delay 11.5)
        (bind _returnvalue_3 (Game|SpawnActorfromClass "/Game/SoundSystem/Sounds/BP_InterMono.BP_InterMono_C" (Transformation|GetActorTransform (Game|GetPlayerCharacter 0)) "Undefined" "MultiplyWithRoot" 0 0 1.0 "Sometimes he was looking at the new ones, feeling afraid that he would see her there. But part of him wanted her to come. To come and take him home." 11.0 true 0))
        (Default|CheckValues _returnvalue_3)
        (Utilities|FlowControl|Delay 11.5)))
    (else
      (Game|Player|SetViewTargetwithBlend (Game|GetPlayerController 0) (Variables|Default|GetPlayer%20Ref) 1.0 "VTBlend_Linear" 0.0 false)
      (Pawn|Components|CharacterMovement|SetMovementMode (Variables|/Script/Engine.Character|GetCharacterMovement (Variables|Default|GetPlayer%20Ref)) "MOVE_Walking" 0)
      (Variables|/Game/ThirdPerson/Blueprints/BP_ThirdPersonCharacter.BP_ThirdPersonCharacter_C|SetIsMovementLocked (Variables|Default|GetPlayer%20Ref) false)
      (Variables|/Game/ThirdPerson/Blueprints/BP_ThirdPersonCharacter.BP_ThirdPersonCharacter_C|SetbIsCameraLocked (Variables|Default|GetPlayer%20Ref) false)
      (Variables|Default|SetbIsViewingBoard false))))

(event EventOnReset
  ;[0.07059 1 0.6196] Reset
  (|CallParentFunction)
  (Transformation|SetWorldTransform (Variables|Default|GetFigure) (Variables|Default|GetStartingLocation) false false)
  (Variables|Default|SetsavedProgressCount 0)
  (bind _values (Utilities|Map|Values (Variables|Default|GetQuestItemRefList)))
  (for _array_element _values
    (Development|SetHiddeninGame (Variables|/Game/Mechanics/BaseBlueprints/BP_BaseInspectableQuestItem.BP_BaseInspectableQuestItem_C|GetStaticMesh _array_element) true false)
    (Variables|/Script/Engine.PrimitiveComponent|SetbGenerateOverlapEvents (Variables|/Game/Mechanics/BaseBlueprints/BP_BaseInspectableQuestItem.BP_BaseInspectableQuestItem_C|GetStaticMesh _array_element) false))
  (Variables|Default|SetbIsActivated false)
  (Variables|Default|SetbIsQuestCompleted false)
  (Default|ResetSnow (Variables|Default|GetRoomManagerRef)))

(event EventSaveforReset
  ;[0.07059 1 0.6196] Reset
  (Variables|Default|SetStartingLocation (Transformation|GetWorldTransform (Variables|Default|GetFigure))))

(event EventTick
  (params (DeltaSeconds :type Float%20%28single-precision%29))
  ;[0.07059 1 0.6196] Event Tick
  (for _array_element (Variables|Default|GetQuestItemMap)
    (if (Variables|/Game/Mechanics/Inspectable/QuestItems/BP_Clue_Base.BP_Clue_Base_C|GetbIsFound _array_element)
      (Math|Integer|IncrementInt (Variables|Default|GetQuestProgress))))
  (if (not (== (Variables|Default|GetQuestProgress) 0))
    (if (== (Variables|Default|GetQuestProgress) 5)
      (CallFunction|OnActivation))
    (Transformation|SetWorldTransform (Variables|Default|GetFigure) (Math|Transform|MakeTransform (.location (.Value (Utilities|Map|Find (Variables|Default|GetQuestProgressLocations) (Variables|Default|GetQuestProgress)))) (.rotation (.Value (Utilities|Map|Find (Variables|Default|GetQuestProgressLocations) (Variables|Default|GetQuestProgress)))) "1.000000,1.000000,1.000000") false false)
    (CallFunction|LightPath)
    (if (== (Variables|Default|GetQuestProgress) (Variables|Default|GetsavedProgressCount))
      _
      (else
        (bind _output_get (Variables|Default|SetsavedProgressCount (Variables|Default|GetQuestProgress)))
        (Default|UpdateRoom (Variables|Default|GetRoomManagerRef) _output_get)))
    (Variables|Default|SetQuestProgress 0)
    (Utilities|FlowControl|DoOnce false
      (:Completed
        ;[0 0.09229 1] Comment
        (if (== (Variables|Default|GetsavedProgressCount) 1)
          (bind _returnvalue (Game|SpawnActorfromClass "/Game/SoundSystem/Sounds/BP_InterMono.BP_InterMono_C" (Transformation|GetActorTransform (Game|GetPlayerCharacter 0)) "Undefined" "MultiplyWithRoot" 0 "/Game/SoundSystem/Sounds/VoiceRecordings/Mother/1947/StartedWorkingInMarch.StartedWorkingInMarch" 1.0 "Mother: I started working at the factory in March. I hated the idea of helping the army. But I wasn’t just helping them. I often wondered how we could talk about the working class without understanding it, without being part of it. Still, I doubted I could be of any real use." 19.0 true 0))
          (Default|CheckValues _returnvalue)
          (Audio|SpawnSoundatLocation "/Game/SoundSystem/Sounds/VoiceRecordings/Mother/1947/MotherLullabay_1.MotherLullabay_1" (.location (Transformation|GetActorTransform (Utilities|Array|Get(acopy) (Variables|Default|GetQuestItemMap) (- (Variables|Default|GetsavedProgressCount) 1)))) "0, 0, 0" 1.0 1.0 0.0 0 0)
          (elif (== (Variables|Default|GetsavedProgressCount) 2)
            (bind _returnvalue_2 (Game|SpawnActorfromClass "/Game/SoundSystem/Sounds/BP_InterMono.BP_InterMono_C" (Transformation|GetActorTransform (Game|GetPlayerCharacter 0)) "Undefined" "MultiplyWithRoot" 0 "/Game/SoundSystem/Sounds/VoiceRecordings/Mother/1947/BeforeIMetLise.BeforeIMetLise" 1.0 "Mother: That was before I met (Anne-)Liese. She reminded me of my sister—restless, reckless, always stirring up trouble." 7.0 true 0))
            (Default|CheckValues _returnvalue_2)
            (Audio|SpawnSoundatLocation "/Game/SoundSystem/Sounds/VoiceRecordings/Mother/1947/MotherLullabay_1.MotherLullabay_1" (.location (Transformation|GetActorTransform (Utilities|Array|Get(acopy) (Variables|Default|GetQuestItemMap) (- (Variables|Default|GetsavedProgressCount) 1)))) "0, 0, 0" 1.0 1.0 0.0 0 0)
            (elif (== (Variables|Default|GetsavedProgressCount) 3)
              (bind _returnvalue_3 (Game|SpawnActorfromClass "/Game/SoundSystem/Sounds/BP_InterMono.BP_InterMono_C" (Transformation|GetActorTransform (Game|GetPlayerCharacter 0)) "Undefined" "MultiplyWithRoot" 0 "/Game/SoundSystem/Sounds/VoiceRecordings/Mother/1947/WhenInvitationCame.WhenInvitationCame" 1.0 "Mother: When the invitation came to join the organization, I almost laughed. What could a handful of women do against the monster that had swallowed our country? But they fought back. And more than anything, they could help with what mattered most—finding you." 17.0 true 0))
              (Audio|SpawnSoundatLocation "/Game/SoundSystem/Sounds/VoiceRecordings/Mother/1947/MotherLullabay_1.MotherLullabay_1" (.location (Transformation|GetActorTransform (Utilities|Array|Get(acopy) (Variables|Default|GetQuestItemMap) (- (Variables|Default|GetsavedProgressCount) 1)))) "0, 0, 0" 1.0 1.0 0.0 0 0)
              (Default|CheckValues _returnvalue_3)
              (Utilities|FlowControl|Delay 17.5)
              (bind _returnvalue_4 (Game|SpawnActorfromClass "/Game/SoundSystem/Sounds/BP_InterMono.BP_InterMono_C" (Transformation|GetActorTransform (Game|GetPlayerCharacter 0)) "Undefined" "MultiplyWithRoot" 0 "/Game/SoundSystem/Sounds/VoiceRecordings/Hans/SheWasLookingForMe.SheWasLookingForMe" 1.0 "She was looking for me…" 1.0 true 0))
              (Default|CheckValues _returnvalue_4)
              (elif (== (Variables|Default|GetsavedProgressCount) 4)
                (bind _returnvalue_5 (Game|SpawnActorfromClass "/Game/SoundSystem/Sounds/BP_InterMono.BP_InterMono_C" (Transformation|GetActorTransform (Game|GetPlayerCharacter 0)) "Undefined" "MultiplyWithRoot" 0 "/Game/SoundSystem/Sounds/VoiceRecordings/Mother/1947/LiseToldMeAboutAnna.LiseToldMeAboutAnna" 1.0 "Mother: Liese told me about Anna. Sometimes I felt ashamed, for using your room to hide her. But at night, when I heard the faint rustling from the other side of the wall, I felt a little less alone. I pretended it was you. And on those quiet evenings, when I came home and we shared a meal together, I realized—I don’t know which one of us saved the other. Maybe it was Anna who saved me." 19.0 true 0))
                (Default|CheckValues _returnvalue_5)
                (Audio|SpawnSoundatLocation "/Game/SoundSystem/Sounds/VoiceRecordings/Mother/1947/MotherLullabay_1.MotherLullabay_1" (.location (Transformation|GetActorTransform (Utilities|Array|Get(acopy) (Variables|Default|GetQuestItemMap) (- (Variables|Default|GetsavedProgressCount) 1)))) "0, 0, 0" 1.0 1.0 0.0 0 0)
                (elif (== (Variables|Default|GetsavedProgressCount) 5)
                  (bind _returnvalue_6 (Game|SpawnActorfromClass "/Game/SoundSystem/Sounds/BP_InterMono.BP_InterMono_C" (Transformation|GetActorTransform (Game|GetPlayerCharacter 0)) "Undefined" "MultiplyWithRoot" 0 "/Game/SoundSystem/Sounds/VoiceRecordings/Mother/1947/YourHeartIsAsBigAsMountain.YourHeartIsAsBigAsMountain" 1.0 "Mother: I love you, darling. Your heart is as vast as the mountains. Remember that." 19.0 true 0))
                  (Default|CheckValues _returnvalue_6)
                  (Audio|SpawnSoundatLocation "/Game/SoundSystem/Sounds/VoiceRecordings/Mother/1947/MotherLullabay_1.MotherLullabay_1" (.location (Transformation|GetActorTransform (Utilities|Array|Get(acopy) (Variables|Default|GetQuestItemMap) (- (Variables|Default|GetsavedProgressCount) 1)))) "0, 0, 0" 1.0 1.0 0.0 0 0))))))))))

(fn ConstructionScript
  (|CallParentFunction))

(fn LightPath
  (for _array_element (Variables|Default|GetQuestItemMap)
    (if (Variables|/Game/Mechanics/Inspectable/QuestItems/BP_Clue_Base.BP_Clue_Base_C|GetbIsFound _array_element)
      (Development|SetHiddeninGame (Variables|/Game/Mechanics/BaseBlueprints/BP_BaseInspectableQuestItem.BP_BaseInspectableQuestItem_C|GetStaticMesh (.Value (Utilities|Map|Find (Variables|Default|GetQuestItemRefList) (Variables|/Game/Mechanics/Inspectable/QuestItems/BP_Clue_Base.BP_Clue_Base_C|GetNumber _array_element)))) false false)
      (Variables|/Script/Engine.PrimitiveComponent|SetbGenerateOverlapEvents (Variables|/Game/Mechanics/BaseBlueprints/BP_BaseInspectableQuestItem.BP_BaseInspectableQuestItem_C|GetStaticMesh (.Value (Utilities|Map|Find (Variables|Default|GetQuestItemRefList) (Variables|/Game/Mechanics/Inspectable/QuestItems/BP_Clue_Base.BP_Clue_Base_C|GetNumber _array_element)))) true)))
  (for _index (range 1 (Variables|Default|GetQuestProgress))
    ;[0 1 0.664] Updating new Paths and Locations
    (if (== _index 1)
      (Variables|/Script/Text3D.Text3DComponent|SetFrontMaterial (Variables|Default|GetNumber1) "/Engine/VREditor/BasicMeshes/MI_Cube_03.MI_Cube_03")
      (elif (== _index 2)
        (Variables|/Script/Text3D.Text3DComponent|SetFrontMaterial (Variables|Default|GetPath1) "/Engine/VREditor/BasicMeshes/MI_Cube_03.MI_Cube_03")
        (Variables|/Script/Text3D.Text3DComponent|SetFrontMaterial (Variables|Default|GetNumber2) "/Engine/VREditor/BasicMeshes/MI_Cube_03.MI_Cube_03")
        ;[0 1 0.664] Changing old numbers
        (Variables|/Script/Text3D.Text3DComponent|SetFrontMaterial (Variables|Default|GetNumber1) "/Engine/VREditor/BasicMeshes/MI_Cube_01.MI_Cube_01")
        (elif (== _index 3)
          (Variables|/Script/Text3D.Text3DComponent|SetFrontMaterial (Variables|Default|GetPath2) "/Engine/VREditor/BasicMeshes/MI_Cube_03.MI_Cube_03")
          (Variables|/Script/Text3D.Text3DComponent|SetFrontMaterial (Variables|Default|GetNumber3) "/Engine/VREditor/BasicMeshes/MI_Cube_03.MI_Cube_03")
          (Variables|/Script/Text3D.Text3DComponent|SetFrontMaterial (Variables|Default|GetPath1) "/Engine/VREditor/BasicMeshes/MI_Cube_01.MI_Cube_01")
          (Variables|/Script/Text3D.Text3DComponent|SetFrontMaterial (Variables|Default|GetNumber2) "/Engine/VREditor/BasicMeshes/MI_Cube_01.MI_Cube_01")
          (elif (== _index 4)
            (Variables|/Script/Text3D.Text3DComponent|SetFrontMaterial (Variables|Default|GetPath3) "/Engine/VREditor/BasicMeshes/MI_Cube_03.MI_Cube_03")
            (Variables|/Script/Text3D.Text3DComponent|SetFrontMaterial (Variables|Default|GetNumber4) "/Engine/VREditor/BasicMeshes/MI_Cube_03.MI_Cube_03")
            (Variables|/Script/Text3D.Text3DComponent|SetFrontMaterial (Variables|Default|GetPath2) "/Engine/VREditor/BasicMeshes/MI_Cube_01.MI_Cube_01")
            (Variables|/Script/Text3D.Text3DComponent|SetFrontMaterial (Variables|Default|GetNumber3) "/Engine/VREditor/BasicMeshes/MI_Cube_01.MI_Cube_01")
            (elif (== _index 5)
              (Variables|/Script/Text3D.Text3DComponent|SetFrontMaterial (Variables|Default|GetPath4) "/Engine/VREditor/BasicMeshes/MI_Cube_03.MI_Cube_03")
              (Variables|/Script/Text3D.Text3DComponent|SetFrontMaterial (Variables|Default|GetNumber5) "/Engine/VREditor/BasicMeshes/MI_Cube_03.MI_Cube_03")
              (Variables|/Script/Text3D.Text3DComponent|SetFrontMaterial (Variables|Default|GetPath3) "/Engine/VREditor/BasicMeshes/MI_Cube_01.MI_Cube_01")
              (Variables|/Script/Text3D.Text3DComponent|SetFrontMaterial (Variables|Default|GetNumber4) "/Engine/VREditor/BasicMeshes/MI_Cube_01.MI_Cube_01")
              (Development|SetHiddeninGame (Variables|Default|GetPath5) false false)
              (Development|SetHiddeninGame (Variables|Default|GetNumber6) false false)
              (Development|SetHiddeninGame (Variables|Default|GetFigurePlatform6) false false)
              (elif (== _index 6)
                (Variables|/Script/Text3D.Text3DComponent|SetFrontMaterial (Variables|Default|GetPath5) "/Engine/VREditor/BasicMeshes/MI_Cube_03.MI_Cube_03")
                (Variables|/Script/Text3D.Text3DComponent|SetFrontMaterial (Variables|Default|GetNumber6) "/Engine/VREditor/BasicMeshes/MI_Cube_03.MI_Cube_03")
                (Variables|/Script/Text3D.Text3DComponent|SetFrontMaterial (Variables|Default|GetPath4) "/Engine/VREditor/BasicMeshes/MI_Cube_01.MI_Cube_01")
                (Variables|/Script/Text3D.Text3DComponent|SetFrontMaterial (Variables|Default|GetNumber5) "/Engine/VREditor/BasicMeshes/MI_Cube_01.MI_Cube_01")))))))))