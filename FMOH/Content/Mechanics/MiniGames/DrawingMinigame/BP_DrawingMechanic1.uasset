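; Interactable drawing board for the drawing minigame, letting the player paint on it with the mouse.
; Interacting toggles a mode that blends the view to the board, shows the cursor, enables input and locks player movement and camera.
; While left mouse is held, Tick traces from the cursor and passes the hit's collision UV to an M_Marker dynamic material drawn into RT_ArtBoard.
; BeginPlay and OnReset clear that render target.
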(event Custom|DrawOnBoard
  (params (LocationToDraw :type Vector%202D%20Structure))
  (bind _mi_drawingmarker (Variables|Default|GetMI_DrawingMarker))
  (Rendering|Material|SetVectorParameterValue _mi_drawingmarker "DrawLocation" (Math|Conversions|ToLinearColor(Vector) (Math|Conversions|ToVector(Vector2D) LocationToDraw)) :!class /Script/Engine.MaterialInstanceDynamic)
  (Rendering|DrawMaterialtoRenderTarget "/Game/Mechanics/MiniGames/DrawingMinigame/RT_ArtBoard.RT_ArtBoard" _mi_drawingmarker))

(event EventBeginPlay
  (|CallParentFunction)
  (bind _returnvalue (Rendering|Material|CreateDynamicMaterialInstance "/Game/Mechanics/MiniGames/DrawingMinigame/M_Marker.M_Marker" "None" "None" :!class /Script/Engine.KismetMaterialLibrary))
  (Variables|Default|SetMI_DrawingMarker _returnvalue)
  (Rendering|ClearRenderTarget2D "/Game/Mechanics/MiniGames/DrawingMinigame/RT_ArtBoard.RT_ArtBoard"))

(event EventTick
  (params (DeltaSeconds :type Float%20%28single-precision%29))
  (bind _returnvalue (Game|GetPlayerController 0))
  (bind (_worldlocation _worlddirection) (Game|Player|ConvertMouseLocationToWorldSpace _returnvalue))
  (if (Variables|Default|GetIsDrawing)
    (bind _outhit (Collision|LineTraceByChannel _worldlocation (+ _worldlocation (* _worlddirection (Math|Conversions|ToVector(Float) 1e+03))) "TraceTypeQuery1" true 0 "None" false))
    (CallFunction|DrawonBoard (.UV (Class|GameplayStatics|FindCollisionUV _outhit)))))

(event EventOnReset
  (bind _returnvalue (Rendering|Material|CreateDynamicMaterialInstance "/Game/Mechanics/MiniGames/DrawingMinigame/M_Marker.M_Marker" "None" "None" :!class /Script/Engine.KismetMaterialLibrary))
  (Variables|Default|SetMI_DrawingMarker _returnvalue)
  (Rendering|ClearRenderTarget2D "/Game/Mechanics/MiniGames/DrawingMinigame/RT_ArtBoard.RT_ArtBoard"))

(event EventOnInteract
  (params (PlayerRef :type BP%20Third%20Person%20Character%20Object%20Reference))
  (bind _returnvalue (Game|GetPlayerController 0))
  (Variables|Default|SetPlayer%20Ref PlayerRef)
  (Utilities|FlowControl|FlipFlop
    (:A
      (Variables|/Script/Engine.PlayerController|SetbShowMouseCursor _returnvalue true)
      (Variables|/Game/ThirdPerson/Blueprints/BP_ThirdPersonCharacter.BP_ThirdPersonCharacter_C|SetIsMovementLocked (Variables|Default|GetPlayer%20Ref) true)
      (Variables|/Game/ThirdPerson/Blueprints/BP_ThirdPersonCharacter.BP_ThirdPersonCharacter_C|SetbIsCameraLocked (Variables|Default|GetPlayer%20Ref) true)
      (Game|Player|SetViewTargetwithBlend _returnvalue self 1.0 "VTBlend_Linear" 0.0 false)
      (Input|EnableInput _returnvalue))
    (:B
      (Variables|/Script/Engine.PlayerController|SetbShowMouseCursor _returnvalue false)
      (Variables|/Game/ThirdPerson/Blueprints/BP_ThirdPersonCharacter.BP_ThirdPersonCharacter_C|SetIsMovementLocked (Variables|Default|GetPlayer%20Ref) false)
      (Variables|/Game/ThirdPerson/Blueprints/BP_ThirdPersonCharacter.BP_ThirdPersonCharacter_C|SetbIsCameraLocked (Variables|Default|GetPlayer%20Ref) false)
      (Game|Player|SetViewTargetwithBlend _returnvalue (Variables|Default|GetPlayer%20Ref) 1.0 "VTBlend_Linear" 0.0 false)
      (Input|DisableInput _returnvalue)
      (Input|SetInputModeGameOnly _returnvalue false))))

(event Input|MouseEvents|LeftMouseButton
  (params (Key :type Key%20Structure :default "None"))
  (:Pressed
    (Variables|Default|SetIsDrawing true))
  (:Released
    (Variables|Default|SetIsDrawing false)))

(fn ConstructionScript
  (|CallParentFunction))