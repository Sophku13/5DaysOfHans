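; BP_Needle is the interactable needle of the vinyl player in the 1969 minigame, starting and stopping the record's spin.
; Interacting plays a timeline forward or in reverse, swinging the Anchor's yaw to move the needle on or off.
; When either swing finishes, it toggles IsActive and sets IsTurning to match on the BP_VinylPlayer found in the level at BeginPlay.
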(event EventBeginPlay
  (|CallParentFunction)
  (bind _returnvalue (Actor|GetActorOfClass "/Game/Mechanics/MiniGames/1969/BP_VinylPlayer.BP_VinylPlayer_C"))
  (Variables|Default|SetVinylPlayerRef _returnvalue))

(event Collision|EventActorBeginOverlap
  (params (OtherActor :type Actor%20Object%20Reference)))

(event EventOnInteract
  (params (PlayerRef :type BP%20Third%20Person%20Character%20Object%20Reference))
  (bind _vinylplayerref (Variables|Default|GetVinylPlayerRef))
  (if (not (Variables|Default|GetbIsActive))
    (bind _newtrack_0 (Timeline|Timeline PlayFromStart)
      (:Update
        (Transformation|SetRelativeRotation (Variables|Default|GetAnchor) (Math|Rotator|MakeRotator 0.0 0.0 (Math|Float|Lerp 0.0 35.0 _newtrack_0)) false false))
      (:Finished
        (if (not (Variables|Default|GetbIsActive))
          (Variables|Default|SetbIsActive true)
          (Variables|/Game/Mechanics/MiniGames/1969/BP_VinylPlayer.BP_VinylPlayer_C|SetbIsTurning _vinylplayerref true)
          (else
            (Variables|Default|SetbIsActive false)
            (Variables|/Game/Mechanics/MiniGames/1969/BP_VinylPlayer.BP_VinylPlayer_C|SetbIsTurning _vinylplayerref false)))))
    (else
      (Timeline|Timeline ReverseFromEnd))))

(fn ConstructionScript
  (|CallParentFunction))