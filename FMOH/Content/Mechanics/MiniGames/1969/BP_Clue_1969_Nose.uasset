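; BP_Clue_1969_Nose is the nose clue in the 1969 minigame, which hands interaction over to a linked pickup.
; Interacting empty-handed flags the clue found and runs parent logic; if it can be found, it hides, disables mesh overlaps and triggers the pickup.
; SaveforReset unhides the pickup for a found clue, while OnReset teleports the clue to its BeginPlay transform and clears the found flag.
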(event Collision|EventActorBeginOverlap
  (params (OtherActor :type Actor%20Object%20Reference))
  (|CallParentFunction OtherActor) ; This node is disabled and will not be called.\nDrag off pins to build functionality.
)

(event EventTick
  (params (DeltaSeconds :type Float%20%28single-precision%29))
  (|CallParentFunction DeltaSeconds) ; This node is disabled and will not be called.\nDrag off pins to build functionality.
)

(event EventOnInteract
  (params (PlayerRef :type BP%20Third%20Person%20Character%20Object%20Reference))
  (Variables|Default|SetPlayer%20Ref PlayerRef)
  (if (not (Variables|/Game/ThirdPerson/Blueprints/BP_ThirdPersonCharacter.BP_ThirdPersonCharacter_C|GetbIsCarryingItem PlayerRef))
    (Variables|/Game/ThirdPerson/Blueprints/BP_ThirdPersonCharacter.BP_ThirdPersonCharacter_C|SetbIsMovingOn PlayerRef true)
    (Variables|Default|SetbIsFound true)
    (|CallParentFunction PlayerRef)
    (if (Variables|Default|GetbCanBeFound)
      (Rendering|SetActorHiddenInGame true)
      (Variables|/Script/Engine.PrimitiveComponent|SetbGenerateOverlapEvents (Variables|Default|GetStaticMesh) false)
      (Default|OnInteract (Variables|Default|GetPickUpRef) PlayerRef))))

(event EventSaveforReset
  (if (Variables|Default|GetbIsFound)
    (Rendering|SetActorHiddenInGame (Variables|Default|GetPickUpRef) false)
    (Variables|/Game/ThirdPerson/Blueprints/BP_ThirdPersonCharacter.BP_ThirdPersonCharacter_C|SetbIsMovingOn (Variables|Default|GetPlayer%20Ref) true)))

(event EventOnReset
  (Transformation|SetActorTransform (Variables|Default|GetStartPosition) false true)
  (Variables|Default|SetbIsFound false))

(event EventBeginPlay
  (Variables|Default|SetStartPosition (Transformation|GetActorTransform)))

(fn ConstructionScript
  (|CallParentFunction))