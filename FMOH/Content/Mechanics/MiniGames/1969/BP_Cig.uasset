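; Cigarette pickup actor for the 1969 minigame, collected through an interact event.
; On interact it hides itself rather than being destroyed, then finds the BP_CigPlanter via GetActorOfClass and passes itself to CigPickedUp.
; The construction script applies the CigMesh variable to the Cig mesh component, so the look can vary per instance.
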(event EventBeginPlay
  (|CallParentFunction) ; This node is disabled and will not be called.\nDrag off pins to build functionality.
)

(event Collision|EventActorBeginOverlap
  (params (OtherActor :type Actor%20Object%20Reference)))

(event EventTick
  (params (DeltaSeconds :type Float%20%28single-precision%29)))

(event EventOnInteract
  (params (PlayerRef :type BP%20Third%20Person%20Character%20Object%20Reference))
  (Rendering|SetActorHiddenInGame true)
  (bind _returnvalue (Actor|GetActorOfClass "/Game/Mechanics/MiniGames/1969/BP_CigPlanter.BP_CigPlanter_C"))
  (Default|CigPickedUp _returnvalue self))

(fn ConstructionScript
  (|CallParentFunction)
  (Components|StaticMesh|SetStaticMesh (Variables|Default|GetCig) (Variables|Default|GetCigMesh)))