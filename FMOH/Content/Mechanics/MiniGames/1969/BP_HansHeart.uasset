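; BP_HansHeart is an interactable heart prop in the 1969 minigame that breaks when the player interacts with it.
; On interact it records the heart mesh's world transform, then hides the mesh and disables its collision.
; It spawns a BP_BreakingHeart actor at that transform, swapping the intact heart for the breaking version instead of destroying itself.
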(event EventBeginPlay
  (|CallParentFunction) ; This node is disabled and will not be called.\nDrag off pins to build functionality.
)

(event EventOnInteract
  (params (PlayerRef :type BP%20Third%20Person%20Character%20Object%20Reference))
  (bind _heartmesh (Variables|Default|GetHeartMesh))
  (Variables|Default|SetSpawnTransform (Transformation|GetWorldTransform (Variables|Default|GetHeartMesh)))
  (Rendering|SetVisibility _heartmesh false false)
  (Collision|SetCollisionEnabled _heartmesh "NoCollision")
  (Game|SpawnActorfromClass "/Game/Mechanics/MiniGames/1969/BP_BreakingHeart.BP_BreakingHeart_C" (Variables|Default|GetSpawnTransform) "Undefined" "MultiplyWithRoot" 0 0))

(fn ConstructionScript
  (|CallParentFunction))