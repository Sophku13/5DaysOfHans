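; BP_CigPlanter is the 1969 minigame planter where the player picks up cigarettes in a close-up view.
; Interacting locks the player, blends the camera to the planter and enables the cursor, with click traces forwarding interact messages to hit actors.
; CigPickedUp collects cigarettes until six complete the quest, returning the camera and opening the WBP_1969 widget in UI-only input.
; OnReset unhides collected cigarettes and clears completion.
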(event Custom|CigPickedUp
  (params (Cig :type BP%20Cig%20Object%20Reference%20%28by%20ref%29))
  (bind _ciglist (Variables|Default|GetCigList))
  (Utilities|Array|Add _ciglist Cig)
  (if (>= (Utilities|Array|Length _ciglist) 6)
    (CallFunction|OnActivation (Variables|Default|GetPlayer%20Ref))))

(event EventOnReset
  (bind _ciglist (Variables|Default|GetCigList))
  ;[1 1 1] Reset
  (for _array_element _ciglist
    (Rendering|SetActorHiddenInGame _array_element false))
  (Utilities|Array|Clear _ciglist)
  (Variables|Default|SetbQuestCompleted false))

(event EventOnActivation
  (params (PlayerRef :type BP%20Third%20Person%20Character%20Object%20Reference))
  (bind _returnvalue (Game|GetPlayerController 0))
  (bind _returnvalue_2 (Game|GetPlayerController 0))
  ;[1 1 1] Comment
  (Variables|Default|SetbQuestCompleted true)
  (bind _output_get (Variables|Default|SetPlayer%20Ref PlayerRef))
  (Variables|/Game/ThirdPerson/Blueprints/BP_ThirdPersonCharacter.BP_ThirdPersonCharacter_C|SetIsMovementLocked _output_get false)
  (Variables|/Game/ThirdPerson/Blueprints/BP_ThirdPersonCharacter.BP_ThirdPersonCharacter_C|SetbIsCameraLocked _output_get false)
  (Variables|/Script/Engine.PlayerController|SetbShowMouseCursor _returnvalue_2 false)
  (Input|SetInputModeGameOnly _returnvalue_2 false)
  (Game|Player|SetViewTargetwithBlend _returnvalue_2 (Game|GetPlayerCharacter 0) 1.0 "VTBlend_Linear" 0.0 false)
  (Input|DisableInput (Game|GetPlayerController 0))
  (bind _returnvalue_3 (UserInterface|CreateWidget "/Game/Mechanics/MiniGames/1969/WBP_1969.WBP_1969_C" 0 (Variables|Default|GetObject%20Description) (Variables|Default|GetPlayer%20Ref) "Nose"))
  (UserInterface|Viewport|AddtoViewport _returnvalue_3 0)
  (Input|SetInputModeUIOnly _returnvalue 0 "DoNotLock" false)
  (Variables|/Script/Engine.PlayerController|SetbShowMouseCursor _returnvalue true))

(event EventOnInteract
  (params (PlayerRef :type BP%20Third%20Person%20Character%20Object%20Reference))
  (bind _returnvalue (Game|GetPlayerController 0))
  ;[1 1 1] Switch the View
  (if (not (Variables|Default|GetbQuestCompleted))
    (bind _output_get (Variables|Default|SetPlayer%20Ref PlayerRef))
    (Variables|/Game/ThirdPerson/Blueprints/BP_ThirdPersonCharacter.BP_ThirdPersonCharacter_C|SetIsMovementLocked _output_get true)
    (Variables|/Game/ThirdPerson/Blueprints/BP_ThirdPersonCharacter.BP_ThirdPersonCharacter_C|SetbIsCameraLocked _output_get true)
    (Variables|/Script/Engine.PlayerController|SetbShowMouseCursor _returnvalue true)
    (Game|Player|SetViewTargetwithBlend _returnvalue self 1.0 "VTBlend_Linear" 0.0 false)
    (Input|SetInputModeGameandUI (Game|GetPlayerController 0) 0 "DoNotLock" true false)
    (Input|EnableInput (Game|GetPlayerController 0))))

(event Input|MouseEvents|LeftMouseButton
  (params (Key :type Key%20Structure :default "None"))
  (bind _returnvalue (Game|GetPlayerController 0))
  (bind (_worldlocation _worlddirection) (Game|Player|ConvertMouseLocationToWorldSpace _returnvalue))
  ;[1 1 1] Comment
  (:Pressed
    (bind _outhit (Collision|LineTraceByChannel _worldlocation (+ _worldlocation (* _worlddirection (Math|Conversions|ToVector(Float) 5e+02))) "TraceTypeQuery1" false 0 "None" false))
    (Class|BPIInteractable|OnInteract(Message) (.HitActor (Collision|BreakHitResult _outhit)) (Variables|Default|GetPlayer%20Ref))))

(fn ConstructionScript
  (|CallParentFunction))