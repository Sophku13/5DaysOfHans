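; Base carryable quest item for the 1969 minigame, with mesh and material set in the construction script.
; Interacting attaches it to the player's socket, if their hands are free, and has BP_1969Manager activate positions for it.
; Placing it at a quest location completes it, while dropping or resetting returns it to its cached start transform.
; Widget open events shift it by an offset, and it can be hidden.
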(event Custom|PlaceInQuestLocation
  (params (QuestItemLocation :type Transform))
  (bind (_location _rotation) (Math|Transform|BreakTransform QuestItemLocation))
  (Transformation|DetachFromActor self "KeepRelative" "KeepRelative" "KeepRelative")
  (Variables|Default|SetbIsPickedUp false)
  (Transformation|SetActorLocationAndRotation self _location _rotation)
  (Variables|Default|SetbIsQuestCompleted true)
  (Variables|/Game/ThirdPerson/Blueprints/BP_ThirdPersonCharacter.BP_ThirdPersonCharacter_C|SetbIsCarryingItem (Variables|Default|GetPlayer%20Ref) false))

(event Custom|MakeInvisible
  (Rendering|SetActorHiddenInGame true))

(event Custom|WidetWithTextIsOpen
  (Transformation|SetActorLocation (+ (Transformation|GetActorLocation) (Variables|Default|GetOffsetForTextWidget)) false false))

(event Custom|WidgetWithoutTextIsOpen
  (Transformation|SetActorLocation (- (Transformation|GetActorLocation) (Variables|Default|GetOffsetForTextWidget)) false false))

(event Input|EnhancedActionEvents|EnhancedInputActionIA_Drop
  (params (ActionValue :type Boolean) (ElapsedSeconds :type Float%20%28double-precision%29) (TriggeredSeconds :type Float%20%28double-precision%29) (InputAction :type Input%20Action%20Object%20Reference :default "/Game/Character/Input/Actions/IA_Drop.IA_Drop"))
  (bind _startinglocation (Variables|Default|GetStartingLocation))
  (if (Variables|Default|GetbIsPickedUp)
    (Transformation|DetachFromActor self "KeepRelative" "KeepRelative" "KeepRelative")
    (Variables|Default|SetbIsPickedUp false)
    (Transformation|SetActorLocationAndRotation self (.location _startinglocation) (.rotation _startinglocation) false true)
    (Variables|/Game/ThirdPerson/Blueprints/BP_ThirdPersonCharacter.BP_ThirdPersonCharacter_C|SetbIsCarryingItem (Variables|Default|GetPlayer%20Ref) false)))

(event EventBeginPlay
  (|CallParentFunction)
  (Variables|Default|SetStartingLocation (Transformation|GetWorldTransform (Variables|Default|GetQuestItemMesh)))
  (bind _returnvalue (Actor|GetActorOfClass "/Game/Mechanics/MiniGames/1969/BP_1969Manager.BP_1969Manager_C"))
  (Variables|Default|SetManagerRef _returnvalue))

(event Collision|EventActorBeginOverlap
  (params (OtherActor :type Actor%20Object%20Reference))
  (|CallParentFunction OtherActor) ; This node is disabled and will not be called.\nDrag off pins to build functionality.
)

(event EventOnReset
  (bind _startinglocation (Variables|Default|GetStartingLocation))
  (|CallParentFunction)
  (Transformation|SetActorLocationAndRotation self (.location _startinglocation) (.rotation _startinglocation) false true)
  (Variables|Default|SetbIsQuestCompleted false)
  (Variables|Default|SetbIsActivated false)
  (Variables|Default|SetbIsPickedUp false))

(event EventOnInteract
  (params (PlayerRef :type BP%20Third%20Person%20Character%20Object%20Reference))
  (Variables|Default|SetPlayer%20Ref PlayerRef)
  (if (and (not (Variables|Default|GetbIsQuestCompleted)) (not (Variables|/Game/ThirdPerson/Blueprints/BP_ThirdPersonCharacter.BP_ThirdPersonCharacter_C|GetbIsCarryingItem PlayerRef)))
    (Variables|/Game/ThirdPerson/Blueprints/BP_ThirdPersonCharacter.BP_ThirdPersonCharacter_C|SetbIsCarryingItem PlayerRef true)
    (Transformation|AttachComponentToComponent (Variables|/Script/Engine.Character|GetMesh PlayerRef) "VBItemAttachSocket" "SnapToTarget" "SnapToTarget" "KeepRelative" false)
    (Variables|Default|SetbIsPickedUp true)
    (Default|ActivatePositions (Variables|Default|GetManagerRef) (Variables|Default|GetMesh) self)))

(event EventSaveforReset
  (|CallParentFunction))

(fn ConstructionScript
  (bind _questitemmesh (Variables|Default|GetQuestItemMesh))
  (|CallParentFunction)
  (Components|StaticMesh|SetStaticMesh _questitemmesh (Variables|Default|GetMesh))
  (Rendering|Material|SetMaterial _questitemmesh 0 (Variables|Default|GetMaterial)))