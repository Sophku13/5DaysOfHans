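; One-way or paired portal actor that reveals itself when the third-person character enters its activation trigger, also interacting with any linked locked door and clearing its key flag.
; Once active, its teleport box moves overlapping actors to TeleportLocation, sets player control rotation, plays a sound and briefly disables camera rotation lag.
; Each tick, PortalView copies camera rotation with a 180 or 90 degree yaw offset for the portal image.
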(event OnComponentBeginOverlap(TeleportBox)
  (params (OverlappedComponent :type Primitive%20Component%20Object%20Reference) (OtherActor :type Actor%20Object%20Reference) (OtherComp :type Primitive%20Component%20Object%20Reference) (OtherBodyIndex :type Integer) (bFromSweep :type Boolean) (SweepResult :type Hit%20Result%20Structure%20%28by%20ref%29))
  (bind _returnvalue (Game|GetPlayerCharacter 0))
  (bind _teleportlocation (Variables|Default|GetTeleportLocation))
  (bind _returnvalue_2 (Transformation|GetActorTransform _returnvalue))
  (bind _relativerotation (Variables|/Script/Engine.SceneComponent|GetRelativeRotation _teleportlocation))
  ;[1 1 1] Teleportation through Portal Frames
  (if (Variables|Default|GetbIsActive)
    (if (Variables|Default|GetbCanTeleport)
      (Variables|/Script/Engine.SpringArmComponent|SetbEnableCameraRotationLag (Variables|/Game/ThirdPerson/Blueprints/BP_ThirdPersonCharacter.BP_ThirdPersonCharacter_C|GetCameraBoom (Variables|Default|GetPlayerRef)) false)
      (Variables|Default|SetbCanTeleport false)
      (Transformation|SetActorLocationAndRotation OtherActor (Transformation|GetWorldLocation _teleportlocation) "0, 0, 0" false true)
      (Pawn|SetControlRotation (Game|GetPlayerController (Variables|/Script/Engine.Pawn|GetPlayerState (Game|GetPlayerCharacter 0))) (Math|Rotator|MakeRotator (.roll _relativerotation) (.pitch _relativerotation) (.yaw _relativerotation)))
      (Audio|PlaySoundatLocation (Variables|Default|GetSound) (.location _returnvalue_2) (.rotation _returnvalue_2) 1.0 1.0 0.0 0 0 0 0)
      (Variables|Default|SetbCanTeleport true)
      (Utilities|FlowControl|Delay 1.0)
      (Variables|/Script/Engine.SpringArmComponent|SetbEnableCameraRotationLag (Variables|/Game/ThirdPerson/Blueprints/BP_ThirdPersonCharacter.BP_ThirdPersonCharacter_C|GetCameraBoom (Variables|Default|GetPlayerRef)) true))))

(event OnComponentBeginOverlap(ActivationTrigger)
  (params (OverlappedComponent :type Primitive%20Component%20Object%20Reference) (OtherActor :type Actor%20Object%20Reference) (OtherComp :type Primitive%20Component%20Object%20Reference) (OtherBodyIndex :type Integer) (bFromSweep :type Boolean) (SweepResult :type Hit%20Result%20Structure%20%28by%20ref%29))
  (bind _asbp_third_person_character (Utilities|Casting|CastToBP_ThirdPersonCharacter OtherActor))
  (Variables|Default|SetPlayerRef _asbp_third_person_character)
  (Development|SetHiddeninGame (Variables|Default|GetPortalMesh) false false)
  (Variables|Default|SetbIsActive true)
  (bind _lockeddoorref (Variables|Default|GetLockedDoorRef)
    (:then
      (Default|OnInteract _lockeddoorref)
      (Variables|/Game/Mechanics/InteractableObjects/BP_DoorKeyLocked.BP_DoorKeyLocked_C|SetbIsDoorKeyAquired _lockeddoorref false))
    (:else)))

(event Custom|Reset
  ;[1 1 1] Comment
  (Variables|/Script/Engine.PrimitiveComponent|SetbGenerateOverlapEvents (Variables|Default|GetTeleportBox) true)
  (Development|SetHiddeninGame (Variables|Default|GetPortalMesh) true false)
  (Variables|Default|SetbIsActive true))

(event EventBeginPlay)

(event Collision|EventActorBeginOverlap
  (params (OtherActor :type Actor%20Object%20Reference)))

(event EventTick
  (params (DeltaSeconds :type Float%20%28single-precision%29))
  (bind _returnvalue (Game|GetPlayerCameraManager 0))
  (bind _portalview (Variables|Default|GetPortalView))
  (bind _returnvalue_2 (Transformation|GetWorldLocation _portalview))
  (bind _transformcomponent (Variables|/Script/Engine.PlayerCameraManager|GetTransformComponent _returnvalue))
  (bind _returnvalue_3 (Transformation|GetWorldRotation _transformcomponent))
  ;[1 1 1] Portal Image is moving aligned with the player in Portall 1
  (if (not (Variables|Default|GetbIs90DegreesTurned))
    (Transformation|SetWorldLocationAndRotation _portalview _returnvalue_2 (Math|Rotator|MakeRotator (.roll _returnvalue_3) (.pitch _returnvalue_3) (- (.yaw _returnvalue_3) 1.8e+02)) false false)
    (else
      (Transformation|SetWorldLocationAndRotation _portalview _returnvalue_2 (Math|Rotator|MakeRotator (.roll _returnvalue_3) (.pitch _returnvalue_3) (- (.yaw _returnvalue_3) 9e+01)) false false))))

(fn ConstructionScript)

(fn SpawnPortal
  (params (Portal%20Visual :type Material%20Object%20Reference)))