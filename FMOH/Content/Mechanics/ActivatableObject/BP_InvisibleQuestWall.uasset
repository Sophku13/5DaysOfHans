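; BP_InvisibleQuestWall is an activatable barrier that blocks passage and explains why with a character monologue.
; OnActivation toggles IsActivated, switching the wall asset's collision off when activated and back on when deactivated.
; The first hit on the wall plays a 2D monologue sound and spawns a short-lived BP_InterMono at the player for the fear-of-the-dark subtitle, guarded by a DoOnce.
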(event OnComponentHit(WallAsset)
  (params (HitComponent :type Primitive%20Component%20Object%20Reference) (OtherActor :type Actor%20Object%20Reference) (OtherComp :type Primitive%20Component%20Object%20Reference) (NormalImpulse :type Vector :default "0, 0, 0") (Hit :type Hit%20Result%20Structure%20%28by%20ref%29))
  (Utilities|FlowControl|DoOnce false
    (:Completed
      (Audio|PlaySound2D "/Game/SoundSystem/Sounds/VoiceRecordings/InnerMonologue/SC_Monologue_04.SC_Monologue_04" 1.0 1.0 0.0 0 0)
      (bind _returnvalue (Game|SpawnActorfromClass "/Game/SoundSystem/Sounds/BP_InterMono.BP_InterMono_C" (Transformation|GetActorTransform (Game|GetPlayerCharacter 0)) "Undefined" "MultiplyWithRoot" 0 0 1.0 "It is too dark. The monster will get me." 2.0 true 0))
      (Default|CheckValues _returnvalue))))

(event EventBeginPlay
  (|CallParentFunction) ; This node is disabled and will not be called.\nDrag off pins to build functionality.
)

(event Collision|EventActorBeginOverlap
  (params (OtherActor :type Actor%20Object%20Reference))
  (|CallParentFunction OtherActor) ; This node is disabled and will not be called.\nDrag off pins to build functionality.
)

(event EventTick
  (params (DeltaSeconds :type Float%20%28single-precision%29))
  (|CallParentFunction DeltaSeconds) ; This node is disabled and will not be called.\nDrag off pins to build functionality.
)

(event EventOnActivation
  (params (PlayerRef :type BP%20Third%20Person%20Character%20Object%20Reference))
  (bind _wallasset (Variables|Default|GetWallAsset))
  (if (Variables|Default|GetbIsActivated)
    (Variables|Default|SetbIsActivated false)
    (Collision|SetCollisionEnabled _wallasset "QueryAndPhysics")
    (else
      (Variables|Default|SetbIsActivated true)
      (Collision|SetCollisionEnabled _wallasset "NoCollision"))))

(fn ConstructionScript
  (|CallParentFunction))