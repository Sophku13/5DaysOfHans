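; BP_ActivatableLamp is an activatable lamp actor whose spot light switches on and off.
; Each OnActivation event runs a FlipFlop that alternately shows and hides the SpotLight component, starting with show.
; Visibility changes do not propagate to child components, and the default BeginPlay, overlap and Tick events are disabled.
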(event EventBeginPlay
  (|CallParentFunction) ; This node is disabled and will not be called.\nDrag off pins to build functionality.
)

(event Collision|EventActorBeginOverlap
  (params (OtherActor :type Actor%20Object%20Reference))
  (|CallParentFunction OtherActor) ; This node is disabled and will not be called.\nDrag off pins to build functionality.
)

(event EventTick
  (params (DeltaSeconds :type Float%20%28single-precision%29))
  (|CallParentFunction DeltaSeconds) ; This node is disabled and will not be called.\nDrag off pins to build functionality.
)

(event EventOnActivation
  (params (PlayerRef :type BP%20Third%20Person%20Character%20Object%20Reference))
  (bind _spotlight (Variables|Default|GetSpotLight))
  (Utilities|FlowControl|FlipFlop
    (:A
      (Rendering|SetVisibility _spotlight true false))
    (:B
      (Rendering|SetVisibility _spotlight false false))))

(fn ConstructionScript
  (|CallParentFunction))