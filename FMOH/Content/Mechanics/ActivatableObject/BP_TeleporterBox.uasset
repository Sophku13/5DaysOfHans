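; BP_TeleporterBox is a one-shot teleporter trigger that moves the player character to a preset destination.
; Overlap on TeleportBox casts the other actor to BP_ThirdPersonCharacter and passes it to OnActivation.
; OnActivation sets the character's location and rotation from the Scene component's world transform, then sets WasActivated so later activations do nothing.
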(event OnComponentBeginOverlap(TeleportBox)
  (params (OverlappedComponent :type Primitive%20Component%20Object%20Reference) (OtherActor :type Actor%20Object%20Reference) (OtherComp :type Primitive%20Component%20Object%20Reference) (OtherBodyIndex :type Integer) (bFromSweep :type Boolean) (SweepResult :type Hit%20Result%20Structure%20%28by%20ref%29))
  (bind _asbp_third_person_character (Utilities|Casting|CastToBP_ThirdPersonCharacter OtherActor))
  (CallFunction|OnActivation _asbp_third_person_character))

(event EventBeginPlay
  (|CallParentFunction) ; This node is disabled and will not be called.\nDrag off pins to build functionality.
)

(event Collision|EventActorBeginOverlap
  (params (OtherActor :type Actor%20Object%20Reference))
  (|CallParentFunction OtherActor) ; This node is disabled and will not be called.\nDrag off pins to build functionality.
)

(event EventTick
  (params (DeltaSeconds :type Float%20%28single-precision%29))
  (|CallParentFunction DeltaSeconds) ; This node is disabled and will not be called.\nDrag off pins to build functionality.
)

(event EventOnActivation
  (params (PlayerRef :type BP%20Third%20Person%20Character%20Object%20Reference))
  (bind _scene (Variables|Default|GetScene))
  (bind _returnvalue (Transformation|GetWorldTransform _scene))
  (if (not (Variables|Default|GetbWasActivated))
    (Transformation|SetActorTransform PlayerRef (Math|Transform|MakeTransform (.location _returnvalue) (.rotation _returnvalue) "1.000000,1.000000,1.000000"))
    (Variables|Default|SetbWasActivated true)))

(fn ConstructionScript
  (|CallParentFunction))