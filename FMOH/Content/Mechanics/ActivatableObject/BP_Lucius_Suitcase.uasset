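; BP_Lucius_Suitcase is an activatable suitcase the player rotates open by holding the drag input while looking at it.
; A camera line trace on press confirms the target and locks the third-person camera until release.
; Tick applies the player's up/down rate to the pitch of its Anchor and LuciusRef's Anchor in tandem.
; Passing the upper limit snaps both to 90 degrees, stops further dragging and triggers LuciusRef's interaction.
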(event Input|EnhancedActionEvents|EnhancedInputActionIA_DragObjects
  (params (ActionValue :type Boolean) (ElapsedSeconds :type Float%20%28double-precision%29) (TriggeredSeconds :type Float%20%28double-precision%29) (InputAction :type Input%20Action%20Object%20Reference :default "/Game/Character/Input/Actions/IA_DragObjects.IA_DragObjects"))
  ;[1 1 1] Comment
  ;;[1 1 1] Comment
  (:Started
    (Variables|Default|SetbIsHoldingLMB true)
    (bind _asbp_third_person_character (Utilities|Casting|CastToBP_ThirdPersonCharacter (Game|GetPlayerCharacter 0)))
    (Variables|Default|SetPlayerRef _asbp_third_person_character)
    (bind (_outhit _returnvalue) (Collision|LineTraceForObjects (Transformation|GetWorldLocation (Variables|/Game/ThirdPerson/Blueprints/BP_ThirdPersonCharacter.BP_ThirdPersonCharacter_C|GetFollowCamera _asbp_third_person_character)) (+ (Transformation|GetWorldLocation (Variables|/Game/ThirdPerson/Blueprints/BP_ThirdPersonCharacter.BP_ThirdPersonCharacter_C|GetFollowCamera _asbp_third_person_character)) (* (Math|Vector|GetForwardVector (Variables|/Game/ThirdPerson/Blueprints/BP_ThirdPersonCharacter.BP_ThirdPersonCharacter_C|GetFollowCamera _asbp_third_person_character)) 5e+02)) (Utilities|Array|MakeArray "ObjectTypeQuery1") false 0 "None" false))
    (if _returnvalue
      (bind _asbp_lucius_suitcase (Utilities|Casting|CastToBP_Lucius_Suitcase (.HitActor (Collision|BreakHitResult _outhit)))
        (:then
          (if (== _asbp_lucius_suitcase self)
            (Variables|Default|SetbLookingAtSuitcase true)
            (Variables|/Game/ThirdPerson/Blueprints/BP_ThirdPersonCharacter.BP_ThirdPersonCharacter_C|SetbIsCameraLocked _asbp_third_person_character true)
            (else
              (Variables|Default|SetbLookingAtSuitcase false :!label _label))))
        (:CastFailed
          (goto _label)))
      (else
        (goto _label))))
  (:Canceled
    (Variables|Default|SetbIsHoldingLMB false :!label _label_2)
    (if (Variables|Default|GetbLookingAtSuitcase)
      (Variables|/Game/ThirdPerson/Blueprints/BP_ThirdPersonCharacter.BP_ThirdPersonCharacter_C|SetbIsCameraLocked _asbp_third_person_character false)))
  (:Completed
    (goto _label_2)))

(event EventBeginPlay
  ;[1 1 1] Comment
  (|CallParentFunction)
  (Input|EnableInput (Game|GetPlayerController 0)))

(event Collision|EventActorBeginOverlap
  (params (OtherActor :type Actor%20Object%20Reference))
  (|CallParentFunction OtherActor) ; This node is disabled and will not be called.\nDrag off pins to build functionality.
)

(event EventOnActivation
  (params (PlayerRef :type BP%20Third%20Person%20Character%20Object%20Reference))
  (bind _luciusref (Variables|Default|GetLuciusRef))
  (Variables|Default|SetbIsLockPositionReached true)
  (Variables|/Game/Mechanics/MiniGames/LuciusMiniGame/BP_LuciusMiniGame.BP_LuciusMiniGame_C|SetbIsInPosition _luciusref true)
  (Default|OnInteract _luciusref PlayerRef))

(event EventTick
  (params (DeltaSeconds :type Float%20%28single-precision%29))
  (bind _anchor (Variables|Default|GetAnchor))
  (bind _relativerotation (Variables|/Script/Engine.SceneComponent|GetRelativeRotation _anchor))
  ;[1 1 1] Comment
  ;;[1 1 1] Comment
  (if (not (Variables|Default|GetbIsLockPositionReached))
    (if (Variables|Default|GetbIsHoldingLMB)
      (if (Variables|Default|GetbLookingAtSuitcase)
        (if (Math|Float|NearlyEqual(Float) (.pitch _relativerotation) (Math|Float|ClampAngle (.pitch _relativerotation) 0.0 85.0) 0.001)
          (Transformation|AddLocalRotation _anchor (Math|Rotator|MakeRotator 0.0 (* (Variables|/Game/ThirdPerson/Blueprints/BP_ThirdPersonCharacter.BP_ThirdPersonCharacter_C|GetUpDownRate (stale Input|EnhancedActionEvents|EnhancedInputActionIA_DragObjects _asbp_third_person_character)) (Variables|Default|GetSensitivity)) 0.0) false false)
          (Transformation|AddLocalRotation (Variables|/Game/Mechanics/MiniGames/LuciusMiniGame/BP_LuciusMiniGame.BP_LuciusMiniGame_C|GetAnchor (Variables|Default|GetLuciusRef)) (Math|Rotator|MakeRotator 0.0 (* (Variables|/Game/ThirdPerson/Blueprints/BP_ThirdPersonCharacter.BP_ThirdPersonCharacter_C|GetUpDownRate (stale Input|EnhancedActionEvents|EnhancedInputActionIA_DragObjects _asbp_third_person_character)) (Variables|Default|GetSensitivity)) 0.0) false false)
          (elif (< (.pitch _relativerotation) 0.0)
            (Transformation|SetRelativeRotation _anchor "0.000000,0.000000,0.000000" false false)
            (Transformation|SetRelativeRotation (Variables|/Game/Mechanics/MiniGames/LuciusMiniGame/BP_LuciusMiniGame.BP_LuciusMiniGame_C|GetAnchor (Variables|Default|GetLuciusRef)) "0, 0, 0" false false)
            (else
              (Transformation|SetRelativeRotation _anchor "90.000000,0.000000,0.000000" false false)
              (Transformation|SetRelativeRotation (Variables|/Game/Mechanics/MiniGames/LuciusMiniGame/BP_LuciusMiniGame.BP_LuciusMiniGame_C|GetAnchor (Variables|Default|GetLuciusRef)) "90.000000,0.000000,0.000000" false false)
              (CallFunction|OnActivation (Variables|Default|GetPlayerRef)))))))))

(fn ConstructionScript
  (|CallParentFunction))