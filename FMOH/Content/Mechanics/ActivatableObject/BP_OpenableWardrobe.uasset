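; Activatable wardrobe whose two doors the player drags open and shut, once OnActivation has unlocked it.
; Pressing the drag input traces from the follow camera, picks the left or right door by component tag and locks the character's camera until release.
; While held, Tick rotates that door by the character's TurnRate times Sensitivity, snapping it back inside its swing limits.
; The trace checks only tags, not which wardrobe was hit.
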(event Input|EnhancedActionEvents|EnhancedInputActionIA_DragObjects
  (params (ActionValue :type Boolean) (ElapsedSeconds :type Float%20%28double-precision%29) (TriggeredSeconds :type Float%20%28double-precision%29) (InputAction :type Input%20Action%20Object%20Reference :default "/Game/Character/Input/Actions/IA_DragObjects.IA_DragObjects"))
  ;[1 1 1] Comment
  ;;[1 1 1] Comment
  (:Started
    (Variables|Default|SetbIsHoldingLMB true)
    (bind _asbp_third_person_character (Utilities|Casting|CastToBP_ThirdPersonCharacter (Game|GetPlayerCharacter 0)))
    (bind (_outhit _returnvalue) (Collision|LineTraceForObjects (Transformation|GetWorldLocation (Variables|/Game/ThirdPerson/Blueprints/BP_ThirdPersonCharacter.BP_ThirdPersonCharacter_C|GetFollowCamera _asbp_third_person_character)) (+ (Transformation|GetWorldLocation (Variables|/Game/ThirdPerson/Blueprints/BP_ThirdPersonCharacter.BP_ThirdPersonCharacter_C|GetFollowCamera _asbp_third_person_character)) (* (Math|Vector|GetForwardVector (Variables|/Game/ThirdPerson/Blueprints/BP_ThirdPersonCharacter.BP_ThirdPersonCharacter_C|GetFollowCamera _asbp_third_person_character)) 5e+02)) (Utilities|Array|MakeArray "ObjectTypeQuery1") false 0 "None" false))
    (if _returnvalue
      (if (== (Utilities|Array|Get(acopy) (Variables|/Script/Engine.ActorComponent|GetComponentTags (.HitComponent (Collision|BreakHitResult _outhit)))) "Right")
        (Variables|Default|SetbLookingAtRight true)
        (Variables|Default|SetbLookingAtLeft false)
        (Variables|/Game/ThirdPerson/Blueprints/BP_ThirdPersonCharacter.BP_ThirdPersonCharacter_C|SetbIsCameraLocked _asbp_third_person_character true :!label _label)
        (elif (== (Utilities|Array|Get(acopy) (Variables|/Script/Engine.ActorComponent|GetComponentTags (.HitComponent (Collision|BreakHitResult _outhit)))) "Left")
          (Variables|Default|SetbLookingAtLeft true)
          (Variables|Default|SetbLookingAtRight false)
          (goto _label)))
      (else
        (Variables|Default|SetbLookingAtRight false)
        (Variables|Default|SetbLookingAtLeft false))))
  (:Canceled
    (Variables|Default|SetbIsHoldingLMB false :!label _label_2)
    (if (or (Variables|Default|GetbLookingAtLeft) (Variables|Default|GetbLookingAtRight))
      (Variables|/Game/ThirdPerson/Blueprints/BP_ThirdPersonCharacter.BP_ThirdPersonCharacter_C|SetbIsCameraLocked _asbp_third_person_character false)))
  (:Completed
    (goto _label_2)))

(event EventBeginPlay
  ;[1 1 1] Comment
  (|CallParentFunction)
  (Input|EnableInput (Game|GetPlayerController 0)))

(event Collision|EventActorBeginOverlap
  (params (OtherActor :type Actor%20Object%20Reference))
  (|CallParentFunction OtherActor) ; This node is disabled and will not be called.\nDrag off pins to build functionality.
)

(event EventOnActivation
  (params (PlayerRef :type BP%20Third%20Person%20Character%20Object%20Reference))
  ;[1 1 1] Comment
  (Variables|Default|SetbCanBeOpened true))

(event EventTick
  (params (DeltaSeconds :type Float%20%28single-precision%29))
  (bind _closet_dr (Variables|Default|Getcloset_DR))
  (bind _closet_dl (Variables|Default|Getcloset_DL))
  (bind _relativerotation (Variables|/Script/Engine.SceneComponent|GetRelativeRotation _closet_dl))
  (bind _relativerotation_2 (Variables|/Script/Engine.SceneComponent|GetRelativeRotation _closet_dr))
  ;[1 1 1] Comment
  ;;[1 1 1] Comment
  (if (Variables|Default|GetbCanBeOpened)
    (if (Variables|Default|GetbIsHoldingLMB)
      (if (Variables|Default|GetbLookingAtLeft)
        (if (Math|Float|NearlyEqual(Float) (.yaw _relativerotation) (Math|Float|ClampAngle (.yaw _relativerotation) 0.0 1.2e+02) 0.001)
          (Transformation|AddLocalRotation _closet_dl (Math|Rotator|MakeRotator 0.0 0.0 (* (Variables|/Game/ThirdPerson/Blueprints/BP_ThirdPersonCharacter.BP_ThirdPersonCharacter_C|GetTurnRate (stale Input|EnhancedActionEvents|EnhancedInputActionIA_DragObjects _asbp_third_person_character)) (Variables|Default|GetSensitivity))) false false)
          (elif (< (.yaw _relativerotation) 0.0)
            (Transformation|SetRelativeRotation _closet_dl "0.000000,0.500000,0.000000" false false)
            (else
              (Transformation|SetRelativeRotation _closet_dl "0.000000,119.000000,0.000000" false false))))
        (elif (Variables|Default|GetbLookingAtRight)
          (if (Math|Float|NearlyEqual(Float) (.yaw _relativerotation_2) (Math|Float|ClampAngle (.yaw _relativerotation_2) -1.2e+02 0.0) 0.001)
            (Transformation|AddLocalRotation _closet_dr (Math|Rotator|MakeRotator 0.0 0.0 (* (Variables|/Game/ThirdPerson/Blueprints/BP_ThirdPersonCharacter.BP_ThirdPersonCharacter_C|GetTurnRate (stale Input|EnhancedActionEvents|EnhancedInputActionIA_DragObjects _asbp_third_person_character)) (Variables|Default|GetSensitivity))) false false)
            (elif (> (.yaw _relativerotation_2) 0.0)
              (Transformation|SetRelativeRotation _closet_dr "0.000000,-0.500000,0.000000" false false)
              (else
                (Transformation|SetRelativeRotation _closet_dr "0.000000,-119.000000,0.000000" false false)))))))))

(fn ConstructionScript
  (|CallParentFunction))