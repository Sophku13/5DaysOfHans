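; Listener actor that unlocks a door once every tracked breakable glass and plate is broken.
; Tick polls the broken state of both lists, and the activation event triggers the locked door's activation and interaction behind a one-shot flag.
; A separate ObjectBroken event increments and prints a counter, then tells the parents' arguing sound actors to stop shouting.
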(event Custom|Event%20Object%20Broken
  (bind _stopshoutingcounter (Variables|Default|GetStopShoutingCounter))
  (Math|Integer|IncrementInt _stopshoutingcounter
    (:%20%20
      (Development|PrintString (Utilities|String|ToString(Integer) _stopshoutingcounter))
      (bind _outactors (Actor|GetAllActorsOfClass "/Game/SoundSystem/Sounds/VoiceRecordings/Parents/BP_ParentsArguingSound.BP_ParentsArguingSound_C"))
      (Default|EventStopShouting _outactors))))

(event EventBeginPlay
  (|CallParentFunction) ; This node is disabled and will not be called.\nDrag off pins to build functionality.
)

(event Collision|EventActorBeginOverlap
  (params (OtherActor :type Actor%20Object%20Reference))
  (|CallParentFunction OtherActor) ; This node is disabled and will not be called.\nDrag off pins to build functionality.
)

(event EventTick
  (params (DeltaSeconds :type Float%20%28single-precision%29))
  (|CallParentFunction DeltaSeconds)
  (Variables|Default|SetbAllTargetsBroken true)
  (for _array_element (Variables|Default|GetGlassList)
    (if (not (and (Variables|Default|GetbAllTargetsBroken) (Variables|/Game/Assets/Fracture/BP_BreakableGlass.BP_BreakableGlass_C|GetbIsBroken _array_element)))
      (Variables|Default|SetbAllTargetsBroken false)))
  (for _array_element_2 (Variables|Default|GetPlateList)
    (if (not (and (Variables|Default|GetbAllTargetsBroken) (Variables|/Game/Assets/Fracture/BP_BreakablePlate.BP_BreakablePlate_C|GetbIsBroken _array_element_2)))
      (Variables|Default|SetbAllTargetsBroken false)))
  (if (Variables|Default|GetbAllTargetsBroken)
    (CallFunction|OnActivation)))

(event EventOnActivation
  (params (PlayerRef :type BP%20Third%20Person%20Character%20Object%20Reference))
  (bind _lockeddoor (Variables|Default|GetLockedDoor))
  (if (not (Variables|Default|GetbhasActivated))
    (Default|OnActivation _lockeddoor)
    (Default|OnInteract _lockeddoor PlayerRef)
    (Variables|Default|SetbhasActivated true)))

(fn ConstructionScript
  (|CallParentFunction))