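; Lockable drawer that the player can drag open and shut once OnActivation sets CanBeOpened.
; Holding the drag input line-traces from the character's follow camera and, on hitting this drawer, locks the camera.
; Tick then slides DrawerMesh and a linked MovingActor along local Y by the character's UpDownRate times Sensitivity, snapping back inside fixed limits when overshot.
; The mesh comes from DrawerAsset, applied in the construction script and BeginPlay.
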(event Input|EnhancedActionEvents|EnhancedInputActionIA_DragObjects
  (params (ActionValue :type Boolean) (ElapsedSeconds :type Float%20%28double-precision%29) (TriggeredSeconds :type Float%20%28double-precision%29) (InputAction :type Input%20Action%20Object%20Reference :default "/Game/Character/Input/Actions/IA_DragObjects.IA_DragObjects"))
  ;[1 1 1] Comment
  ;;[1 1 1] Comment
  (:Started
    (Variables|Default|SetbIsHoldingLMB true)
    (bind _asbp_third_person_character (Utilities|Casting|CastToBP_ThirdPersonCharacter (Game|GetPlayerCharacter 0)))
    (bind (_outhit _returnvalue) (Collision|LineTraceForObjects (Transformation|GetWorldLocation (Variables|/Game/ThirdPerson/Blueprints/BP_ThirdPersonCharacter.BP_ThirdPersonCharacter_C|GetFollowCamera _asbp_third_person_character)) (+ (Transformation|GetWorldLocation (Variables|/Game/ThirdPerson/Blueprints/BP_ThirdPersonCharacter.BP_ThirdPersonCharacter_C|GetFollowCamera _asbp_third_person_character)) (* (Math|Vector|GetForwardVector (Variables|/Game/ThirdPerson/Blueprints/BP_ThirdPersonCharacter.BP_ThirdPersonCharacter_C|GetFollowCamera _asbp_third_person_character)) 5e+02)) (Utilities|Array|MakeArray "ObjectTypeQuery1") false 0 "None" false))
    (if _returnvalue
      (bind _asbp_drawer_lockable (Utilities|Casting|CastToBP_DrawerLockable (.HitActor (Collision|BreakHitResult _outhit))))
      (if (== _asbp_drawer_lockable self)
        (Variables|Default|SetbLookingAtDrawer true)
        (Variables|/Game/ThirdPerson/Blueprints/BP_ThirdPersonCharacter.BP_ThirdPersonCharacter_C|SetbIsCameraLocked _asbp_third_person_character true)
        (else
          (Variables|Default|SetbLookingAtDrawer false :!label _label)))
      (else
        (goto _label))))
  (:Canceled
    (Variables|Default|SetbIsHoldingLMB false :!label _label_2)
    (if (Variables|Default|GetbLookingAtDrawer)
      (Variables|/Game/ThirdPerson/Blueprints/BP_ThirdPersonCharacter.BP_ThirdPersonCharacter_C|SetbIsCameraLocked _asbp_third_person_character false)))
  (:Completed
    (goto _label_2)))

(event EventBeginPlay
  ;[1 1 1] Comment
  (|CallParentFunction)
  (Components|StaticMesh|SetStaticMesh (Variables|Default|GetDrawerMesh) (Variables|Default|GetDrawerAsset))
  (Input|EnableInput (Game|GetPlayerController 0)))

(event Collision|EventActorBeginOverlap
  (params (OtherActor :type Actor%20Object%20Reference))
  (|CallParentFunction OtherActor) ; This node is disabled and will not be called.\nDrag off pins to build functionality.
)

(event EventOnActivation
  (params (PlayerRef :type BP%20Third%20Person%20Character%20Object%20Reference))
  (Variables|Default|SetbCanBeOpened true))

(event EventTick
  (params (DeltaSeconds :type Float%20%28single-precision%29))
  (bind _movingactor (Variables|Default|GetMovingActor))
  (bind _drawermesh (Variables|Default|GetDrawerMesh))
  (bind _relativelocation (Variables|/Script/Engine.SceneComponent|GetRelativeLocation _drawermesh))
  ;[1 1 1] Comment
  ;;[1 1 1] Comment
  (if (Variables|Default|GetbCanBeOpened)
    (if (Variables|Default|GetbIsHoldingLMB)
      (if (Variables|Default|GetbLookingAtDrawer)
        (if (Math|Float|NearlyEqual(Float) (.y _relativelocation) (Math|Float|ClampAngle (.y _relativelocation) -5e+01 2.0) 0.001)
          (Transformation|AddLocalOffset _drawermesh (Math|Vector|MakeVector 0.0 (* (Variables|/Game/ThirdPerson/Blueprints/BP_ThirdPersonCharacter.BP_ThirdPersonCharacter_C|GetUpDownRate (stale Input|EnhancedActionEvents|EnhancedInputActionIA_DragObjects _asbp_third_person_character)) (Variables|Default|GetSensitivity)) 0.0) false false)
          (Transformation|AddActorLocalOffset _movingactor (Math|Vector|MakeVector 0.0 (* (Variables|/Game/ThirdPerson/Blueprints/BP_ThirdPersonCharacter.BP_ThirdPersonCharacter_C|GetUpDownRate (stale Input|EnhancedActionEvents|EnhancedInputActionIA_DragObjects _asbp_third_person_character)) (Variables|Default|GetSensitivity)) 0.0) false false)
          (elif (< (.y _relativelocation) -5e+01)
            (Transformation|SetRelativeLocation _drawermesh "0.000000,-49.000000,0.000000" false false)
            (Transformation|SetActorRelativeLocation _movingactor "0.000000,-49.000000,0.000000")
            (else
              (Transformation|SetRelativeLocation _drawermesh "0, 0, 0" false false)
              (Transformation|SetActorRelativeLocation _movingactor))))))))

(fn ConstructionScript
  (|CallParentFunction)
  (Components|StaticMesh|SetStaticMesh (Variables|Default|GetDrawerMesh) (Variables|Default|GetDrawerAsset)))