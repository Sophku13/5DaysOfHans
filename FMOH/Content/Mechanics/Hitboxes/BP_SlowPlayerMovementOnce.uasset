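; One-shot trigger volume that slows BP_ThirdPersonCharacter while inside SlowBox and applies a cinematic camera effect.
; Entering lowers walk speed and plays a Timeline that lerps the first-person camera's post-process settings and widens its aspect ratio.
; Leaving sets walk speed to a fixed standard value, reverses the Timeline and disables the box's collision.
; OnReset re-enables the collision so the slowdown can trigger again.
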(event OnComponentBeginOverlap(SlowBox)
  (params (OverlappedComponent :type Primitive%20Component%20Object%20Reference) (OtherActor :type Actor%20Object%20Reference) (OtherComp :type Primitive%20Component%20Object%20Reference) (OtherBodyIndex :type Integer) (bFromSweep :type Boolean) (SweepResult :type Hit%20Result%20Structure%20%28by%20ref%29))
  ;[0 1 0.6176] Slows the Playerdown when they are in the hitbox
  (bind _asbp_third_person_character (Utilities|Casting|CastToBP_ThirdPersonCharacter OtherActor))
  (Variables|/Script/Engine.CharacterMovementComponent|SetMaxWalkSpeed (Variables|/Script/Engine.Character|GetCharacterMovement _asbp_third_person_character) 75.0)
  (bind _newtrack_0 (Timeline|Timeline PlayFromStart)
    (:Update
      (Variables|/Script/Engine.CameraComponent|SetPostProcessSettings (Variables|/Game/ThirdPerson/Blueprints/BP_ThirdPersonCharacter.BP_ThirdPersonCharacter_C|GetFirstPersonCameraREF _asbp_third_person_character) (Utilities|Struct|MakePostProcessSettings (Math|Float|Lerp 1.0 0.3 _newtrack_0)))
      (Class|CameraComponent|SetAspectRatio (Variables|/Game/ThirdPerson/Blueprints/BP_ThirdPersonCharacter.BP_ThirdPersonCharacter_C|GetFirstPersonCameraREF _asbp_third_person_character) (Math|Float|Lerp 1.777778 2.35 _newtrack_0)))))

(event OnComponentEndOverlap(SlowBox)
  (params (OverlappedComponent :type Primitive%20Component%20Object%20Reference) (OtherActor :type Actor%20Object%20Reference) (OtherComp :type Primitive%20Component%20Object%20Reference) (OtherBodyIndex :type Integer))
  ;[0 1 0.6176] Go back to standard
  (bind _asbp_third_person_character (Utilities|Casting|CastToBP_ThirdPersonCharacter OtherActor))
  (Variables|/Script/Engine.CharacterMovementComponent|SetMaxWalkSpeed (Variables|/Script/Engine.Character|GetCharacterMovement _asbp_third_person_character) 1.5e+02)
  (Collision|SetCollisionEnabled (Variables|Default|GetSlowBox) "NoCollision")
  (bind _newtrack_0 (Timeline|Timeline Reverse)
    (:Update
      (Variables|/Script/Engine.CameraComponent|SetPostProcessSettings (Variables|/Game/ThirdPerson/Blueprints/BP_ThirdPersonCharacter.BP_ThirdPersonCharacter_C|GetFirstPersonCameraREF (stale OnComponentBeginOverlap(SlowBox) _asbp_third_person_character)) (Utilities|Struct|MakePostProcessSettings (Math|Float|Lerp 1.0 0.3 _newtrack_0)))
      (Class|CameraComponent|SetAspectRatio (Variables|/Game/ThirdPerson/Blueprints/BP_ThirdPersonCharacter.BP_ThirdPersonCharacter_C|GetFirstPersonCameraREF (stale OnComponentBeginOverlap(SlowBox) _asbp_third_person_character)) (Math|Float|Lerp 1.777778 2.35 _newtrack_0)))))

(event EventBeginPlay)

(event Collision|EventActorBeginOverlap
  (params (OtherActor :type Actor%20Object%20Reference)))

(event EventTick
  (params (DeltaSeconds :type Float%20%28single-precision%29)))

(event EventOnReset
  (Collision|SetCollisionEnabled (Variables|Default|GetSlowBox) "QueryOnly"))

(fn ConstructionScript)