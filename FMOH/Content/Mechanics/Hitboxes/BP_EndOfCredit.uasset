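; BP_EndOfCredit is a trigger that returns the game to the main menu, apparently once the credits end.
; Overlapping CreditEndHitBox sets the character to flying, loads the main menu streamed level with blocking, clears all widgets and fades in the character's menu control.
; It then switches the view to the title camera, shows the menu widget and title background with UI-only input, and flags the character as in the "Book" minigame.
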(event OnComponentBeginOverlap(CreditEndHitBox)
  (params (OverlappedComponent :type Primitive%20Component%20Object%20Reference) (OtherActor :type Actor%20Object%20Reference) (OtherComp :type Primitive%20Component%20Object%20Reference) (OtherBodyIndex :type Integer) (bFromSweep :type Boolean) (SweepResult :type Hit%20Result%20Structure%20%28by%20ref%29))
  (bind _returnvalue (Game|GetPlayerController 0))
  (bind _returnvalue_2 (Actor|GetActorOfClass "/Game/ThirdPerson/Blueprints/BP_ThirdPersonCharacter.BP_ThirdPersonCharacter_C"))
  (Pawn|Components|CharacterMovement|SetMovementMode (Variables|/Script/Engine.Character|GetCharacterMovement _returnvalue_2) "MOVE_Flying" 0)
  (Class|GameplayStatics|LoadStreamLevelbySoftObjectPtr "/Game/Maps/FMOH_MainMenu.FMOH_MainMenu" true true)
  (Viewport|RemoveAllWidgets)
  (Default|Fadein (Variables|/Game/ThirdPerson/Blueprints/BP_ThirdPersonCharacter.BP_ThirdPersonCharacter_C|GetMenuControlRef _returnvalue_2))
  (bind _returnvalue_3 (Actor|GetActorOfClass "/Game/UI/MainMenu/BP_MainMenuTitleCamera.BP_MainMenuTitleCamera_C"))
  (Game|Player|SetViewTargetwithBlend _returnvalue _returnvalue_3 0.0 "VTBlend_Linear" 0.0 false)
  (bind _returnvalue_4 (UserInterface|CreateWidget "/Game/UI/WBP_MainMenu.WBP_MainMenu_C"))
  (UserInterface|Viewport|AddtoViewport _returnvalue_4 1)
  (Input|SetInputModeUIOnly _returnvalue 0 "DoNotLock" false)
  (bind _returnvalue_5 (Actor|GetActorOfClass "/Game/UI/MainMenu/BP_TitleScreenBG.BP_TitleScreenBG_C"))
  (Rendering|SetVisibility (Variables|/Game/UI/MainMenu/BP_TitleScreenBG.BP_TitleScreenBG_C|Gettitle _returnvalue_5) true false)
  (Variables|/Game/UI/MainMenu/BP_TitleScreenBG.BP_TitleScreenBG_C|SetShowTitle _returnvalue_5 true)
  (Default|Fadein _returnvalue_5)
  (Variables|/Script/Engine.PlayerController|SetbShowMouseCursor _returnvalue true)
  (Variables|/Game/ThirdPerson/Blueprints/BP_ThirdPersonCharacter.BP_ThirdPersonCharacter_C|SetbIsInMinigame _returnvalue_2 true)
  (Variables|/Game/ThirdPerson/Blueprints/BP_ThirdPersonCharacter.BP_ThirdPersonCharacter_C|SetActiveMinigameName _returnvalue_2 "Book"))

(fn ConstructionScript)