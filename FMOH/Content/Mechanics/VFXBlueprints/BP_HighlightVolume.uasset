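; BP_HighlightVolume is a trigger volume that switches custom-depth rendering, used for highlighting, on and off for a list of HighlightedObjects.
; Beginning or ending an overlap with LoadBox enables custom depth, while beginning an overlap with UnloadBox disables it.
; Each object supplies the components to toggle through a CreateListOfComponents interface message, with no filtering of the overlapping actor.
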(event OnComponentBeginOverlap(LoadBox)
  (params (OverlappedComponent :type Primitive%20Component%20Object%20Reference) (OtherActor :type Actor%20Object%20Reference) (OtherComp :type Primitive%20Component%20Object%20Reference) (OtherBodyIndex :type Integer) (bFromSweep :type Boolean) (SweepResult :type Hit%20Result%20Structure%20%28by%20ref%29))
  (for _array_element (Variables|Default|GetHighlightedObjects)
    (bind _staticmesharray (Class|BPIHighlight|CreateListOfComponents(Message) _array_element))
    (for _array_element_2 _staticmesharray
      (Rendering|SetRenderCustomDepth _array_element_2 true))))

(event OnComponentBeginOverlap(UnloadBox)
  (params (OverlappedComponent :type Primitive%20Component%20Object%20Reference) (OtherActor :type Actor%20Object%20Reference) (OtherComp :type Primitive%20Component%20Object%20Reference) (OtherBodyIndex :type Integer) (bFromSweep :type Boolean) (SweepResult :type Hit%20Result%20Structure%20%28by%20ref%29))
  (for _array_element (Variables|Default|GetHighlightedObjects)
    (bind _staticmesharray (Class|BPIHighlight|CreateListOfComponents(Message) _array_element))
    (for _array_element_2 _staticmesharray
      (Rendering|SetRenderCustomDepth _array_element_2 false))))

(event OnComponentEndOverlap(LoadBox)
  (params (OverlappedComponent :type Primitive%20Component%20Object%20Reference) (OtherActor :type Actor%20Object%20Reference) (OtherComp :type Primitive%20Component%20Object%20Reference) (OtherBodyIndex :type Integer))
  (for _array_element (Variables|Default|GetHighlightedObjects)
    (bind _staticmesharray (Class|BPIHighlight|CreateListOfComponents(Message) _array_element))
    (for _array_element_2 _staticmesharray
      (Rendering|SetRenderCustomDepth _array_element_2 true))))

(fn ConstructionScript)