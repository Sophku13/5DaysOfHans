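; Fire VFX actor that plays the NSFire Niagara effect as soon as the game begins.
; It enables input from the first player controller, and releasing E unpauses the effect.
; Nodes for pausing, delayed simulation stepping and time dilation are disconnected leftovers from experiments, so nothing in this graph pauses the fire.
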(event EventBeginPlay
  (Input|EnableInput (Game|GetPlayerController 0))
  (Components|Activation|Activate (Variables|Default|GetNS_Fire) false))

(event EventTick
  (params (DeltaSeconds :type Float%20%28single-precision%29))
  ;[0.02624 0.001821 0.162] Played around with time dilation, feel free to ignore
)

(event Input|KeyboardEvents|E
  (params (Key :type Key%20Structure :default "None"))
  ;[0.02624 0.001821 0.162] Played around with time dilation, feel free to ignore
  (:Released
    (Class|NiagaraComponent|SetPaused (Variables|Default|GetNS_Fire) false)))

(fn ConstructionScript)