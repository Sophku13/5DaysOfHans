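; BP_MonologChain is a one-shot trigger box that plays a timed chain of monologue lines with subtitles.
; On overlap it spawns the first BP_InterMono at the overlapping actor, passing sound and subtitle data from the MonoChain map, then disables collision.
; LoadNext re-calls itself after each DelayAfter, spawning later lines at the player.
; The first wait reads the next entry's DelayAfter because ChainPosition increments beforehand.
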(event OnComponentBeginOverlap(Box)
  (params (OverlappedComponent :type Primitive%20Component%20Object%20Reference) (OtherActor :type Actor%20Object%20Reference) (OtherComp :type Primitive%20Component%20Object%20Reference) (OtherBodyIndex :type Integer) (bFromSweep :type Boolean) (SweepResult :type Hit%20Result%20Structure%20%28by%20ref%29))
  (bind _monochain (Variables|Default|GetMonoChain))
  (bind _chainposition (Variables|Default|GetchainPosition))
  (bind _value (Utilities|Map|Find _monochain _chainposition))
  (bind _returnvalue (Game|SpawnActorfromClass "/Game/SoundSystem/Sounds/BP_InterMono.BP_InterMono_C" (Transformation|GetActorTransform OtherActor) "Undefined" "MultiplyWithRoot" 0 (.sound _value) (.volumemultiplier _value) (.subtitletext _value) (.lifetime _value) true 0))
  (Default|CheckValues _returnvalue)
  (Math|Integer|IncrementInt (Variables|Default|GetchainPosition)
    (:%20%20
      (Collision|SetCollisionEnabled (Variables|Default|GetBox) "NoCollision")
      (Utilities|FlowControl|Delay (.delayafter _value))
      (CallFunction|LoadNext))))

(event Custom|LoadNext
  (bind _monochain (Variables|Default|GetMonoChain))
  (bind _chainposition (Variables|Default|GetchainPosition))
  (bind _value (Utilities|Map|Find _monochain _chainposition))
  (if (<= _chainposition (Utilities|Map|Length (Variables|Default|GetMonoChain)))
    (bind _returnvalue (Game|SpawnActorfromClass "/Game/SoundSystem/Sounds/BP_InterMono.BP_InterMono_C" (Transformation|GetActorTransform (Game|GetPlayerCharacter 0)) "Undefined" "MultiplyWithRoot" 0 (.sound _value) (.volumemultiplier _value) (.subtitletext _value) (.lifetime _value) true 0))
    (Default|CheckValues _returnvalue)
    (Utilities|FlowControl|Delay (.delayafter _value))
    (Math|Integer|IncrementInt (Variables|Default|GetchainPosition)
      (:%20%20
        (CallFunction|LoadNext)))))

(event EventBeginPlay)

(event Collision|EventActorBeginOverlap
  (params (OtherActor :type Actor%20Object%20Reference)))

(event EventTick
  (params (DeltaSeconds :type Float%20%28single-precision%29)))

(fn ConstructionScript)