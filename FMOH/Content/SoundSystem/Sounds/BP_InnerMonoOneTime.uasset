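; BP_InnerMonoOneTime is a one-shot inner monologue actor, triggered by a box overlap or by SpawnWithValues.
; Both paths disable box collision and run CheckValues, which plays any valid sound in 2D, treating zero volume as full.
; It creates the WBP_Subtitles widget when SubtitleText is empty, as the check is wired.
; After LifeTime, or one second if that is near zero, it removes the widget and destroys itself.
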(event OnComponentBeginOverlap(Box)
  (params (OverlappedComponent :type Primitive%20Component%20Object%20Reference) (OtherActor :type Actor%20Object%20Reference) (OtherComp :type Primitive%20Component%20Object%20Reference) (OtherBodyIndex :type Integer) (bFromSweep :type Boolean) (SweepResult :type Hit%20Result%20Structure%20%28by%20ref%29))
  ;[0 1 0.515] Player Overlap in Level
  (CallFunction|CheckValues)
  (Collision|SetCollisionEnabled (Variables|Default|GetBox) "NoCollision"))

(event Custom|SpawnWithValues
  (params (Sound :type Sound%20Base%20Object%20Reference) (Volume%20Multiplier :type Float%20%28single-precision%29) (SubtitleText :type Text) (LifeTime :type Float%20%28double-precision%29))
  ;[0 1 0.596] Access through Blueprints
  (Variables|Default|SetSound Sound)
  (Variables|Default|SetVolume%20Multiplier Volume%20Multiplier)
  (Variables|Default|SetSubtitleText SubtitleText)
  (Variables|Default|SetLifeTime LifeTime)
  (Collision|SetCollisionEnabled (Variables|Default|GetBox) "NoCollision")
  (CallFunction|CheckValues))

(event Custom|CheckValues
  ;[0 1 0.5631] Automatically Checking which values are set and starts operations accordingly
  (Variables|Default|GetSound
    (:then
      (if (Math|Float|NearlyEqual(Float) (Variables|Default|GetVolume%20Multiplier) 0.0 0.001)
        (Variables|Default|SetVolume%20Multiplier 1.0)
        (CallFunction|PlayInnerMonologue)
        (else
          (CallFunction|PlayInnerMonologue))))
    (:else
      _))
  (if (Utilities|Text|TextIsEmpty (Variables|Default|GetSubtitleText))
    (CallFunction|DisplaySubtitles))
  (if (Math|Float|NearlyEqual(Float) (Variables|Default|GetLifeTime) 0.0 1.0)
    (Utilities|FlowControl|Delay 1.0)
    (else
      (Utilities|FlowControl|Delay (Variables|Default|GetLifeTime))))
  (CallFunction|CleanUp))

(event Custom|PlayInnerMonologue
  ;[0 1 0.566] Spawns InnerMonolog Sound
  (Audio|SpawnSound2D (Variables|Default|GetSound) (Variables|Default|GetVolume%20Multiplier) 1.0 0.0 0))

(event Custom|CleanUp
  ;[0 1 0.5597] CleanUp when Operation is complete
  (bind _subtitlewidgetref (Variables|Default|GetSubtitleWidgetRef)
    (:then
      (Widget|RemovefromParent _subtitlewidgetref))
    (:else
      _))
  (Actor|DestroyActor))

(event Custom|DisplaySubtitles
  ;[0 1 0.6617] Display Subtitles on Screen
  (bind _returnvalue (UserInterface|CreateWidget "/Game/UI/WBP_Subtitles.WBP_Subtitles_C" (Game|GetPlayerController 0) (Variables|Default|GetSubtitleText)))
  (bind _output_get (Variables|Default|SetSubtitleWidgetRef _returnvalue))
  (UserInterface|Viewport|AddtoViewport _output_get 0))

(fn ConstructionScript)