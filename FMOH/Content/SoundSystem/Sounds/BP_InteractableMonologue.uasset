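; Interactable monologue trigger actor that plays a configurable 2D sound when its box is overlapped.
; Ending the overlap disables the actor's collision, so the trigger does not fire again.
; The starting transform is saved on BeginPlay and restored by teleport on reset, which does not re-enable collision.
; The interact event is an empty stub.
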(event OnComponentBeginOverlap(Box)
  (params (OverlappedComponent :type Primitive%20Component%20Object%20Reference) (OtherActor :type Actor%20Object%20Reference) (OtherComp :type Primitive%20Component%20Object%20Reference) (OtherBodyIndex :type Integer) (bFromSweep :type Boolean) (SweepResult :type Hit%20Result%20Structure%20%28by%20ref%29))
  (Audio|SpawnSound2D (Variables|Default|GetSound) (Variables|Default|GetVolume%20Multiplier) 1.0 0.0 0))

(event OnComponentEndOverlap(Box)
  (params (OverlappedComponent :type Primitive%20Component%20Object%20Reference) (OtherActor :type Actor%20Object%20Reference) (OtherComp :type Primitive%20Component%20Object%20Reference) (OtherBodyIndex :type Integer))
  (Collision|SetActorEnableCollision false))

(event EventBeginPlay
  (CallFunction|SaveforReset))

(event EventOnInteract
  (params (PlayerRef :type BP%20Third%20Person%20Character%20Object%20Reference)))

(event EventOnReset
  (bind _startinglocation (Variables|Default|GetStartingLocation))
  (Transformation|SetActorLocationAndRotation self (.location _startinglocation) (.rotation _startinglocation) false true))

(event EventSaveforReset
  (Variables|Default|SetStartingLocation (Transformation|GetWorldTransform (Variables|Default|GetDefaultSceneRoot))))

(fn ConstructionScript)