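; Interactable radio tuning knob that switches a linked radio between three channels.
; Interacting toggles a blended close-up view that locks the player's camera and sets Flying movement, with K also exiting.
; While viewing, holding the drag input after a camera trace hits the switcher lets Tick rotate the knob by player TurnRate, with angle-limit checks.
; Knob yaw serves as frequency: three bands select RadioBP channels, and values outside them play tuning static.
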(event Custom|Set%20Channel
  (params (RadioFrequency :type Float%20%28double-precision%29))
  (bind _radio_bp (Variables|Default|GetRadio%20BP))
  (bind _radio_bp_2 (Variables|Default|GetRadio%20BP))
  (bind _radio_bp_3 (Variables|Default|GetRadio%20BP))
  (bind _output_get (Variables|Default|SetRadioFrequency (Math|Float|Truncate RadioFrequency)))
  (Development|PrintString (Utilities|String|ToString(Integer) _output_get))
  (if (and (<= (Variables|Default|GetRadioFrequency) 20) (>= (Variables|Default|GetRadioFrequency) -40))
    (Variables|Default|SetCurrentChannelNr 0)
    (switch name (Utilities|Array|Get(acopy) (Variables|Default|GetChannelNames) (Variables|Default|GetCurrentChannelNr)) :!label _label
      (:Channel1
        (Default|RadioSwitchChannelto _radio_bp_2 (Variables|/Game/SoundSystem/Sounds/Radio/BP_ActivatableInteractableRadio.BP_ActivatableInteractableRadio_C|GetMS_Channel1 _radio_bp_2) 1))
      (:Channel2
        (Default|RadioSwitchChannelto _radio_bp_3 (Variables|/Game/SoundSystem/Sounds/Radio/BP_ActivatableInteractableRadio.BP_ActivatableInteractableRadio_C|GetMS_Channel2 _radio_bp_3) 2))
      (:Channel3
        (Default|RadioSwitchChannelto _radio_bp (Variables|/Game/SoundSystem/Sounds/Radio/BP_ActivatableInteractableRadio.BP_ActivatableInteractableRadio_C|GetMS_Channel3 _radio_bp) 3)))
    (elif (and (<= (Variables|Default|GetRadioFrequency) 110) (> (Variables|Default|GetRadioFrequency) 50))
      (Variables|Default|SetCurrentChannelNr 1)
      (goto _label)
      (elif (and (<= (Variables|Default|GetRadioFrequency) 170) (> (Variables|Default|GetRadioFrequency) 150))
        (Variables|Default|SetCurrentChannelNr 2)
        (goto _label)
        (else
          (Development|PrintString "Static Sound")
          (Audio|Components|Audio|Play (Variables|Default|GetMS_RadioTuning) 0.0))))))

(event Input|EnhancedActionEvents|EnhancedInputActionIA_DragObjects
  (params (ActionValue :type Boolean) (ElapsedSeconds :type Float%20%28double-precision%29) (TriggeredSeconds :type Float%20%28double-precision%29) (InputAction :type Input%20Action%20Object%20Reference :default "/Game/Character/Input/Actions/IA_DragObjects.IA_DragObjects"))
  (bind _camera (Variables|Default|GetCamera))
  (bind _returnvalue (Transformation|GetWorldLocation _camera))
  ;[1 1 1] Comment
  ;;[1 1 1] Comment
  (:Started
    (Variables|Default|SetbIsHoldingLMB true)
    (if (Variables|Default|GetbIsViewingSwitcher?)
      (bind _asbp_third_person_character (Utilities|Casting|CastToBP_ThirdPersonCharacter (Game|GetPlayerCharacter 0)))
      (bind (_outhit _returnvalue_2) (Collision|LineTraceForObjects _returnvalue (+ _returnvalue (* (Math|Vector|GetForwardVector _camera) 1e+02)) (Utilities|Array|MakeArray "ObjectTypeQuery1") false 0 "ForOneFrame" false))
      (if _returnvalue_2
        (bind _asbp_radio_channel_switcher (Utilities|Casting|CastToBP_RadioChannelSwitcher (.HitActor (Collision|BreakHitResult _outhit))))
        (if (== _asbp_radio_channel_switcher self)
          (Variables|Default|SetbLookingAtRadio true)
          (else
            (Variables|Default|SetbLookingAtRadio false :!label _label)))
        (else
          (goto _label)))))
  (:Canceled
    (Variables|Default|SetbIsHoldingLMB false :!label _label_2))
  (:Completed
    (goto _label_2)))

(event EventBeginPlay
  (|CallParentFunction)
  (Input|EnableInput (Game|GetPlayerController 0))
  (CallFunction|SetChannel (.yaw (Variables|/Script/Engine.SceneComponent|GetRelativeRotation (Variables|Default|GetSwitcher)))))

(event Collision|EventActorBeginOverlap
  (params (OtherActor :type Actor%20Object%20Reference)))

(event EventOnInteract
  (params (PlayerRef :type BP%20Third%20Person%20Character%20Object%20Reference))
  (bind _output_get (Variables|Default|SetPlayer%20Ref PlayerRef))
  (if (not (Variables|Default|GetbIsViewingSwitcher?))
    (Game|Player|SetViewTargetwithBlend (Game|GetPlayerController 0) self 1.0 "VTBlend_Linear" 0.0 false)
    (Pawn|Components|CharacterMovement|SetMovementMode (Variables|/Script/Engine.Character|GetCharacterMovement _output_get) "MOVE_Flying" 0)
    (Variables|Default|SetbIsViewingSwitcher? true)
    (Variables|/Game/ThirdPerson/Blueprints/BP_ThirdPersonCharacter.BP_ThirdPersonCharacter_C|SetbIsCameraLocked (Variables|Default|GetPlayer%20Ref) true)
    (else
      (Game|Player|SetViewTargetwithBlend (Game|GetPlayerController 0) (Variables|Default|GetPlayer%20Ref) 1.0 "VTBlend_Linear" 0.0 false)
      (Pawn|Components|CharacterMovement|SetMovementMode (Variables|/Script/Engine.Character|GetCharacterMovement (Variables|Default|GetPlayer%20Ref)) "MOVE_Walking" 0)
      (Variables|Default|SetbIsViewingSwitcher? false)
      (Variables|/Game/ThirdPerson/Blueprints/BP_ThirdPersonCharacter.BP_ThirdPersonCharacter_C|SetbIsCameraLocked (Variables|Default|GetPlayer%20Ref) false))))

(event EventTick
  (params (DeltaSeconds :type Float%20%28single-precision%29))
  (bind _switcher (Variables|Default|GetSwitcher))
  (bind _openangle (Variables|Default|GetOpenAngle))
  (bind _returnvalue (Transformation|GetWorldRotation _switcher))
  ;[1 1 1] Comment
  ;;[1 1 1] Comment
  (if (Variables|Default|GetbIsViewingSwitcher?)
    (if (Variables|Default|GetbIsHoldingLMB)
      (if (Variables|Default|GetbLookingAtRadio)
        (if (not (== (.yaw _returnvalue) (Math|Float|ClampAngle (.yaw _returnvalue) (Variables|Default|GetCloseAngle) (Variables|Default|GetOpenAngle))))
          (Transformation|AddLocalRotation _switcher (Math|Rotator|MakeRotator 0.0 0.0 (* (Variables|/Game/ThirdPerson/Blueprints/BP_ThirdPersonCharacter.BP_ThirdPersonCharacter_C|GetTurnRate (stale Input|EnhancedActionEvents|EnhancedInputActionIA_DragObjects _asbp_third_person_character)) (Variables|Default|GetSensitivity))) false false)
          (CallFunction|SetChannel (.Yaw (Math|Rotator|BreakRotator (Variables|/Script/Engine.SceneComponent|GetRelativeRotation (Variables|Default|GetSwitcher)))))
          (elif (>= (.yaw _returnvalue) _openangle)
            (Transformation|SetRelativeRotation _switcher (Math|Rotator|MakeRotator 0.0 0.0 (- _openangle 1.0)) false false)
            (else
              (Transformation|SetRelativeRotation _switcher (Math|Rotator|MakeRotator 0.0 0.0 (+ (Variables|Default|GetCloseAngle) 1.0)) false false))))))))

(event Input|KeyboardEvents|K
  (params (Key :type Key%20Structure :default "None"))
  (bind _player_ref (Variables|Default|GetPlayer%20Ref))
  (:Pressed
    (Game|Player|SetViewTargetwithBlend (Game|GetPlayerController 0) _player_ref 1.0 "VTBlend_Linear" 0.0 false)
    (Pawn|Components|CharacterMovement|SetMovementMode (Variables|/Script/Engine.Character|GetCharacterMovement _player_ref) "MOVE_Walking" 0)
    (Variables|Default|SetbIsViewingSwitcher? false)
    (Variables|/Game/ThirdPerson/Blueprints/BP_ThirdPersonCharacter.BP_ThirdPersonCharacter_C|SetbIsCameraLocked _player_ref false)))

(fn ConstructionScript
  (|CallParentFunction))