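; Power button actor for the second radio in the sound system, pressed by the player through an interact event.
; On interact it calls OnActivation on its referenced radio Blueprint, passing the player along.
; It then fakes a press by dropping the button mesh slightly in world Z and raising it back after a short Delay.
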(event EventBeginPlay
  (|CallParentFunction) ; This node is disabled and will not be called.\nDrag off pins to build functionality.
)

(event Collision|EventActorBeginOverlap
  (params (OtherActor :type Actor%20Object%20Reference)))

(event EventTick
  (params (DeltaSeconds :type Float%20%28single-precision%29)))

(event EventOnInteract
  (params (PlayerRef :type BP%20Third%20Person%20Character%20Object%20Reference))
  (bind _button (Variables|Default|GetButton))
  (bind _button_2 (Variables|Default|GetButton))
  (Default|OnActivation (Variables|Default|GetRadio%20BP) PlayerRef)
  (Transformation|SetWorldLocation _button (- (Transformation|GetWorldLocation _button) "0.000000,0.000000,2.000000") false false)
  (Utilities|FlowControl|Delay 0.4)
  (Transformation|SetWorldLocation _button_2 (+ (Transformation|GetWorldLocation _button_2) "0.000000,0.000000,2.000000") false false))

(fn ConstructionScript
  (|CallParentFunction))