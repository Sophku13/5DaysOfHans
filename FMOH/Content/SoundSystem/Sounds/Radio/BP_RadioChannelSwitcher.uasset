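; Interactable radio tuning knob that puts the player in a close-up minigame for switching channels on the linked RadioBP.
; Interacting blends the view to this actor and locks player controls; interacting again or pressing K restores them.
; While the radio is on, dragging after a camera trace hits the switcher rotates the knob on Tick from TurnRate, within angle limits.
; Knob roll maps to frequency bands that select channels, with tuning static playing in the gaps.
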(event Custom|Set%20Channel
  (params (RadioFrequency :type Float%20%28double-precision%29))
  (bind _radio_bp (Variables|Default|GetRadio%20BP))
  (bind _ms_radiotuning (Variables|Default|GetMS_RadioTuning))
  (bind _radio_bp_2 (Variables|Default|GetRadio%20BP))
  (bind _radio_bp_3 (Variables|Default|GetRadio%20BP))
  (bind _output_get (Variables|Default|SetRadioFrequency (Math|Float|Truncate RadioFrequency)))
  (if (and (<= (Variables|Default|GetRadioFrequency) 20) (>= (Variables|Default|GetRadioFrequency) -40))
    (Variables|Default|SetCurrentChannelNr 0)
    (Audio|Components|Audio|SetVolumeMultiplier (Variables|Default|GetMS_RadioTuning) 0.0 :!class /Script/Engine.AudioComponent :!label _label)
    (switch name (Utilities|Array|Get(acopy) (Variables|Default|GetChannelNames) (Variables|Default|GetCurrentChannelNr))
      (:Channel1
        (Default|RadioSwitchChannelto _radio_bp_2 (Variables|/Game/SoundSystem/Sounds/Radio/BP_ActivatableInteractableRadio.BP_ActivatableInteractableRadio_C|GetMS_Channel1 _radio_bp_2) 1))
      (:Channel2
        (Default|RadioSwitchChannelto _radio_bp_3 (Variables|/Game/SoundSystem/Sounds/Radio/BP_ActivatableInteractableRadio.BP_ActivatableInteractableRadio_C|GetMS_Channel2 _radio_bp_3) 2))
      (:Channel3
        (Default|RadioSwitchChannelto _radio_bp (Variables|/Game/SoundSystem/Sounds/Radio/BP_ActivatableInteractableRadio.BP_ActivatableInteractableRadio_C|GetMS_Channel3 _radio_bp) 3)))
    (elif (and (<= (Variables|Default|GetRadioFrequency) 110) (> (Variables|Default|GetRadioFrequency) 50))
      (Variables|Default|SetCurrentChannelNr 1)
      (goto _label)
      (elif (and (<= (Variables|Default|GetRadioFrequency) 170) (> (Variables|Default|GetRadioFrequency) 150))
        (Variables|Default|SetCurrentChannelNr 2)
        (goto _label)
        (else
          (Audio|Components|Audio|Play _ms_radiotuning 0.0)
          (Audio|Components|Audio|SetVolumeMultiplier _ms_radiotuning 1.0 :!class /Script/Engine.AudioComponent)
          (Audio|Components|Audio|SetVolumeMultiplier (Variables|/Game/SoundSystem/Sounds/Radio/BP_ActivatableInteractableRadio.BP_ActivatableInteractableRadio_C|GetCurrentChannelComponent (Variables|Default|GetRadio%20BP)) 0.0 :!class /Script/Engine.AudioComponent)
          (if (Math|Boolean|ANDBoolean (<= (Variables|Default|GetRadioFrequency) 20) (>= (Variables|Default|GetRadioFrequency) -40) (Math|Boolean|ANDBoolean (<= (Variables|Default|GetRadioFrequency) 110) (> (Variables|Default|GetRadioFrequency) 50) (and (<= (Variables|Default|GetRadioFrequency) 170) (> (Variables|Default|GetRadioFrequency) 150))))
            (Audio|Components|Audio|SetVolumeMultiplier (Variables|Default|GetMS_RadioTuning) 0.0 :!class /Script/Engine.AudioComponent)))))))

(event Input|EnhancedActionEvents|EnhancedInputActionIA_DragObjects
  (params (ActionValue :type Boolean) (ElapsedSeconds :type Float%20%28double-precision%29) (TriggeredSeconds :type Float%20%28double-precision%29) (InputAction :type Input%20Action%20Object%20Reference :default "/Game/Character/Input/Actions/IA_DragObjects.IA_DragObjects"))
  (bind _camera (Variables|Default|GetCamera))
  (bind _returnvalue (Transformation|GetWorldLocation _camera))
  ;[1 1 1] Comment
  ;;[1 1 1] Comment
  (:Started
    (Variables|Default|SetbIsHoldingLMB true :!label _label)
    (if (Variables|Default|GetbIsViewingSwitcher?)
      (bind _asbp_third_person_character (Utilities|Casting|CastToBP_ThirdPersonCharacter (Game|GetPlayerCharacter 0)))
      (bind (_outhit _returnvalue_2) (Collision|LineTraceForObjects _returnvalue (+ _returnvalue (* (Math|Vector|GetForwardVector _camera) 1e+02)) (Utilities|Array|MakeArray "ObjectTypeQuery1") false 0 "Persistent" false))
      (if _returnvalue_2
        (bind _asbp_radio_channel_switcher (Utilities|Casting|CastToBP_RadioChannelSwitcher (.HitActor (Collision|BreakHitResult _outhit))))
        (if (== _asbp_radio_channel_switcher self)
          (Variables|Default|SetbLookingAtRadio true)
          (else
            (Variables|Default|SetbLookingAtRadio false :!label _label_2)))
        (else
          (goto _label_2)))))
  (:Ongoing
    (goto _label))
  (:Canceled
    (Variables|Default|SetbIsHoldingLMB false :!label _label_3)
    (if (Variables|Default|GetbLookingAtRadio)
      _))
  (:Completed
    (goto _label_3)))

(event EventBeginPlay
  (|CallParentFunction)
  (Input|EnableInput (Game|GetPlayerController 0))
  (CallFunction|SetChannel (.roll (Variables|/Script/Engine.SceneComponent|GetRelativeRotation (Variables|Default|GetSwitcher)))))

(event Collision|EventActorBeginOverlap
  (params (OtherActor :type Actor%20Object%20Reference)))

(event EventOnInteract
  (params (PlayerRef :type BP%20Third%20Person%20Character%20Object%20Reference))
  (Variables|Default|SetPlayer%20Ref PlayerRef)
  (if (not (Variables|Default|GetbIsViewingSwitcher?))
    (Variables|/Game/ThirdPerson/Blueprints/BP_ThirdPersonCharacter.BP_ThirdPersonCharacter_C|SetbIsCameraLocked (Variables|Default|GetPlayer%20Ref) true)
    (Game|Player|SetViewTargetwithBlend (Game|GetPlayerController 0) self 0.0 "VTBlend_Linear" 0.0 false)
    (Variables|Default|SetbIsViewingSwitcher? true)
    (Variables|/Game/ThirdPerson/Blueprints/BP_ThirdPersonCharacter.BP_ThirdPersonCharacter_C|SetIsMovementLocked (Variables|Default|GetPlayer%20Ref) true)
    (Variables|/Game/ThirdPerson/Blueprints/BP_ThirdPersonCharacter.BP_ThirdPersonCharacter_C|SetbIsInMinigame (Variables|Default|GetPlayer%20Ref) true)
    (Widget|SetVisibility (Variables|/Game/ThirdPerson/Blueprints/BP_ThirdPersonCharacter.BP_ThirdPersonCharacter_C|GetCrosshair%20REF (Variables|Default|GetPlayer%20Ref)) "Hidden")
    (else
      (Game|Player|SetViewTargetwithBlend (Game|GetPlayerController 0) (Variables|Default|GetPlayer%20Ref) 0.0 "VTBlend_Linear" 0.0 false)
      (Variables|Default|SetbIsViewingSwitcher? false)
      (Variables|/Game/ThirdPerson/Blueprints/BP_ThirdPersonCharacter.BP_ThirdPersonCharacter_C|SetbIsCameraLocked (Variables|Default|GetPlayer%20Ref) false)
      (Variables|/Game/ThirdPerson/Blueprints/BP_ThirdPersonCharacter.BP_ThirdPersonCharacter_C|SetIsMovementLocked (Variables|Default|GetPlayer%20Ref) false)
      (Variables|/Game/ThirdPerson/Blueprints/BP_ThirdPersonCharacter.BP_ThirdPersonCharacter_C|SetbIsInMinigame (Variables|Default|GetPlayer%20Ref) false)
      (Widget|SetVisibility (Variables|/Game/ThirdPerson/Blueprints/BP_ThirdPersonCharacter.BP_ThirdPersonCharacter_C|GetCrosshair%20REF (Variables|Default|GetPlayer%20Ref)) "Visible"))))

(event EventTick
  (params (DeltaSeconds :type Float%20%28single-precision%29))
  (bind _openangle (Variables|Default|GetOpenAngle))
  (bind _switcher (Variables|Default|GetSwitcher))
  (bind _returnvalue (Transformation|GetWorldRotation _switcher))
  ;[1 1 1] Comment
  ;;[1 1 1] Comment
  (if (Variables|Default|GetbIsViewingSwitcher?)
    (if (Variables|/Game/SoundSystem/Sounds/Radio/BP_ActivatableInteractableRadio.BP_ActivatableInteractableRadio_C|GetbIsRadioOn? (Variables|Default|GetRadio%20BP))
      (if (Variables|Default|GetbIsHoldingLMB)
        (if (Variables|Default|GetbLookingAtRadio)
          (if (Math|Float|NearlyEqual(Float) (.roll _returnvalue) (Math|Float|ClampAngle (.roll _returnvalue) (Variables|Default|GetCloseAngle) (Variables|Default|GetOpenAngle)) 1e-05)
            (Transformation|AddWorldRotation _switcher (Math|Rotator|MakeRotator (* (Variables|/Game/ThirdPerson/Blueprints/BP_ThirdPersonCharacter.BP_ThirdPersonCharacter_C|GetTurnRate (stale Input|EnhancedActionEvents|EnhancedInputActionIA_DragObjects _asbp_third_person_character)) (Variables|Default|GetSensitivity)) 0.0 0.0) false false)
            (CallFunction|SetChannel (.roll (Transformation|GetWorldRotation (Variables|Default|GetSwitcher))))
            (elif (>= (.roll _returnvalue) _openangle)
              (Transformation|SetWorldRotation _switcher (Math|Rotator|MakeRotator (- _openangle 5.0) 0.0 1.8e+02) false false)
              (else
                (Transformation|SetWorldRotation _switcher (Math|Rotator|MakeRotator (+ (Variables|Default|GetCloseAngle) 5.0) 0.0 1.8e+02) false false)))))))))

(event Input|KeyboardEvents|K
  (params (Key :type Key%20Structure :default "None"))
  (bind _player_ref (Variables|Default|GetPlayer%20Ref))
  (:Pressed
    (Game|Player|SetViewTargetwithBlend (Game|GetPlayerController 0) _player_ref 0.0 "VTBlend_Linear" 0.0 false)
    (Variables|Default|SetbIsViewingSwitcher? false)
    (Variables|/Game/ThirdPerson/Blueprints/BP_ThirdPersonCharacter.BP_ThirdPersonCharacter_C|SetbIsCameraLocked _player_ref false)
    (Variables|/Game/ThirdPerson/Blueprints/BP_ThirdPersonCharacter.BP_ThirdPersonCharacter_C|SetIsMovementLocked _player_ref false)
    (Variables|/Game/ThirdPerson/Blueprints/BP_ThirdPersonCharacter.BP_ThirdPersonCharacter_C|SetbIsInMinigame _player_ref false)
    (Widget|SetVisibility (Variables|/Game/ThirdPerson/Blueprints/BP_ThirdPersonCharacter.BP_ThirdPersonCharacter_C|GetCrosshair%20REF _player_ref) "Visible")))

(fn ConstructionScript
  (|CallParentFunction))