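; BP_Radio_02 is a radio actor that toggles on and off when activated, playing a switch sound at its location.
; Turning on waits briefly, then asks the referenced channel switcher to set the channel from its knob's yaw; turning off stops the current channel's audio.
; RadioSwitchChannelTo records the selected channel and, while on, swaps channels by volume, muting the previous component and raising the new one.
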(event Custom|Turn%20Radio%20On
  (bind _chanelswitcherref (Variables|Default|GetChanelSwitcherRef))
  (Audio|PlaySoundatLocation "/Game/SoundSystem/Sounds/SFX/Actions/RADIO-SWITCH-ON_6EXT8-11087.RADIO-SWITCH-ON_6EXT8-11087" (Transformation|GetWorldLocation (Variables|Default|GetRadio)) "0, 0, 0" 1.0 1.0 0.0 0 0 0 0)
  (Utilities|FlowControl|Delay 0.2)
  (Variables|Default|SetbIsRadioOn? true)
  (Default|SetChannel _chanelswitcherref (.yaw (Variables|/Script/Engine.SceneComponent|GetRelativeRotation (Variables|/Game/SoundSystem/Sounds/Radio/BP_RadioChannelSwitcher.BP_RadioChannelSwitcher_C|GetSwitcher _chanelswitcherref)))))

(event Custom|Turn%20Radio%20Off
  (Audio|PlaySoundatLocation "/Game/SoundSystem/Sounds/SFX/Actions/RADIO-SWITCH-OFF_6EXT8-11085.RADIO-SWITCH-OFF_6EXT8-11085" (Transformation|GetWorldLocation (Variables|Default|GetRadio)) "0, 0, 0" 1.0 1.0 0.0 0 0 0 0)
  (Audio|Components|Audio|Stop (Variables|Default|GetCurrentChannelComponent))
  (Variables|Default|SetbIsRadioOn? false))

(event Custom|Toggle%20Radio%20ON%20OFF
  (if (Variables|Default|GetbIsRadioOn?)
    (CallFunction|TurnRadioOff)
    (else
      (CallFunction|TurnRadioon))))

(event Custom|Radio%20Switch%20Channel%20To
  (params (ChannelComponent :type Audio%20Component%20Object%20Reference) (CurrentChannel :type Integer))
  (Variables|Default|SetCurrentChannel CurrentChannel)
  (if (Variables|Default|GetbIsRadioOn?)
    (Audio|Components|Audio|Play (Variables|Default|GetCurrentChannelComponent) 0.0)
    (Audio|Components|Audio|SetVolumeMultiplier ChannelComponent 1.0 :!class /Script/Engine.AudioComponent)
    (if (== ChannelComponent (Variables|Default|GetCurrentChannelComponent))
      _
      (else
        (Audio|Components|Audio|SetVolumeMultiplier (Variables|Default|GetCurrentChannelComponent) 0.0 :!class /Script/Engine.AudioComponent)))
    (Variables|Default|SetCurrentChannelComponent ChannelComponent)
    (else
      (Variables|Default|SetCurrentChannelComponent ChannelComponent))))

(event EventBeginPlay
  (|CallParentFunction) ; This node is disabled and will not be called.\nDrag off pins to build functionality.
)

(event Collision|EventActorBeginOverlap
  (params (OtherActor :type Actor%20Object%20Reference))
  (|CallParentFunction OtherActor) ; This node is disabled and will not be called.\nDrag off pins to build functionality.
)

(event EventTick
  (params (DeltaSeconds :type Float%20%28single-precision%29))
  (|CallParentFunction DeltaSeconds) ; This node is disabled and will not be called.\nDrag off pins to build functionality.
)

(event EventOnInteract
  (params (PlayerRef :type BP%20Third%20Person%20Character%20Object%20Reference)))

(event EventOnActivation
  (params (PlayerRef :type BP%20Third%20Person%20Character%20Object%20Reference))
  (CallFunction|ToggleRadioONOFF))

(fn ConstructionScript
  (|CallParentFunction))