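; Inner monologue actor that plays a 2D voice line and shows subtitles, triggered by box overlap or Blueprint call to SpawnWithValues.
; CheckValues replaces the player's current voice or subtitle for whichever content is set, registers itself on the player, then cleans up after LifeTime.
; CleanUp removes the subtitle; early cleanup can also stop the voice and destroy non-respawning instances.
; OnReset re-enables the trigger's collision.
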(event OnComponentBeginOverlap(Box)
  (params (OverlappedComponent :type Primitive%20Component%20Object%20Reference) (OtherActor :type Actor%20Object%20Reference) (OtherComp :type Primitive%20Component%20Object%20Reference) (OtherBodyIndex :type Integer) (bFromSweep :type Boolean) (SweepResult :type Hit%20Result%20Structure%20%28by%20ref%29))
  ;[0 1 0.515] Player Overlap in Level
  (CallFunction|CheckValues)
  (Collision|SetCollisionEnabled (Variables|Default|GetBox) "NoCollision"))

(event Custom|SpawnWithValues
  (params (Sound :type Sound%20Base%20Object%20Reference) (Volume%20Multiplier :type Float%20%28single-precision%29) (SubtitleText :type Text) (LifeTime :type Float%20%28double-precision%29) (bIsNotRespawning :type Boolean))
  ;[0 1 0.596] Access through Blueprints
  (Collision|SetCollisionEnabled (Variables|Default|GetBox) "NoCollision")
  (Variables|Default|SetSound Sound)
  (Variables|Default|SetVolume%20Multiplier Volume%20Multiplier)
  (Variables|Default|SetSubtitleText SubtitleText)
  (Variables|Default|SetLifeTime LifeTime)
  (Variables|Default|SetbIsNotRespawning bIsNotRespawning)
  (CallFunction|CheckValues))

(event Custom|CheckValues
  ;[0 1 0.5631] Automatically Checking which values are set and starts operations accordingly
  (Variables|Default|GetSound
    (:then
      (bind _currentvoice (Variables|/Game/ThirdPerson/Blueprints/BP_ThirdPersonCharacter.BP_ThirdPersonCharacter_C|GetCurrentVoice (Variables|Default|GetPlayerRef))
        (:then
          (Audio|Components|Audio|Stop _currentvoice))
        (:else
          _))
      (if (Math|Float|NearlyEqual(Float) (Variables|Default|GetVolume%20Multiplier) 0.0 0.001)
        (Variables|Default|SetVolume%20Multiplier 1.0)
        (CallFunction|PlayInnerMonologue)
        (else
          (CallFunction|PlayInnerMonologue))))
    (:else
      _))
  (if (not (Utilities|Text|TextIsEmpty (Variables|Default|GetSubtitleText)))
    (bind _subtitleref (Variables|/Game/ThirdPerson/Blueprints/BP_ThirdPersonCharacter.BP_ThirdPersonCharacter_C|GetSubtitleRef (Variables|Default|GetPlayerRef))
      (:then
        (Widget|RemovefromParent _subtitleref))
      (:else
        _))
    (CallFunction|DisplaySubtitles))
  (Variables|/Game/ThirdPerson/Blueprints/BP_ThirdPersonCharacter.BP_ThirdPersonCharacter_C|SetInnerMonologRef (Variables|Default|GetPlayerRef) self)
  (if (Math|Float|NearlyEqual(Float) (Variables|Default|GetLifeTime) 0.0 0.1)
    (Utilities|FlowControl|Delay 1.0)
    (else
      (Utilities|FlowControl|Delay (Variables|Default|GetLifeTime))))
  (CallFunction|CleanUp false))

(event Custom|PlayInnerMonologue
  (bind _playerref (Variables|Default|GetPlayerRef))
  ;[0 1 0.566] Spawns InnerMonolog Sound
  (bind _returnvalue (Audio|SpawnSound2D (Variables|Default|GetSound) (Variables|Default|GetVolume%20Multiplier) 1.0 0.0 0 true))
  (Variables|Default|SetSoundRef _returnvalue)
  (Variables|/Game/ThirdPerson/Blueprints/BP_ThirdPersonCharacter.BP_ThirdPersonCharacter_C|SetCurrentVoice _playerref _returnvalue)
  (Variables|/Game/ThirdPerson/Blueprints/BP_ThirdPersonCharacter.BP_ThirdPersonCharacter_C|SetbIsPlayingVoiceLine _playerref true))

(event Custom|CleanUp
  (params (EarlyCleanup :type Boolean))
  ;[0 1 0.5597] CleanUp when Operation is complete
  (if (Variables|Default|GetbIsNotRespawning)
    (bind _subtitlewidgetref (Variables|Default|GetSubtitleWidgetRef)
      (:then
        (Widget|RemovefromParent _subtitlewidgetref))
      (:else
        _))
    (if EarlyCleanup
      (bind _currentvoice (Variables|/Game/ThirdPerson/Blueprints/BP_ThirdPersonCharacter.BP_ThirdPersonCharacter_C|GetCurrentVoice (Variables|Default|GetPlayerRef))
        (:then
          (Audio|Components|Audio|Stop _currentvoice))
        (:else
          _))
      (Actor|DestroyActor))
    (else
      (Collision|SetCollisionEnabled (Variables|Default|GetBox) "NoCollision")
      (bind _subtitlewidgetref_2 (Variables|Default|GetSubtitleWidgetRef)
        (:then
          (Widget|RemovefromParent _subtitlewidgetref_2)
          (if EarlyCleanup
            (bind _currentvoice_2 (Variables|/Game/ThirdPerson/Blueprints/BP_ThirdPersonCharacter.BP_ThirdPersonCharacter_C|GetCurrentVoice (Variables|Default|GetPlayerRef))
              (:then
                (Audio|Components|Audio|Stop _currentvoice_2))
              (:else))))
        (:else)))))

(event Custom|DisplaySubtitles
  ;[0 1 0.6617] Display Subtitles on Screen
  (bind _subtitlewidgetref (Variables|Default|GetSubtitleWidgetRef)
    (:then
      _)
    (:else
      (bind _returnvalue (UserInterface|CreateWidget "/Game/UI/WBP_Subtitles.WBP_Subtitles_C" (Game|GetPlayerController 0) (Variables|Default|GetSubtitleText)))
      (bind _output_get (Variables|Default|SetSubtitleWidgetRef _returnvalue))))
  (Variables|/Game/ThirdPerson/Blueprints/BP_ThirdPersonCharacter.BP_ThirdPersonCharacter_C|SetSubtitleRef (Variables|Default|GetPlayerRef) (Variables|Default|GetSubtitleWidgetRef))
  (UserInterface|Viewport|AddtoViewport _output_get 0))

(event EventBeginPlay
  (bind _returnvalue (Actor|GetActorOfClass "/Game/ThirdPerson/Blueprints/BP_ThirdPersonCharacter.BP_ThirdPersonCharacter_C"))
  (Variables|Default|SetPlayerRef _returnvalue)
  (if (not (Variables|Default|GetbIsNotRespawning))
    (Variables|/Script/Engine.PrimitiveComponent|SetbGenerateOverlapEvents (Variables|Default|GetBox) true)))

(event EventOnReset
  ;[0 1 0.5457] OnReset
  (Collision|SetCollisionEnabled (Variables|Default|GetBox) "QueryOnly"))

(fn ConstructionScript
  (|CallParentFunction))