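; Sound actor that starts the parents' arguing audio and flags BP_ParentsFightingMinigame as fighting.
; Once both trigger boxes have been overlapped, each disabling its collision, a delay precedes the audio, followed by a subtitled inner monologue through BP_InterMono.
; StopShouting mutes and stops the sound.
; OnReset mutes it and re-arms the boxes but leaves ParentsFighting set, which blocks StartShouting from replaying.
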(event OnComponentBeginOverlap(BoxA)
  (params (OverlappedComponent :type Primitive%20Component%20Object%20Reference) (OtherActor :type Actor%20Object%20Reference) (OtherComp :type Primitive%20Component%20Object%20Reference) (OtherBodyIndex :type Integer) (bFromSweep :type Boolean) (SweepResult :type Hit%20Result%20Structure%20%28by%20ref%29))
  (Variables|Default|SetbIsBoxAActivated true)
  (Collision|SetCollisionEnabled (Variables|Default|GetBoxA) "NoCollision")
  (CallFunction|StartShouting))

(event OnComponentBeginOverlap(BoxB)
  (params (OverlappedComponent :type Primitive%20Component%20Object%20Reference) (OtherActor :type Actor%20Object%20Reference) (OtherComp :type Primitive%20Component%20Object%20Reference) (OtherBodyIndex :type Integer) (bFromSweep :type Boolean) (SweepResult :type Hit%20Result%20Structure%20%28by%20ref%29))
  (Variables|Default|SetbIsBoxBActivated true)
  (Collision|SetCollisionEnabled (Variables|Default|GetBoxB) "NoCollision")
  (CallFunction|StartShouting))

(event Custom|Start%20Shouting
  (if (not (Variables|Default|GetbParentsFighting))
    (if (and (Variables|Default|GetbIsBoxAActivated) (Variables|Default|GetbIsBoxBActivated))
      (Utilities|FlowControl|Delay 5.0)
      (Audio|Components|Audio|SetVolumeMultiplier (Variables|Default|GetMS_ParentsArgueing) 1.0 :!class /Script/Engine.AudioComponent)
      (Audio|Components|Audio|Play (Variables|Default|GetMS_ParentsArgueing) 0.0)
      (bind _returnvalue (Actor|GetActorOfClass "/Game/Mechanics/MiniGames/ParentsFighting/BP_ParentsFightingMinigame.BP_ParentsFightingMinigame_C"))
      (Variables|/Game/Mechanics/MiniGames/ParentsFighting/BP_ParentsFightingMinigame.BP_ParentsFightingMinigame_C|SetbParentsAreFighting _returnvalue true)
      (Variables|Default|SetbParentsFighting true)
      ;[0 0.0386 0.8906] Spawns subtitle
      (Utilities|FlowControl|Delay 2.0)
      (bind _returnvalue_2 (Game|SpawnActorfromClass "/Game/SoundSystem/Sounds/BP_InterMono.BP_InterMono_C" (Transformation|GetActorTransform (Game|GetPlayerCharacter 0)) "Undefined" "MultiplyWithRoot" 0 "/Game/SoundSystem/Sounds/VoiceRecordings/Hans/YoungHans/SieSchreienWieder.SieSchreienWieder" 1.0 "They are shouting again. I need to make them stop." 5.0 true 0))
      (Default|CheckValues _returnvalue_2))))

(event Custom|Event%20Stop%20Shouting
  (Audio|Components|Audio|SetVolumeMultiplier (Variables|Default|GetMS_ParentsArgueing) 0.0 :!class /Script/Engine.AudioComponent)
  (Audio|Components|Audio|Stop (Variables|Default|GetMS_ParentsArgueing)))

(event EventBeginPlay
  (|CallParentFunction) ; This node is disabled and will not be called.\nDrag off pins to build functionality.
)

(event Collision|EventActorBeginOverlap
  (params (OtherActor :type Actor%20Object%20Reference)))

(event EventOnReset
  (Audio|Components|Audio|SetVolumeMultiplier (Variables|Default|GetMS_ParentsArgueing) 0.0 :!class /Script/Engine.AudioComponent)
  (Collision|SetCollisionEnabled (Variables|Default|GetBoxA) "QueryOnly")
  (Collision|SetCollisionEnabled (Variables|Default|GetBoxB) "QueryOnly")
  (Variables|Default|SetbIsBoxAActivated false)
  (Variables|Default|SetbIsBoxBActivated false))

(fn ConstructionScript
  (|CallParentFunction))